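; Level-transition actor that lets the player move to another level by pressing Interact while nearby.
; Player overlap shows a tooltip widget and Niagara effect and enables input, unless the GameInstance reports a scene is being viewed.
; Interacting plays a sliding-door sound, saves the current room as PreviousRoom in the GameInstance, fades to black and opens LevelToLoad after a short delay.
; BeginPlay fades from black and sets up the hidden tooltip.
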(event `self.ReceiveBeginPlay`
  (bind _returnvalue (`|CreateWidget` "/Game/ProjectContents/BP/Widgets/WBP_FadeBlack.WBP_FadeBlack_C" (`GameplayStatics.GetPlayerController` 0)))
  (`UserWidget.AddToViewport` _returnvalue 0)
  (`/Game/ProjectContents/BP/Widgets/WBP_FadeBlack.FadeFromBlack` _returnvalue)
  (bind _aswbp_move_levels_text (cast `/Game/ProjectContents/BP/Widgets/WBP_MoveLEvelsText` (`WidgetComponent.GetUserWidgetObject` (`self.Widget`))))
  (bind _output_get (set `self.WidgetObject` _aswbp_move_levels_text))
  (`/Game/ProjectContents/BP/Widgets/WBP_MoveLEvelsText.SetHidden` _output_get)
  (`KismetSystemLibrary.Delay` 0.3)
  (`/Game/ProjectContents/BP/Widgets/WBP_MoveLEvelsText.SetTextBox` (`self.WidgetObject`) (`self.ToolTipText`)))

(event `self.ReceiveActorBeginOverlap`
  (params (OtherActor :type "Actor Object Reference"))
  ;[1 1 1] Toggle Visibility
  (cast `/Game/ProjectContents/BP/Player/BP_PawnPlayerBase` OtherActor)
  (bind _asbp_game_instance (cast `/Game/ProjectContents/BP/BP_GameInstance` (`GameplayStatics.GetGameInstance`)))
  (if (`/Game/ProjectContents/BP/BP_GameInstance.isViewingScene` _asbp_game_instance)
    (`self.DisableInput` (`GameplayStatics.GetPlayerController` 0))
    (`/Game/ProjectContents/BP/Widgets/WBP_MoveLEvelsText.SetHidden` (`self.WidgetObject`))
    (`ActorComponent.Deactivate` (`self.Niagara`))
    (else
      (`/Game/ProjectContents/BP/Widgets/WBP_MoveLEvelsText.SetVisible` (`self.WidgetObject`))
      (set `self.isPlayerNear` true)
      (`self.EnableInput` (`GameplayStatics.GetPlayerController` 0))
      (`ActorComponent.Activate` (`self.Niagara`) false))))

(event `self.ReceiveActorEndOverlap`
  (params (OtherActor :type "Actor Object Reference"))
  ;[1 1 1] Toggle Visibility
  (cast `/Game/ProjectContents/BP/Player/BP_PawnPlayerBase` OtherActor)
  (set `self.isPlayerNear` false)
  (`/Game/ProjectContents/BP/Widgets/WBP_MoveLEvelsText.SetHidden` (`self.WidgetObject`))
  (`ActorComponent.Deactivate` (`self.Niagara`)))

(event `LoadNextLevel`
  ;[1 1 1] Load Next Level
  (bind _returnvalue (`|CreateWidget` "/Game/ProjectContents/BP/Widgets/WBP_FadeBlack.WBP_FadeBlack_C" (`GameplayStatics.GetPlayerController` 0)))
  (`UserWidget.AddToViewport` _returnvalue 0)
  (`/Game/ProjectContents/BP/Widgets/WBP_FadeBlack.FadeToBlack` _returnvalue)
  (`KismetSystemLibrary.Delay` 0.4)
  (`GameplayStatics.OpenLevel` (`self.LevelToLoad`)))

(event `InputAction|Interact` :consume false
  (params (Key :type "Key Structure"))
  ;[1 1 1] Interact - Action
  (:`Pressed`
    (if (`self.isPlayerNear`)
      (`GameplayStatics.PlaySound2D` "/Game/ProjectContents/SFX/SFX_SlidingDoor_Open.SFX_SlidingDoor_Open" 1.0 1.0 0.0 null null)
      (bind _asbp_game_instance (cast `/Game/ProjectContents/BP/BP_GameInstance` (`GameplayStatics.GetGameInstance`)))
      (set `/Game/ProjectContents/BP/BP_GameInstance.PreviousRoom` (`self.CurrentRoom`) _asbp_game_instance)
      (`self.LoadNextLevel`))))

(fn `UserConstructionScript`)