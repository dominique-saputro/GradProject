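; Dialog manager actor that shows dialogue text on chosen actors.
; Display events find TextRender components tagged DisplayTextRender to show text persistently, briefly, or as a timed line sequence that re-calls itself, with DisplayDialog returning the total wait.
; A second Test-prefixed path fills the actor's WBP_DialogBox widget component from a stored list, stepping with a sound while the GameInstance is viewing a scene, or auto-scrolling on a delay.
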(event `self.ReceiveBeginPlay`)

(event `DisplayTextAlways`
  (params (`Selected Actor` :type "Actor Object Reference") (Text :type Text))
  ;[1 1 1] Display Text On Actor Always
  (for _array_element (`self.GetComponentsByTag` `Selected Actor` "/Script/Engine.TextRenderComponent" "DisplayTextRender")
    (`TextRenderComponent.K2_SetText` _array_element Text)
    (`SceneComponent.SetVisibility` _array_element true false)))

(event `DisplayTextOnce`
  (params (DisplayActor :type "Actor Object Reference") (DisplayText :type Text) (TextDelay :type "Float (double-precision)"))
  ;[1 1 1] Display Text On Actor Once
  (for _array_element (`self.GetComponentsByTag` DisplayActor "/Script/Engine.TextRenderComponent" "DisplayTextRender")
    (`TextRenderComponent.K2_SetText` _array_element DisplayText)
    (`SceneComponent.SetVisibility` _array_element true false)
    (`KismetSystemLibrary.Delay` TextDelay)
    (`SceneComponent.SetVisibility` _array_element false false)))

(event `Remove Display Text`
  (params (SelectedActor :type "Actor Object Reference"))
  ;[1 1 1] Remove Display Text on Actor
  (for _array_element (`self.GetComponentsByTag` SelectedActor "/Script/Engine.TextRenderComponent" "DisplayTextRender")
    (`SceneComponent.SetVisibility` _array_element false false)))

(event `CycleLongDialog`
  (params (`Selected Actor` :type "Actor Object Reference") (`Text Array` :type "Array of Text") (`Text Delay` :type "Float (double-precision)"))
  ;[1 1 1] Cycle Long Text On Actor
  (for _array_element (`self.GetComponentsByTag` `Selected Actor` "/Script/Engine.TextRenderComponent" "DisplayTextRender")
    (if (== (`self.CurrentTextIndex`) (`KismetArrayLibrary.Array_Length` `Text Array`))
      (`KismetSystemLibrary.PrintString` "DialogCycleFinished")
      (set `self.CurrentTextIndex` 0)
      (`SceneComponent.SetVisibility` _array_element false false)
      (else
        (`TextRenderComponent.K2_SetText` _array_element (`|GetArrayItem` `Text Array` (`self.CurrentTextIndex`)))
        (`SceneComponent.SetVisibility` _array_element true false)
        (`KismetSystemLibrary.Delay` `Text Delay`)
        (`/Engine/EditorBlueprintResources/StandardMacros.IncrementInt` (`self.CurrentTextIndex`)
          (:`  `
            (`self.CycleLongDialog` `Selected Actor` `Text Array` `Text Delay`)))))))

(event `Test-SetDialogList`
  (params (SelectedActor :type "Actor Object Reference") (DialogList :type "Array of Text"))
  (set `self.Selected Actor` SelectedActor)
  (set `self.SelectedActorDialogBox` (`self.GetComponentByClass` SelectedActor "/Script/UMG.WidgetComponent"))
  (set `self.CurrentDialogList` DialogList))

(event `Test-CycleOnKey`
  (bind _selectedactordialogbox (`self.SelectedActorDialogBox`))
  (bind _asbp_game_instance (cast `/Game/ProjectContents/BP/BP_GameInstance` (`GameplayStatics.GetGameInstance`)))
  (if (`/Game/ProjectContents/BP/BP_GameInstance.isViewingScene` _asbp_game_instance)
    (`GameplayStatics.PlaySound2D` "/Engine/VREditor/Sounds/UI/Selection_Changes.Selection_Changes" 1.0 1.0 0.0 null null)
    (if (== (`self.CurrentTextIndex`) (`KismetArrayLibrary.Array_Length` (`self.CurrentDialogList`)))
      (set `self.isDIalogFinished` true)
      (`SceneComponent.SetVisibility` (`self.SelectedActorDialogBox`) false false)
      (set `self.CurrentTextIndex` 0)
      (else
        (bind _aswbp_dialog_box (cast `/Game/ProjectContents/BP/Widgets/WBP_DialogBox` (`WidgetComponent.GetWidget` _selectedactordialogbox)))
        (`/Game/ProjectContents/BP/Widgets/WBP_DialogBox.SetText` _aswbp_dialog_box (`|GetArrayItem` (`self.CurrentDialogList`) (`self.CurrentTextIndex`)))
        (`SceneComponent.SetVisibility` _selectedactordialogbox true false)
        (`/Engine/EditorBlueprintResources/StandardMacros.IncrementInt` (`self.CurrentTextIndex`))))))

(event `Test - AutoScroll`
  (params (CycleDelay :type "Float (double-precision)"))
  (if (`self.isDIalogFinished`)
    (set `self.isAutoScrollFinished` true)
    (else
      (`self.Test-CycleOnKey`)
      (`KismetSystemLibrary.Delay` CycleDelay)
      (`self.Test - AutoScroll` CycleDelay))))

(fn `Calculate Dialog Delay`
  (params (`Dialog Array` :type "Array of Text") (`Text Delay` :type "Float (double-precision)"))
  (returns (`Dialog Delay` :type "Float (double-precision)"))
  (return (+ (* (`KismetArrayLibrary.Array_Length` `Dialog Array`) `Text Delay`) 0.5)))

(fn `Display Dialog`
  (params (`Selected Actor` :type "Actor Object Reference") (`Text Array` :type "Array of Text") (`Text Delay` :type "Float (double-precision)"))
  (returns (`Dialog Delay` :type "Float (double-precision)"))
  (`self.CycleLongDialog` `Selected Actor` `Text Array` `Text Delay`)
  (bind _dialog_delay (`self.Calculate Dialog Delay` `Text Array` `Text Delay`))
  (return _dialog_delay))

(fn `UserConstructionScript`)