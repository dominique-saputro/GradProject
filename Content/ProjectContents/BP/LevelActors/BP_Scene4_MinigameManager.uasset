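; Manager actor for the Scene 4 cafeteria minigame, where the player supplies ingredients to make yakisobapan.
; BeginPlay spawns bread, ginger, noodle and sauce kitchen items and shows the first need as a sprite.
; Interacting inside the box with noodle and sauce has the staff NPC cook and spawn yakisoba on timed delays.
; Otherwise it checks inventory against the current need, advancing or showing "I need" text, and finally displays yakisobapan.
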(event `Handle Yakisoba`
  (bind _staffactor (`/Game/ProjectContents/BP/SceneManager/BP_SceneManager_Scene04_Cafeteria.StaffActor` (`self.SceneManager`)))
  (bind _returnvalue (`self.K2_GetActorLocation` _staffactor))
  ;[1 1 1] Handle Yakisoba
  (`KismetArrayLibrary.Array_RemoveItem` (`self.Inventory`) "noodle")
  (`KismetArrayLibrary.Array_RemoveItem` (`self.Inventory`) "sauce")
  (bind _asbp_npcactor_staff (cast `/Game/ProjectContents/BP/NPC/BP_NPCActor_Staff` _staffactor))
  (`/Game/ProjectContents/BP/NPC/BP_NPCActorBase.MoveNPC Event` _asbp_npcactor_staff _returnvalue (- _returnvalue (300.0 0.0 0.0)))
  (`KismetSystemLibrary.Delay` 3.0)
  (`GameplayStatics.PlaySound2D` "/Game/ProjectContents/SFX/SFX_Cooking.SFX_Cooking" 1.0 1.0 0.0 null null)
  (`KismetSystemLibrary.Delay` 4.0)
  (bind _returnvalue_2 (`|SpawnActorFromClass` (`self.KitchenItems`) (`KismetMathLibrary.MakeTransform` (`self.Yakisoba SpawnLocation`)) "Undefined" "OverrideRootScale" null null))
  (bind _asbp_kitchen_items (cast `/Game/ProjectContents/BP/Objects/BP_KitchenItems` _returnvalue_2))
  (set `/Game/ProjectContents/BP/Objects/BP_KitchenItems.ItemName` "yakisoba" _asbp_kitchen_items)
  (set `/Game/ProjectContents/BP/Objects/BP_KitchenItems.SelectedSprite` "/Game/ProjectContents/Spites/Cafeteria/yakisoba_Sprite.yakisoba_Sprite" _asbp_kitchen_items)
  (bind _output_get (set `self.Yakisoba` _asbp_kitchen_items))
  (`/Game/ProjectContents/BP/Objects/BP_KitchenItems.UpdateSprite` _output_get)
  (`KismetSystemLibrary.Delay` 1.0)
  (bind _asbp_npcactor_staff_2 (cast `/Game/ProjectContents/BP/NPC/BP_NPCActor_Staff` (`/Game/ProjectContents/BP/SceneManager/BP_SceneManager_Scene04_Cafeteria.StaffActor` (`self.SceneManager`))))
  (`/Game/ProjectContents/BP/BP_FunctionLib.Flip FlipBook` _asbp_npcactor_staff_2)
  (bind _returnvalue_3 (`self.K2_GetActorLocation` _asbp_npcactor_staff_2))
  (`/Game/ProjectContents/BP/NPC/BP_NPCActorBase.MoveNPC Event` _asbp_npcactor_staff_2 _returnvalue_3 (+ _returnvalue_3 (300.0 0.0 0.0)))
  (`KismetSystemLibrary.Delay` 3.0))

(event `self.ReceiveBeginPlay`
  (`|ExecutionSequence`
    (:`then_0`
      (bind _returnvalue (`|SpawnActorFromClass` (`self.KitchenItems`) (`KismetMathLibrary.MakeTransform` (`self.Bread SpawnLocation`)) "Undefined" "OverrideRootScale" null null))
      (bind _asbp_kitchen_items (cast `/Game/ProjectContents/BP/Objects/BP_KitchenItems` _returnvalue))
      (set `/Game/ProjectContents/BP/Objects/BP_KitchenItems.ItemName` "bread" _asbp_kitchen_items)
      (set `/Game/ProjectContents/BP/Objects/BP_KitchenItems.SelectedSprite` "/Game/ProjectContents/Spites/Cafeteria/bread_Sprite_0.bread_Sprite_0" _asbp_kitchen_items)
      (bind _output_get (set `self.Bread` _asbp_kitchen_items))
      (`/Game/ProjectContents/BP/Objects/BP_KitchenItems.UpdateSprite` _output_get))
    (:`then_1`
      (bind _returnvalue_2 (`|SpawnActorFromClass` (`self.KitchenItems`) (`KismetMathLibrary.MakeTransform` (`self.Ginger SpawnLocation`)) "Undefined" "OverrideRootScale" null null))
      (bind _asbp_kitchen_items_2 (cast `/Game/ProjectContents/BP/Objects/BP_KitchenItems` _returnvalue_2))
      (set `/Game/ProjectContents/BP/Objects/BP_KitchenItems.ItemName` "ginger" _asbp_kitchen_items_2)
      (set `/Game/ProjectContents/BP/Objects/BP_KitchenItems.SelectedSprite` "/Game/ProjectContents/Spites/Cafeteria/ginger_Sprite_0.ginger_Sprite_0" _asbp_kitchen_items_2)
      (bind _output_get_2 (set `self.Ginger` _asbp_kitchen_items_2))
      (`/Game/ProjectContents/BP/Objects/BP_KitchenItems.UpdateSprite` _output_get_2))
    (:`then_2`
      (bind _returnvalue_3 (`|SpawnActorFromClass` (`self.KitchenItems`) (`KismetMathLibrary.MakeTransform` (`self.Noodle SpawnLocation`)) "Undefined" "OverrideRootScale" null null))
      (bind _asbp_kitchen_items_3 (cast `/Game/ProjectContents/BP/Objects/BP_KitchenItems` _returnvalue_3))
      (set `/Game/ProjectContents/BP/Objects/BP_KitchenItems.ItemName` "noodle" _asbp_kitchen_items_3)
      (set `/Game/ProjectContents/BP/Objects/BP_KitchenItems.SelectedSprite` "/Game/ProjectContents/Spites/Cafeteria/noodle_Sprite_0.noodle_Sprite_0" _asbp_kitchen_items_3)
      (bind _output_get_3 (set `self.Noodle` _asbp_kitchen_items_3))
      (`/Game/ProjectContents/BP/Objects/BP_KitchenItems.UpdateSprite` _output_get_3))
    (:`then_3`
      (bind _returnvalue_4 (`|SpawnActorFromClass` (`self.KitchenItems`) (`KismetMathLibrary.MakeTransform` (`self.Sauce SpawnLocation`)) "Undefined" "OverrideRootScale" null null))
      (bind _asbp_kitchen_items_4 (cast `/Game/ProjectContents/BP/Objects/BP_KitchenItems` _returnvalue_4))
      (set `/Game/ProjectContents/BP/Objects/BP_KitchenItems.ItemName` "sauce" _asbp_kitchen_items_4)
      (set `/Game/ProjectContents/BP/Objects/BP_KitchenItems.SelectedSprite` "/Game/ProjectContents/Spites/Cafeteria/sauce_Sprite_0.sauce_Sprite_0" _asbp_kitchen_items_4)
      (bind _output_get_4 (set `self.Sauce` _asbp_kitchen_items_4))
      (`/Game/ProjectContents/BP/Objects/BP_KitchenItems.UpdateSprite` _output_get_4))
    (:`then_4`
      (bind _returnvalue_5 (`GameplayStatics.GetActorOfClass` "/Game/ProjectContents/BP/SceneManager/BP_SceneManager_Scene04_Cafeteria.BP_SceneManager_Scene04_Cafeteria_C"))
      (set `self.SceneManager` _returnvalue_5)
      (`self.SetCurrentNeed`))))

(event `Change Need`
  (bind _result (`/Engine/EditorBlueprintResources/StandardMacros.IncrementInt` (`self.CurrentNeedIndex`))
    (:`  `
      (if (< _result (`KismetArrayLibrary.Array_Length` (`self.Needs`)))
        (`self.SetCurrentNeed`)
        (else
          (`self.Handle Finish`))))))

(event `Handle Finish`
  (`PaperSpriteComponent.SetSprite` (`self.PaperSprite`) null)
  (`KismetSystemLibrary.Delay` 2.0)
  (`PaperSpriteComponent.SetSprite` (`self.PaperSprite`) "/Game/ProjectContents/Spites/Cafeteria/yakisobapan_Sprite_0.yakisobapan_Sprite_0")
  (`KismetSystemLibrary.Delay` 2.0)
  (`SceneComponent.SetVisibility` (`self.PaperSprite`) false false))

(event `self.Box.OnComponentBeginOverlap`
  (params (OverlappedComponent :type "PrimitiveComponent Object Reference") (OtherActor :type "Actor Object Reference") (OtherComp :type "PrimitiveComponent Object Reference") (OtherBodyIndex :type Integer) (bFromSweep :type Boolean) (SweepResult :type "HitResult Structure (by ref)"))
  (cast `/Game/ProjectContents/BP/Player/BP_PawnPlayerBase` OtherActor)
  (`self.EnableInput` (`GameplayStatics.GetPlayerController` 0)))

(event `InputAction|Interact`
  (params (Key :type "Key Structure"))
  (bind _textrender (`self.TextRender`))
  (:`Pressed`
    (if (and (>= (`KismetArrayLibrary.Array_Find` (`self.Inventory`) "noodle") 0) (>= (`KismetArrayLibrary.Array_Find` (`self.Inventory`) "sauce") 0))
      (`self.Handle Yakisoba`)
      (elif (>= (`KismetArrayLibrary.Array_Find` (`self.Inventory`) (`self.CurrentNeed`)) 0)
        (`self.Change Need`)
        (`SceneComponent.SetVisibility` (`self.TextRender`) false false)
        (else
          (`TextRenderComponent.K2_SetText` _textrender (`KismetTextLibrary.Conv_StringToText` (`KismetStringLibrary.Concat_StrStr` "I need " (`self.CurrentNeed`))))
          (`SceneComponent.SetVisibility` _textrender true false))))))

(event `self.Box.OnComponentEndOverlap`
  (params (OverlappedComponent :type "PrimitiveComponent Object Reference") (OtherActor :type "Actor Object Reference") (OtherComp :type "PrimitiveComponent Object Reference") (OtherBodyIndex :type Integer))
  (cast `/Game/ProjectContents/BP/Player/BP_PawnPlayerBase` OtherActor)
  (`self.DisableInput` (`GameplayStatics.GetPlayerController` 0)))

(fn `SetCurrentNeed`
  (bind _output_get (set `self.CurrentNeed` (`|GetArrayItem` (`self.Needs`) (`self.CurrentNeedIndex`))))
  (switch `string` _output_get
    (:`bread`
      (`PaperSpriteComponent.SetSprite` (`self.PaperSprite`) "/Game/ProjectContents/Spites/Cafeteria/bread_Sprite_0.bread_Sprite_0"))
    (:`yakisoba`
      (`PaperSpriteComponent.SetSprite` (`self.PaperSprite`) "/Game/ProjectContents/Spites/Cafeteria/yakisoba_Sprite.yakisoba_Sprite"))
    (:`ginger`
      (`PaperSpriteComponent.SetSprite` (`self.PaperSprite`) "/Game/ProjectContents/Spites/Cafeteria/ginger_Sprite_0.ginger_Sprite_0"))))

(fn `UserConstructionScript`)