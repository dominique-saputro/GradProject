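; Level-placed follow camera that becomes player 0's view target on BeginPlay and tracks ActorToFollow in X and Y at a fixed height.
; Each Tick, GetNewX and GetNewY clamp the target's position to min/max bounds, with an offset added on Y, then the actor moves there without smoothing.
; The construction script pre-aligns only X to a valid target, unclamped.
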(event `self.ReceiveBeginPlay`
  ;[1 1 1] Set Camera
  (`PlayerController.SetViewTargetWithBlend` (`GameplayStatics.GetPlayerController` 0) self 0.0 "VTBlend_EaseInOut" 0.0 false))

(event `self.ReceiveTick`
  (params (DeltaSeconds :type "Float (single-precision)"))
  ;[1 1 1] Adjust camera to player location
  (bind _newcamerax (`self.GetNewX`))
  (set `self.CameraX` _newcamerax)
  (bind _newcameray (`self.GetNewY`))
  (set `self.CameraY` _newcameray)
  (`self.K2_SetActorLocation` (`KismetMathLibrary.MakeVector` (`self.CameraX`) (`self.CameraY`) (`self.CameraZ-Fixed`))))

(fn `GetNewX`
  (returns (NewCameraX :type "Float (double-precision)"))
  (bind _returnvalue_x (`KismetMathLibrary.BreakVector` (`self.K2_GetActorLocation` (`self.ActorToFollow`))))
  (bind _returnvalue_x_2 (`KismetMathLibrary.BreakVector` (`self.K2_GetActorLocation` (`self.ActorToFollow`))))
  (if (< _returnvalue_x_2 (`self.MinCameraX`))
    (return (`self.MinCameraX`))
    (elif (> _returnvalue_x (`self.MaxCameraX`))
      (return (`self.MaxCameraX`))
      (else
        (return _returnvalue_x)))))

(fn `GetNewY`
  (returns (NewCameraY :type "Float (double-precision)"))
  (bind (_returnvalue_x _returnvalue_y) (`KismetMathLibrary.BreakVector` (`self.K2_GetActorLocation` (`self.ActorToFollow`))))
  (bind (_returnvalue_x_2 _returnvalue_y_2) (`KismetMathLibrary.BreakVector` (`self.K2_GetActorLocation` (`self.ActorToFollow`))))
  (bind _returnvalue (+ _returnvalue_y (`self.CameraYOffset`)))
  (if (< (+ _returnvalue_y_2 (`self.CameraYOffset`)) (`self.MinCameraY`))
    (return (`self.MinCameraY`))
    (elif (> _returnvalue (`self.MaxCameraY`))
      (return (`self.MaxCameraY`))
      (else
        (return _returnvalue)))))

(fn `UserConstructionScript`
  (bind _actortofollow (`self.ActorToFollow`))
  (bind _returnvalue_x (`KismetMathLibrary.BreakVector` (`self.K2_GetActorLocation` _actortofollow)))
  (`/Engine/EditorBlueprintResources/StandardMacros.IsValid` _actortofollow
    (:`Is Valid`
      (bind _output_get (set `self.CameraX` _returnvalue_x))
      (`self.K2_SetActorLocation` (`KismetMathLibrary.MakeVector` _output_get (`self.CameraY`) (`self.CameraZ-Fixed`))))))