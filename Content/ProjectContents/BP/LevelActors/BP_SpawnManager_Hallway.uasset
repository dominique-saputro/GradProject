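; Level manager for the hallway that sets up its exits, music and player start position.
; On BeginPlay it spawns the LevelActors and configures them as BP_MoveLevels exits to the classroom, cafeteria and upstairs staff hallway by array index.
; CheckScene then destroys the upstairs or cafeteria exit depending on the game instance's CurrentScene.
; It also starts the hallway music and moves the player pawn to a position matching PreviousRoom.
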(event `self.ReceiveBeginPlay`
  (`self.LevelSetup`)
  (`self.CheckScene`)
  (`GameplayStatics.PlaySound2D` "/Game/ProjectContents/Music/BGM_HallwayClassroom.BGM_HallwayClassroom" 1.0 1.0 2.0 null null)
  (bind _asbp_game_instance (cast `/Game/ProjectContents/BP/BP_GameInstance` (`GameplayStatics.GetGameInstance`)))
  (switch `string` (`/Game/ProjectContents/BP/BP_GameInstance.PreviousRoom` _asbp_game_instance)
    (:`Classroom`
      (set `self.PlayerStart` (1125.0 10.0 360.0)))
    (:`Cafeteria`
      (set `self.PlayerStart` (2600.0 10.0 360.0)))
    (:`UpstairsHallway`
      (set `self.PlayerStart` (2610.0 10.0 360.0))))
  (`self.K2_SetActorLocation` (`GameplayStatics.GetPlayerPawn` 0) (`self.PlayerStart`) false false))

(event `CheckScene`
  (bind _asbp_game_instance (cast `/Game/ProjectContents/BP/BP_GameInstance` (`GameplayStatics.GetGameInstance`)))
  (if (< (`/Game/ProjectContents/BP/BP_GameInstance.CurrentScene` _asbp_game_instance) 5)
    (`self.K2_DestroyActor` (`|GetArrayItem` (`self.MoveLevelActors`) 2))
    (else
      (`self.K2_DestroyActor` (`|GetArrayItem` (`self.MoveLevelActors`) 1)))))

(fn `LevelSetup`
  (for (_array_element _array_index) (`self.LevelActors`)
    (bind _returnvalue (`|SpawnActorFromClass` _array_element (`|GetArrayItem` (`self.ActorSpawns`) _array_index) "Undefined" "OverrideRootScale" null null))
    (`KismetArrayLibrary.Array_Add` (`self.MoveLevelActors`) _returnvalue))
  (for (_array_element_2 _array_index_2) (`self.MoveLevelActors`)
    (switch `int` _array_index_2
      (:`0`
        (set `self.Tool Tip Text` "Go to classroom")
        (set `self.Level to Load` "Game_Classroom"))
      (:`1`
        (set `self.Tool Tip Text` "Go to cafeteria")
        (set `self.Level to Load` "Game_Cafeteria"))
      (:`2`
        (set `self.Tool Tip Text` "Go upstairs")
        (set `self.Level to Load` "Game_Staff_Hallway")))
    (bind _asbp_move_levels (cast `/Game/ProjectContents/BP/LevelActors/BP_MoveLevels` _array_element_2))
    (set `/Game/ProjectContents/BP/LevelActors/BP_MoveLevels.CurrentRoom` "Hallway" _asbp_move_levels)
    (set `/Game/ProjectContents/BP/LevelActors/BP_MoveLevels.ToolTipText` (`self.Tool Tip Text`) _asbp_move_levels)
    (set `/Game/ProjectContents/BP/LevelActors/BP_MoveLevels.LevelToLoad` (`self.Level to Load`) _asbp_move_levels)))

(fn `UserConstructionScript`)