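; Base player pawn with a Paper2D flipbook character, moved along world X and Y by axis input.
; BeginPlay sets movement speed, replicates the flipbook and adds the bottle UI unless the GameInstance's current scene is 1.
; Tick picks walk or idle animation from velocity and flips sprite yaw by X velocity, using the last input direction when still.
; Events toggle player input, and a test action calls a part-and-scene check.
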(event `self.ReceiveBeginPlay`
  (`ActorComponent.SetIsReplicated` (`self.PaperFlipbook`) true)
  (set `FloatingPawnMovement.MaxSpeed` (`self.MaxSpeed`) (`self.PawnMovement`))
  (bind _asbp_game_instance (cast `/Game/ProjectContents/BP/BP_GameInstance` (`GameplayStatics.GetGameInstance`)))
  (if (not (== (`/Game/ProjectContents/BP/BP_GameInstance.CurrentScene` _asbp_game_instance) 1))
    (bind _returnvalue (`|CreateWidget` "/Game/ProjectContents/BP/Widgets/WBP_BottleUI.WBP_BottleUI_C" (`GameplayStatics.GetPlayerController` 0)))
    (`UserWidget.AddToViewport` _returnvalue 0)))

(event `UpdateAnim`
  ;[1 1 1] Handle Animation
  (if (> (`KismetMathLibrary.VSize` (`self.GetVelocity`)) 0.0)
    (`PaperFlipbookComponent.SetFlipbook` (`self.PaperFlipbook`) (`self.Walk FlipBook`))
    (else
      (`PaperFlipbookComponent.SetFlipbook` (`self.PaperFlipbook`) (`self.Idle FlipBook`)))))

(event `InputAxis|Move Forward / Backward`
  (params (AxisValue :type "Float (single-precision)"))
  ;[1 1 1] Handle movement - ForwardBackward
  (if (not (== AxisValue 0.0))
    (`self.AddMovementInput` (0.0 1.0 0.0) AxisValue)))

(event `self.ReceiveTick`
  (params (DeltaSeconds :type "Float (single-precision)"))
  ;[1 1 1] Tick - Updates animation
  (`self.UpdateAnim`)
  (`/Engine/EditorBlueprintResources/StandardMacros.CompareFloat` (.x (`MovementComponent.Velocity` (`self.GetMovementComponent`)))
    (:`>`
      (`/Engine/EditorBlueprintResources/StandardMacros.IsValid` (`self.GetController`) :!label _label
        (:`Is Valid`
          (`SceneComponent.K2_SetRelativeRotation` (`self.PaperFlipbook`) (`KismetMathLibrary.MakeRotator` 0.0) false false))))
    (:`==`
      (if (`self.bisMovingRight`)
        (goto _label)
        (else
          (`/Engine/EditorBlueprintResources/StandardMacros.IsValid` (`self.GetController`) :!label _label_2
            (:`Is Valid`
              (`SceneComponent.K2_SetRelativeRotation` (`self.PaperFlipbook`) (`KismetMathLibrary.MakeRotator` 0.0 0.0 180.0) false false))))))
    (:`<`
      (goto _label_2))))

(event `InputAxis|Move Right / Left`
  (params (AxisValue :type "Float (single-precision)"))
  ;[1 1 1] Handle movement
  (if (> AxisValue 0.0)
    (set `self.bisMovingRight` true)
    (elif (< AxisValue 0.0)
      (set `self.bisMovingRight` false)))
  (`self.AddMovementInput` (1.0 0.0 0.0) AxisValue))

(event `DisableMovement`
  (`self.DisableInput` (`GameplayStatics.GetPlayerController` 0)))

(event `InputAction|TestInput`
  (params (Key :type "Key Structure"))
  (:`Pressed`
    (`/Game/ProjectContents/BP/BP_FunctionLib.CheckCurrrentPart and Scene`)))

(event `EnableMovement`
  (`self.EnableInput` (`GameplayStatics.GetPlayerController` 0)))

(fn `UserConstructionScript`)