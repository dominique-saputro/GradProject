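; Scene manager for the Scene 02 classroom story sequence, spawning actors, sorting NPCs by tag and opening with a locker cutscene.
; Interact cycles BP_DialogManager lines, then MoveToNextPart switches on CurrentPart to run numbered dialog beats.
; Event handlers stage camera pans through a dummy follow target and paper-ball reactions.
; The sister's exit spawns a tear drop, whose pickup advances the GameInstance scene, fades out and loads Game_Classroom.
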(event `self.ReceiveBeginPlay`
  (bind _returnvalue (`GameplayStatics.GetActorOfClass` "/Game/ProjectContents/BP/LevelActors/BP_DialogManager.BP_DialogManager_C"))
  (set `self.LevelDialogManager` _returnvalue)
  (bind _iscorrectscene (`/Game/ProjectContents/BP/BP_FunctionLib.CheckSceneIndex` (`self.CurrentScene`)))
  (if _iscorrectscene
    (`self.Level Setup`)
    (`self.LockerScene`)))

(event `LockerScene`
  (bind _returnvalue (`GameplayStatics.GetPlayerController` 0))
  ;[1 1 1] LockerScene
  (`self.DisableInput` (`GameplayStatics.GetPlayerPawn` 0) _returnvalue)
  (bind _returnvalue_2 (`|CreateWidget` "/Game/ProjectContents/BP/Widgets/WBP_LockerCutscene.WBP_LockerCutscene_C" _returnvalue))
  (`UserWidget.AddToViewport` _returnvalue_2 0)
  (`KismetSystemLibrary.Delay` 3.0)
  (`KismetSystemLibrary.PrintString` "PlayLockerSound")
  (`KismetSystemLibrary.Delay` 2.0)
  (`KismetSystemLibrary.PrintString` "PlayLockerSound")
  (`KismetSystemLibrary.Delay` 3.0)
  (`KismetSystemLibrary.PrintString` "Movement enable")
  (`self.EnableInput` (`GameplayStatics.GetPlayerPawn` 0) (`GameplayStatics.GetPlayerController` 0))
  (`self.Part0`))

(event `Handle PlayerDialog1`
  ;[1 1 1] Handle Player Dialog1
  (`/Game/ProjectContents/BP/LevelActors/BP_DialogManager.Display Dialog` (`self.LevelDialogManager`) (`GameplayStatics.GetPlayerPawn` 0) (`self.Player1`) (`self.TextDelay`)))

(event `InputAction|Interact`
  (params (Key :type "Key Structure"))
  ;[1 1 1] OnInteract
  (:`Pressed`
    (if (`/Game/ProjectContents/BP/LevelActors/BP_DialogManager.isDIalogFinished` (`self.LevelDialogManager`))
      (set `/Game/ProjectContents/BP/LevelActors/BP_DialogManager.isDIalogFinished` false (`self.LevelDialogManager`))
      (bind _asbp_game_instance (cast `/Game/ProjectContents/BP/BP_GameInstance` (`GameplayStatics.GetGameInstance`)))
      (set `/Game/ProjectContents/BP/BP_GameInstance.isViewingScene` false _asbp_game_instance)
      (`KismetSystemLibrary.PrintString` "DialogFinished")
      (`self.MoveToNextPart`)
      (else
        (`/Game/ProjectContents/BP/LevelActors/BP_DialogManager.Test-CycleOnKey` (`self.LevelDialogManager`))))))

(event `Handle Change Camera`
  (bind _returnvalue (`self.K2_GetActorLocation` (`GameplayStatics.GetPlayerPawn` 0)))
  ;[1 1 1] Handle Switch Player with Dummy Actor
  (bind _returnvalue_2 (`|SpawnActorFromClass` "/Game/ProjectContents/BP/Objects/BP_DummyActor.BP_DummyActor_C" (`KismetMathLibrary.MakeTransform` _returnvalue) "Undefined" "OverrideRootScale" null null))
  (bind _returnvalue_3 (`GameplayStatics.GetActorOfClass` "/Game/ProjectContents/BP/LevelActors/BP_FollowCamera.BP_FollowCamera_C"))
  (set `/Game/ProjectContents/BP/LevelActors/BP_FollowCamera.ActorToFollow` _returnvalue_2 _returnvalue_3)
  (`KismetSystemLibrary.PrintString` "Switched ActorToFollow")
  (set `self.CameraStart` _returnvalue)
  (set `self.CameraEnd` (+ _returnvalue (300.0 0.0 0.0)))
  (`self.HandleMoveCameraRight`))

(event `Part0`
  (bind _leveldialogmanager (`self.LevelDialogManager`))
  ;[1 1 1] Part0 - PLayer DIalog
  (`/Game/ProjectContents/BP/BP_FunctionLib.SetupDialogManagerCycle` _leveldialogmanager (`GameplayStatics.GetPlayerPawn` 0) (`self.Player1`) self)
  (`/Game/ProjectContents/BP/LevelActors/BP_DialogManager.Test-CycleOnKey` _leveldialogmanager))

(event `HandleMoveCameraRight`
  ;[1 1 1] Handle Move CAmera Right
  (bind _returnvalue (`GameplayStatics.GetActorOfClass` "/Game/ProjectContents/BP/Objects/BP_DummyActor.BP_DummyActor_C"))
  (bind (_direction _alpha) (`Timeline|Timeline_0` :!via `PlayFromStart`)
    (:`Update`
      (`self.K2_SetActorLocation` _returnvalue (`KismetMathLibrary.VLerp` (`self.CameraStart`) (`self.CameraEnd`) _alpha) false false))
    (:`Finished`
      (`KismetSystemLibrary.Delay` 2.0)
      (`self.Part1`))))

(event `Part1`
  (`/Game/ProjectContents/BP/BP_FunctionLib.SetupDialogManagerCycle` (`self.LevelDialogManager`) (`self.TeacherActor`) (`self.Teacher1`) self))

(event `Part2`
  (`/Game/ProjectContents/BP/BP_FunctionLib.SetupDialogManagerCycle` (`self.LevelDialogManager`) (`GameplayStatics.GetPlayerPawn` 0) (`self.Player2`) self)
  (`KismetSystemLibrary.PrintString` "Part2 Set"))

(event `Part3`
  (`/Game/ProjectContents/BP/BP_FunctionLib.Flip FlipBook` (`self.TeacherActor`))
  (bind _dialog_delay (`/Game/ProjectContents/BP/LevelActors/BP_DialogManager.Display Dialog` (`self.LevelDialogManager`) (`self.TeacherActor`) (`self.Teacher2`) (`self.TextDelay`)))
  (`KismetSystemLibrary.Delay` _dialog_delay)
  (`/Game/ProjectContents/BP/BP_FunctionLib.SetupDialogManagerCycle` (`self.LevelDialogManager`) (`self.TeacherActor`) (`self.Teacher3`) self)
  (`KismetSystemLibrary.PrintString` "Part3 Set")
  (`GameplayStatics.PlaySound2D` "/Game/ProjectContents/SFX/SFX_StudentsLaugh.SFX_StudentsLaugh" 1.0 1.0 0.0 null null))

(event `Handle PlayerDialog2`
  ;[1 1 1] Handle PlayerDialog2
  (bind _dialog_delay (`/Game/ProjectContents/BP/LevelActors/BP_DialogManager.Display Dialog` (`self.LevelDialogManager`) (`GameplayStatics.GetPlayerPawn` 0) (`self.Player2`) (`self.TextDelay`)))
  (`KismetSystemLibrary.Delay` (/ _dialog_delay 2.0))
  (`self.HandleMOveCameraLeft`))

(event `HandleMOveCameraLeft`
  ;[1 1 1] Handle Move Camera Left
  (bind _returnvalue (`GameplayStatics.GetActorOfClass` "/Game/ProjectContents/BP/Objects/BP_DummyActor.BP_DummyActor_C"))
  (bind (_direction _alpha) (`Timeline|Timeline_1` :!via `PlayFromStart`)
    (:`Update`
      (`self.K2_SetActorLocation` _returnvalue (`KismetMathLibrary.VLerp` (`self.CameraEnd`) (`self.CameraStart`) _alpha) false false))
    (:`Finished`
      (bind _returnvalue_2 (`GameplayStatics.GetActorOfClass` "/Game/ProjectContents/BP/LevelActors/BP_FollowCamera.BP_FollowCamera_C"))
      (set `/Game/ProjectContents/BP/LevelActors/BP_FollowCamera.ActorToFollow` (`GameplayStatics.GetPlayerPawn` 0) _returnvalue_2)
      (`self.EnableInput` (`GameplayStatics.GetPlayerPawn` 0) (`GameplayStatics.GetPlayerController` 0)))))

(event `Part4`
  (`/Game/ProjectContents/BP/BP_FunctionLib.SetupDialogManagerCycle` (`self.LevelDialogManager`) (`self.BigSisterActor`) (`self.BisSister`) self)
  (`KismetSystemLibrary.PrintString` "Part4 Set"))

(event `Part5`
  (`/Game/ProjectContents/BP/BP_FunctionLib.SetupDialogManagerCycle` (`self.LevelDialogManager`) (`self.TeacherActor`) (`self.Teacher4`) self)
  (`KismetSystemLibrary.PrintString` "Part5 Set"))

(event `Handle Student Dialog`
  ;[1 1 1] Handle Sttudent Dialog
  (`self.DisableInput` (`GameplayStatics.GetPlayerPawn` 0) (`GameplayStatics.GetPlayerController` 0))
  (for _index (range 3)
    (`/Game/ProjectContents/BP/LevelActors/BP_DialogManager.DisplayTextOnce` (`self.LevelDialogManager`) (`|GetArrayItem` (`self.StudentNPCs`) _index) (`self.Student`) (`self.TextDelay`)))
  (`KismetSystemLibrary.Delay` (`self.TextDelay`))
  (for _index_2 (range 3)
    (`/Game/ProjectContents/BP/LevelActors/BP_DialogManager.Remove Display Text` (`self.LevelDialogManager`) (`|GetArrayItem` (`self.StudentNPCs`) _index_2))))

(event `Part6`
  (bind _asbp_npcactor_big_sister (cast `/Game/ProjectContents/BP/NPC/BP_NPCActor_BigSister` (`self.BigSisterActor`)))
  (`/Game/ProjectContents/BP/NPC/BP_NPCActorBase.MoveNPC Event` _asbp_npcactor_big_sister (`self.SisterStart`) (`self.SisterEnd`))
  (`KismetSystemLibrary.Delay` 4.0)
  (`self.K2_DestroyActor` (`self.BigSisterActor`))
  (`self.Handle Tear Drop Spawn`))

(event `HandlePaperBallThrowFinished`
  ;[1 1 1] Handle Teacher After Paper Ball
  (`/Game/ProjectContents/BP/BP_FunctionLib.Flip FlipBook` (`self.TeacherActor`))
  (bind _dialog_delay (`/Game/ProjectContents/BP/LevelActors/BP_DialogManager.Display Dialog` (`self.LevelDialogManager`) (`self.TeacherActor`) (`self.Teacher2`) (`self.TextDelay`)))
  (`KismetSystemLibrary.Delay` _dialog_delay)
  (`/Game/ProjectContents/BP/BP_FunctionLib.Flip FlipBook` (`self.TeacherActor`))
  (`self.HandleSisterDialog`)
  (`GameplayStatics.PlaySound2D` "/Game/ProjectContents/SFX/SFX_StudentsLaugh.SFX_StudentsLaugh" 1.0 1.0 0.0 null null))

(event `HandleSisterDialog`
  ;[1 1 1] Handle Sister
  (bind _dialog_delay (`/Game/ProjectContents/BP/LevelActors/BP_DialogManager.Display Dialog` (`self.LevelDialogManager`) (`self.BigSisterActor`) (`self.BisSister`) (`self.TextDelay`)))
  (`KismetSystemLibrary.Delay` _dialog_delay)
  (bind _asbp_npcactor_big_sister (cast `/Game/ProjectContents/BP/NPC/BP_NPCActor_BigSister` (`self.BigSisterActor`)))
  (`/Game/ProjectContents/BP/NPC/BP_NPCActorBase.MoveNPC Event` _asbp_npcactor_big_sister (`self.SisterStart`) (`self.SisterEnd`))
  (`KismetSystemLibrary.Delay` 4.0)
  (`self.K2_DestroyActor` (`self.BigSisterActor`))
  (`self.Handle Tear Drop Spawn`))

(event `Handle Tear Drop Spawn`
  ;[1 1 1] Spawn Tear Drop
  (`|SpawnActorFromClass` "/Game/ProjectContents/BP/Objects/BP_TearDrop.BP_TearDrop_C" (`KismetMathLibrary.MakeTransform` (`self.TearDropSpawn`)) "Undefined" "OverrideRootScale" null null)
  (`self.EnableInput` (`GameplayStatics.GetPlayerPawn` 0) (`GameplayStatics.GetPlayerController` 0)))

(event `Handle End Scene`
  (bind _returnvalue (`|CreateWidget` "/Game/ProjectContents/BP/Widgets/WBP_FadeBlack.WBP_FadeBlack_C" (`GameplayStatics.GetPlayerController` 0)))
  (`UserWidget.AddToViewport` _returnvalue 0)
  (`/Game/ProjectContents/BP/Widgets/WBP_FadeBlack.FadeToBlack` _returnvalue)
  (`KismetSystemLibrary.Delay` 0.5)
  (`GameplayStatics.OpenLevel` "Game_Classroom"))

(fn `Get NPCs In Level`
  (returns (`Level NPCs` :type "Array of Actor Object Reference"))
  (bind _outactors (`GameplayStatics.GetAllActorsOfClass` "/Game/ProjectContents/BP/NPC/BP_NPCActorBase.BP_NPCActorBase_C"))
  (return _outactors))

(fn `Level Setup`
  (for (_array_element _array_index) (`self.LevelActors`)
    (`|SpawnActorFromClass` _array_element (`|GetArrayItem` (`self.ActorsSpawn`) _array_index) "Undefined" "OverrideRootScale" null null))
  (`self.K2_SetActorLocation` (`GameplayStatics.GetPlayerPawn` 0) (`self.PlayerSpawn`) false false)
  (bind _level_npcs (`self.Get NPCs In Level`))
  (for _array_element_2 _level_npcs
    (if (`self.ActorHasTag` _array_element_2 "Student")
      (`KismetArrayLibrary.Array_Add` (`self.StudentNPCs`) _array_element_2)
      (elif (`self.ActorHasTag` _array_element_2 "Teacher")
        (set `self.TeacherActor` _array_element_2)
        (else
          (set `self.BigSisterActor` _array_element_2)))))
  (bind _asbp_game_instance (cast `/Game/ProjectContents/BP/BP_GameInstance` (`GameplayStatics.GetGameInstance`)))
  (set `/Game/ProjectContents/BP/BP_GameInstance.isViewingScene` true _asbp_game_instance)
  (bind _result (`/Engine/EditorBlueprintResources/StandardMacros.DecrementInt` (`KismetArrayLibrary.Array_Length` (`self.StudentNPCs`)))
    (:`  `
      (for _index (range (+ _result 1))
        (bind _asbp_npcactor_base (cast `/Game/ProjectContents/BP/NPC/BP_NPCActorBase` (`|GetArrayItem` (`self.StudentNPCs`) _index)))
        (`/Game/ProjectContents/BP/NPC/BP_NPCActorBase.SetFlipbookSit` _asbp_npcactor_base))
      (`GameplayStatics.PlaySound2D` "/Game/ProjectContents/Music/BGM_QuietClassroom.BGM_QuietClassroom" 2.0 1.0 0.0 null null))))

(fn `MoveToNextPart`
  (`self.DisableInput` (`GameplayStatics.GetPlayerController` 0))
  (bind _result (`/Engine/EditorBlueprintResources/StandardMacros.IncrementInt` (`self.CurrentPart`))
    (:`  `
      (switch `int` _result
        (:`1`
          (`self.Part1`))
        (:`2`
          (`self.Part2`))
        (:`3`
          (`self.HandleMOveCameraLeft`))
        (:`4`
          (`self.Part4`))
        (:`5`
          (`self.Part5`))
        (:`6`
          (`self.Part6` :!label _label))
        (:`7`
          (goto _label))))))

(fn `OnTearDropPickUp`
  (bind _asbp_game_instance (cast `/Game/ProjectContents/BP/BP_GameInstance` (`GameplayStatics.GetGameInstance`)))
  (`/Game/ProjectContents/BP/BP_GameInstance.MoveToNextScene` _asbp_game_instance)
  (`self.Handle End Scene`))

(fn `UserConstructionScript`)