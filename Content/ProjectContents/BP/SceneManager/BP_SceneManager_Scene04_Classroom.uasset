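; Scene manager for the Scene 4 classroom cutscene, a scripted conversation between three students and the Big Sister.
; If the scene index check passes, BeginPlay spawns the cast, seats the students, hides the sister, starts music and places the player.
; Interact cycles dialog or, once finished, advances a GameInstance-tracked part counter through hard-coded Part events.
; The sister appears midway, and the last part sets progress flags, walks her out and restores input.
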(event `self.ReceiveBeginPlay`
  (bind _iscorrectscene (`/Game/ProjectContents/BP/BP_FunctionLib.CheckSceneIndex` (`self.CurrentScene`)))
  (if _iscorrectscene
    (`self.LevelSetup`)
    (bind _returnvalue (`GameplayStatics.GetActorOfClass` "/Game/ProjectContents/BP/LevelActors/BP_DialogManager.BP_DialogManager_C"))
    (set `self.Level Dialog Manager` _returnvalue)))

(event `InputAction|Interact`
  (params (Key :type "Key Structure"))
  ;[1 1 1] OnInteract
  (:`Pressed`
    (bind _asbp_game_instance (cast `/Game/ProjectContents/BP/BP_GameInstance` (`GameplayStatics.GetGameInstance`)))
    (if (`/Game/ProjectContents/BP/BP_GameInstance.isViewingScene` _asbp_game_instance)
      (if (`/Game/ProjectContents/BP/LevelActors/BP_DialogManager.isDIalogFinished` (`self.Level Dialog Manager`))
        (set `/Game/ProjectContents/BP/LevelActors/BP_DialogManager.isDIalogFinished` false (`self.Level Dialog Manager`))
        (bind _asbp_game_instance_2 (cast `/Game/ProjectContents/BP/BP_GameInstance` (`GameplayStatics.GetGameInstance`)))
        (set `/Game/ProjectContents/BP/BP_GameInstance.isViewingScene` false _asbp_game_instance_2)
        (`KismetSystemLibrary.PrintString` "DialogFinished")
        (`self.MoveToNextPart`)
        (else
          (`/Game/ProjectContents/BP/LevelActors/BP_DialogManager.Test-CycleOnKey` (`self.Level Dialog Manager`)))))))

(event `Handle Dialog Start`
  ;[1 1 1] Handle Start Dialog
  (bind _dialog_delay (`/Game/ProjectContents/BP/LevelActors/BP_DialogManager.Display Dialog` (`self.Level Dialog Manager`) (`|GetArrayItem` (`self.Students`)) (`self.StudentA`) (`self.TextDelay`)))
  (`KismetSystemLibrary.Delay` _dialog_delay)
  (bind _dialog_delay_2 (`/Game/ProjectContents/BP/LevelActors/BP_DialogManager.Display Dialog` (`self.Level Dialog Manager`) (`|GetArrayItem` (`self.Students`) 1) (`self.StudentB`) (`self.TextDelay`)))
  (`KismetSystemLibrary.Delay` _dialog_delay_2)
  (bind _dialog_delay_3 (`/Game/ProjectContents/BP/LevelActors/BP_DialogManager.Display Dialog` (`self.Level Dialog Manager`) (`|GetArrayItem` (`self.Students`) 2) (`self.StudentC`) (`self.TextDelay`)))
  (`KismetSystemLibrary.Delay` _dialog_delay_3)
  (`self.Handle SIster Leave`))

(event `Part0`
  (`/Game/ProjectContents/BP/BP_FunctionLib.SetupDialogManagerCycle` (`self.Level Dialog Manager`) (`|GetArrayItem` (`self.Students`) 1) (`self.StudentB`) self))

(event `Handle SIster Leave`
  (bind _bigsister (`self.BigSister`))
  ;[1 1 1] Handle Sister
  (`/Game/ProjectContents/BP/BP_FunctionLib.Flip FlipBook` _bigsister)
  (bind _asbp_npcactor_big_sister (cast `/Game/ProjectContents/BP/NPC/BP_NPCActor_BigSister` _bigsister))
  (`/Game/ProjectContents/BP/NPC/BP_NPCActorBase.MoveNPC Event` _asbp_npcactor_big_sister (`self.K2_GetActorLocation` _bigsister) (`self.PlayerSpawn`))
  (`KismetSystemLibrary.Delay` 3.0)
  (`self.K2_DestroyActor` _bigsister)
  (`/Game/ProjectContents/BP/BP_FunctionLib.EnablePlayerInput`))

(event `Part1`
  (`/Game/ProjectContents/BP/BP_FunctionLib.SetupDialogManagerCycle` (`self.Level Dialog Manager`) (`|GetArrayItem` (`self.Students`) 2) (`self.StudentC`) self))

(event `Part2`
  (bind _bigsister (`self.BigSister`))
  (bind _asbp_npcactor_big_sister (cast `/Game/ProjectContents/BP/NPC/BP_NPCActor_BigSister` _bigsister))
  (`/Game/ProjectContents/BP/NPC/BP_NPCActor_BigSister.SetVisibilityTrue` _asbp_npcactor_big_sister)
  (`/Game/ProjectContents/BP/BP_FunctionLib.Flip FlipBook` _asbp_npcactor_big_sister)
  (`/Game/ProjectContents/BP/NPC/BP_NPCActorBase.MoveNPC Event` _asbp_npcactor_big_sister (`self.K2_GetActorLocation` _bigsister) (`self.SisterEnd`))
  (`KismetSystemLibrary.Delay` 2.0)
  (`/Game/ProjectContents/BP/BP_FunctionLib.SetupDialogManagerCycle` (`self.Level Dialog Manager`) (`|GetArrayItem` (`self.Students`)) (`self.StudentA`) self))

(event `Part3`
  (`/Game/ProjectContents/BP/BP_FunctionLib.SetupDialogManagerCycle` (`self.Level Dialog Manager`) (`|GetArrayItem` (`self.Students`) 1) (`self.StudentB1`) self))

(event `Part4`
  (`/Game/ProjectContents/BP/BP_FunctionLib.SetupDialogManagerCycle` (`self.Level Dialog Manager`) (`|GetArrayItem` (`self.Students`) 2) (`self.StudentC1`) self))

(event `Part5`
  (`/Game/ProjectContents/BP/BP_FunctionLib.SetupDialogManagerCycle` (`self.Level Dialog Manager`) (`self.BigSister`) (`self.Big Sister`) self))

(event `Part6`
  (`/Game/ProjectContents/BP/BP_FunctionLib.SetupDialogManagerCycle` (`self.Level Dialog Manager`) (`|GetArrayItem` (`self.Students`)) (`self.StudentA1`) self))

(event `Part7`
  (`/Game/ProjectContents/BP/BP_FunctionLib.SetupDialogManagerCycle` (`self.Level Dialog Manager`) (`self.BigSister`) (`self.Big Sister1`) self))

(event `Part8`
  (`/Game/ProjectContents/BP/BP_FunctionLib.SetupDialogManagerCycle` (`self.Level Dialog Manager`) (`|GetArrayItem` (`self.Students`) 1) (`self.StudentB2`) self))

(event `Part9`
  (`/Game/ProjectContents/BP/BP_FunctionLib.SetupDialogManagerCycle` (`self.Level Dialog Manager`) (`self.BigSister`) (`self.Big Sister2`) self))

(event `Part10`
  (`/Game/ProjectContents/BP/BP_FunctionLib.SetupDialogManagerCycle` (`self.Level Dialog Manager`) (`|GetArrayItem` (`self.Students`) 2) (`self.StudentC2`) self))

(event `Part11`
  (`/Game/ProjectContents/BP/BP_FunctionLib.DisablePlayerInput`)
  (bind _asbp_game_instance (cast `/Game/ProjectContents/BP/BP_GameInstance` (`GameplayStatics.GetGameInstance`)))
  (set `/Game/ProjectContents/BP/BP_GameInstance.isScene4ClassroomFinished` true _asbp_game_instance)
  (set `/Game/ProjectContents/BP/BP_GameInstance.isScene4ToCafeteriaFinished` false _asbp_game_instance)
  (`self.Handle SIster Leave`))

(fn `LevelSetup`
  (`|ExecutionSequence`
    (:`then_0`
      (for (_array_element _array_index) (`self.LevelActors`)
        (bind _returnvalue (`|SpawnActorFromClass` _array_element (`|GetArrayItem` (`self.ActorSpawns`) _array_index) "Undefined" "OverrideRootScale" null null))
        (if (`self.ActorHasTag` _returnvalue "Student")
          (`KismetArrayLibrary.Array_Add` (`self.Students`) _returnvalue)
          (elif (`self.ActorHasTag` _returnvalue "BigSister")
            (set `self.BigSister` _returnvalue)))))
    (:`then_1`
      (bind _asbp_npcactor_big_sister (cast `/Game/ProjectContents/BP/NPC/BP_NPCActor_BigSister` (`self.BigSister`)))
      (`/Game/ProjectContents/BP/NPC/BP_NPCActor_BigSister.SetVisibilityFalse` _asbp_npcactor_big_sister)
      (bind _result (`/Engine/EditorBlueprintResources/StandardMacros.DecrementInt` (`KismetArrayLibrary.Array_Length` (`self.Students`)))
        (:`  `
          (for _index (range (+ _result 1))
            (bind _asbp_npcactor_base (cast `/Game/ProjectContents/BP/NPC/BP_NPCActorBase` (`|GetArrayItem` (`self.Students`) _index)))
            (`/Game/ProjectContents/BP/NPC/BP_NPCActorBase.SetFlipbookSit` _asbp_npcactor_base)))))
    (:`then_2`
      (`GameplayStatics.PlaySound2D` "/Game/ProjectContents/Music/BGM_HallwayClassroom.BGM_HallwayClassroom" 1.0 1.0 0.0 null null)
      (`self.K2_SetActorLocation` (`GameplayStatics.GetPlayerPawn` 0) (`self.PlayerSpawn`) false false))))

(fn `MoveToNextPart`
  (`self.DisableInput` (`GameplayStatics.GetPlayerController` 0))
  (bind _result (`/Engine/EditorBlueprintResources/StandardMacros.IncrementInt` (`self.CurrentPart`))
    (:`  `
      (bind _asbp_game_instance (cast `/Game/ProjectContents/BP/BP_GameInstance` (`GameplayStatics.GetGameInstance`)))
      (bind _output_get (set `/Game/ProjectContents/BP/BP_GameInstance.ScenePart` _result _asbp_game_instance))
      (switch `int` _output_get
        (:`1`
          (`self.Part1`))
        (:`2`
          (`self.Part2`))
        (:`3`
          (`self.Part3`))
        (:`4`
          (`self.Part4`))
        (:`5`
          (`self.Part5`))
        (:`6`
          (`self.Part6`))
        (:`7`
          (`self.Part7`))
        (:`8`
          (`self.Part8`))
        (:`9`
          (`self.Part9`))
        (:`10`
          (`self.Part10`))
        (:`11`
          (`self.Part11`))))))

(fn `UserConstructionScript`)