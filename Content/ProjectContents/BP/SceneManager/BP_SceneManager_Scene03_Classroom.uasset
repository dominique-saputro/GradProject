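; Scene manager that runs the Scene 3 classroom cutscene, with dialog between a teacher, the big sister and students.
; LevelSetup clears previous scene actors, spawns this scene's cast and sorts NPCs by tag.
; Interact cycles the dialog manager, then MoveToNextPart stores progress in the GameInstance and dispatches numbered Part events for movement and dialog.
; BeginPlay can resume mid-scene from CurrentPart; the final part removes the sister and advances to the next scene.
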(event `self.ReceiveBeginPlay`
  (bind _returnvalue (`GameplayStatics.GetActorOfClass` "/Game/ProjectContents/BP/LevelActors/BP_DialogManager.BP_DialogManager_C"))
  (set `self.Level Dialog Manager` _returnvalue)
  (bind _iscorrectscene (`/Game/ProjectContents/BP/BP_FunctionLib.CheckSceneIndex` (`self.CurrentScene`)))
  (if _iscorrectscene
    (if (== (`self.CurrentPart`) 0)
      (`self.CorrectScene`)
      (bind _returnvalue_2 (`GameplayStatics.SpawnSound2D` "/Game/ProjectContents/Music/BGM_Ken-Classroom.BGM_Ken-Classroom" 1.0 1.0 0.0 null))
      (bind _output_get (set `self.BGM` _returnvalue_2))
      (`AudioComponent.Play` _output_get 0.0)
      (else
        (`/Engine/EditorBlueprintResources/StandardMacros.DecrementInt` (`self.CurrentPart`)
          (:`  `
            (`self.MoveToNextPart`)))))))

(event `InputAction|Interact`
  (params (Key :type "Key Structure"))
  ;[1 1 1] OnInteract
  (:`Pressed`
    (bind _asbp_game_instance (cast `/Game/ProjectContents/BP/BP_GameInstance` (`GameplayStatics.GetGameInstance`)))
    (if (`/Game/ProjectContents/BP/BP_GameInstance.isViewingScene` _asbp_game_instance)
      (if (`/Game/ProjectContents/BP/LevelActors/BP_DialogManager.isDIalogFinished` (`self.Level Dialog Manager`))
        (set `/Game/ProjectContents/BP/LevelActors/BP_DialogManager.isDIalogFinished` false (`self.Level Dialog Manager`))
        (bind _asbp_game_instance_2 (cast `/Game/ProjectContents/BP/BP_GameInstance` (`GameplayStatics.GetGameInstance`)))
        (set `/Game/ProjectContents/BP/BP_GameInstance.isViewingScene` false _asbp_game_instance_2)
        (`self.MoveToNextPart`)
        (else
          (`/Game/ProjectContents/BP/LevelActors/BP_DialogManager.Test-CycleOnKey` (`self.Level Dialog Manager`)))))))

(event `CorrectScene`
  ;[1 1 1] Correct Scene
  (`self.LevelSetup`)
  (bind _returnvalue (`|CreateWidget` "/Game/ProjectContents/BP/Widgets/WBP_FadeBlack.WBP_FadeBlack_C" (`GameplayStatics.GetPlayerController` 0)))
  (`UserWidget.AddToViewport` _returnvalue 0)
  (`/Game/ProjectContents/BP/Widgets/WBP_FadeBlack.FadeFromBlack` _returnvalue)
  (`self.DisableInput` (`GameplayStatics.GetPlayerPawn` 0) (`GameplayStatics.GetPlayerController` 0))
  (`KismetSystemLibrary.Delay` 2.0)
  (`self.Part0`))

(event `Part0`
  (`KismetSystemLibrary.Delay` 2.0)
  (bind _asbp_npcactor_big_sister (cast `/Game/ProjectContents/BP/NPC/BP_NPCActor_BigSister` (`self.BigSisterActor`)))
  (`/Game/ProjectContents/BP/NPC/BP_NPCActor_BigSister.SetVisibilityTrue` _asbp_npcactor_big_sister)
  (`/Game/ProjectContents/BP/BP_FunctionLib.Flip FlipBook` _asbp_npcactor_big_sister)
  (`/Game/ProjectContents/BP/NPC/BP_NPCActorBase.MoveNPC Event` _asbp_npcactor_big_sister (`self.BigSister StartLocation`) (`self.BigSister GoalLocation`))
  (`KismetSystemLibrary.Delay` 3.0)
  (`/Game/ProjectContents/BP/BP_FunctionLib.Flip FlipBook` _asbp_npcactor_big_sister)
  (`/Game/ProjectContents/BP/BP_FunctionLib.Flip FlipBook` (`self.TeacherActor`))
  (`/Game/ProjectContents/BP/BP_FunctionLib.SetupDialogManagerCycle` (`self.Level Dialog Manager`) (`self.TeacherActor`) (`self.Teacher`) self))

(event `Handle Teacher Animation`
  (bind _teacheractor (`self.TeacherActor`))
  (bind _teacheractor_2 (`self.TeacherActor`))
  ;[1 1 1] Handle Teacher Animation
  (`/Game/ProjectContents/BP/BP_FunctionLib.Flip FlipBook` _teacheractor_2)
  (bind _dialog_delay (`/Game/ProjectContents/BP/LevelActors/BP_DialogManager.Display Dialog` (`self.Level Dialog Manager`) _teacheractor_2 (`self.Teacher`) (`self.TextDelay`)))
  (`KismetSystemLibrary.Delay` _dialog_delay)
  (`/Game/ProjectContents/BP/BP_FunctionLib.Flip FlipBook` _teacheractor)
  (bind _asbp_npcactor_teacher (cast `/Game/ProjectContents/BP/NPC/BP_NPCActor_Teacher` _teacheractor))
  (`/Game/ProjectContents/BP/NPC/BP_NPCActorBase.MoveNPC Event` _asbp_npcactor_teacher (`self.Teacher StartLocation`) (`self.Teacher GoalLocation`))
  (`KismetSystemLibrary.Delay` 3.0)
  (`/Game/ProjectContents/BP/NPC/BP_NPCActor_Teacher.SetVisibilityFalse` _asbp_npcactor_teacher)
  (`KismetSystemLibrary.Delay` 1.0)
  (`self.Handle Sister Animation`))

(event `Handle Scene End`
  ;[1 1 1] Scene3 Classroom End
  (`self.EnableInput` (`GameplayStatics.GetPlayerPawn` 0) (`GameplayStatics.GetPlayerController` 0))
  (bind _asbp_game_instance (cast `/Game/ProjectContents/BP/BP_GameInstance` (`GameplayStatics.GetGameInstance`)))
  (`/Game/ProjectContents/BP/BP_GameInstance.MoveToNextScene` _asbp_game_instance)
  (set `/Game/ProjectContents/BP/BP_GameInstance.isViewingScene` false _asbp_game_instance)
  (set `/Game/ProjectContents/BP/BP_GameInstance.PreviousRoom` "Classroom" _asbp_game_instance))

(event `Part1`
  (bind _teacheractor (`self.TeacherActor`))
  (`/Game/ProjectContents/BP/BP_FunctionLib.Flip FlipBook` _teacheractor)
  (bind _asbp_npcactor_teacher (cast `/Game/ProjectContents/BP/NPC/BP_NPCActor_Teacher` _teacheractor))
  (`/Game/ProjectContents/BP/NPC/BP_NPCActorBase.MoveNPC Event` _asbp_npcactor_teacher (`self.Teacher StartLocation`) (`self.Teacher GoalLocation`))
  (`KismetSystemLibrary.Delay` 3.0)
  (`/Game/ProjectContents/BP/NPC/BP_NPCActor_Teacher.SetVisibilityFalse` _asbp_npcactor_teacher)
  (`self.K2_DestroyActor` (`self.TeacherActor`))
  (`GameplayStatics.PlaySound2D` "/Game/ProjectContents/Music/BGM_HallwayClassroom.BGM_HallwayClassroom" 1.0 1.0 0.0 null null)
  (`/Game/ProjectContents/BP/BP_FunctionLib.SetupDialogManagerCycle` (`self.Level Dialog Manager`) (`|GetArrayItem` (`self.StudentNPCs`)) (`self.StudentA1`) self))

(event `Part2`
  (bind _asbp_npcactor_big_sister (cast `/Game/ProjectContents/BP/NPC/BP_NPCActor_BigSister` (`self.BigSisterActor`)))
  (`/Game/ProjectContents/BP/BP_FunctionLib.Flip FlipBook` _asbp_npcactor_big_sister)
  (`/Game/ProjectContents/BP/BP_FunctionLib.SetupDialogManagerCycle` (`self.Level Dialog Manager`) (`self.BigSisterActor`) (`self.BigSister1`) self))

(event `Handle Sister Animation`
  ;[1 1 1] Handle Sister Animation
  (bind _asbp_npcactor_big_sister (cast `/Game/ProjectContents/BP/NPC/BP_NPCActor_BigSister` (`self.BigSisterActor`)))
  (`/Game/ProjectContents/BP/NPC/BP_NPCActor_BigSister.SetVisibilityTrue` _asbp_npcactor_big_sister)
  (`/Game/ProjectContents/BP/BP_FunctionLib.Flip FlipBook` _asbp_npcactor_big_sister)
  (`/Game/ProjectContents/BP/NPC/BP_NPCActorBase.MoveNPC Event` _asbp_npcactor_big_sister (`self.BigSister StartLocation`) (`self.BigSister GoalLocation`))
  (`KismetSystemLibrary.Delay` 3.0))

(event `Part3`
  (`/Game/ProjectContents/BP/BP_FunctionLib.SetupDialogManagerCycle` (`self.Level Dialog Manager`) (`|GetArrayItem` (`self.StudentNPCs`)) (`self.StudentA2`) self))

(event `Part4`
  (`/Game/ProjectContents/BP/BP_FunctionLib.SetupDialogManagerCycle` (`self.Level Dialog Manager`) (`|GetArrayItem` (`self.StudentNPCs`) 1) (`self.Student B`) self))

(event `Handle StudentA Dialog`
  ;[1 1 1] Students Dialogs
  (bind _dialog_delay (`/Game/ProjectContents/BP/LevelActors/BP_DialogManager.Display Dialog` (`self.Level Dialog Manager`) (`|GetArrayItem` (`self.StudentNPCs`)) (`self.StudentA1`) (`self.TextDelay`)))
  (`KismetSystemLibrary.Delay` _dialog_delay)
  (`self.Handle StudentB Dialog`))

(event `Handle StudentB Dialog`
  ;[1 1 1] Students Dialogs
  (bind _dialog_delay (`/Game/ProjectContents/BP/LevelActors/BP_DialogManager.Display Dialog` (`self.Level Dialog Manager`) (`|GetArrayItem` (`self.StudentNPCs`) 1) (`self.Student B`) (`self.TextDelay`)))
  (`KismetSystemLibrary.Delay` _dialog_delay)
  (`self.Handle StudentC Dialog`))

(event `Part5`
  (`/Game/ProjectContents/BP/BP_FunctionLib.SetupDialogManagerCycle` (`self.Level Dialog Manager`) (`self.BigSisterActor`) (`self.BigSister2`) self))

(event `Handle StudentC Dialog`
  ;[1 1 1] Students Dialogs
  (bind _dialog_delay (`/Game/ProjectContents/BP/LevelActors/BP_DialogManager.Display Dialog` (`self.Level Dialog Manager`) (`|GetArrayItem` (`self.StudentNPCs`) 2) (`self.Student C`) (`self.TextDelay`)))
  (`KismetSystemLibrary.Delay` _dialog_delay)
  (`self.Handle Sister End`))

(event `Part6`
  (`/Game/ProjectContents/BP/BP_FunctionLib.SetupDialogManagerCycle` (`self.Level Dialog Manager`) (`|GetArrayItem` (`self.StudentNPCs`) 2) (`self.Student C`) self))

(event `Part7`
  (`/Game/ProjectContents/BP/BP_FunctionLib.SetupDialogManagerCycle` (`self.Level Dialog Manager`) (`self.BigSisterActor`) (`self.BigSister3`) self))

(event `Handle Sister End`
  (bind _bigsisteractor (`self.BigSisterActor`))
  ;[1 1 1] Handle Sister Exit
  (bind _dialog_delay (`/Game/ProjectContents/BP/LevelActors/BP_DialogManager.Display Dialog` (`self.Level Dialog Manager`) (`self.BigSisterActor`) (`self.BigSister1`) (`self.TextDelay`)))
  (`KismetSystemLibrary.Delay` _dialog_delay)
  (bind _asbp_npcactor_big_sister (cast `/Game/ProjectContents/BP/NPC/BP_NPCActor_BigSister` _bigsisteractor))
  (`/Game/ProjectContents/BP/NPC/BP_NPCActorBase.MoveNPC Event` _asbp_npcactor_big_sister (`self.K2_GetActorLocation` _bigsisteractor) (`self.Exit Location`))
  (`KismetSystemLibrary.Delay` 3.0)
  (`self.K2_DestroyActor` (`self.BigSisterActor`))
  (`self.Handle Scene End`))

(event `Part8`
  (`/Game/ProjectContents/BP/BP_FunctionLib.SetupDialogManagerCycle` (`self.Level Dialog Manager`) (`|GetArrayItem` (`self.StudentNPCs`) 1) (`self.Student B2`) self))

(event `Part9`
  (`/Game/ProjectContents/BP/BP_FunctionLib.SetupDialogManagerCycle` (`self.Level Dialog Manager`) (`|GetArrayItem` (`self.StudentNPCs`) 2) (`self.Student C2`) self))

(event `Part10`
  (`/Game/ProjectContents/BP/BP_FunctionLib.SetupDialogManagerCycle` (`self.Level Dialog Manager`) (`|GetArrayItem` (`self.StudentNPCs`)) (`self.StudentA3`) self))

(event `Part11`
  (bind _bigsisteractor (`self.BigSisterActor`))
  (bind _asbp_npcactor_big_sister (cast `/Game/ProjectContents/BP/NPC/BP_NPCActor_BigSister` _bigsisteractor))
  (`/Game/ProjectContents/BP/BP_FunctionLib.Flip FlipBook` _asbp_npcactor_big_sister)
  (`/Game/ProjectContents/BP/NPC/BP_NPCActorBase.MoveNPC Event` _asbp_npcactor_big_sister (`self.K2_GetActorLocation` _bigsisteractor) (`self.BigSister StartLocation`))
  (`KismetSystemLibrary.Delay` 3.0)
  (`self.K2_DestroyActor` (`self.BigSisterActor`))
  (`self.Handle Scene End`))

(fn `Get Level NPCs`
  (bind _outactors (`GameplayStatics.GetAllActorsOfClass` "/Game/ProjectContents/BP/NPC/BP_NPCActorBase.BP_NPCActorBase_C"))
  (for _array_element _outactors
    (if (`self.ActorHasTag` _array_element "Student")
      (`KismetArrayLibrary.Array_Add` (`self.StudentNPCs`) _array_element)
      (elif (`self.ActorHasTag` _array_element "Teacher")
        (set `self.TeacherActor` _array_element)
        (else
          (set `self.BigSisterActor` _array_element))))))

(fn `LevelSetup`
  (`|ExecutionSequence`
    (:`then_0`
      (bind _outactors (`GameplayStatics.GetAllActorsOfClass` "/Game/ProjectContents/BP/NPC/BP_NPCActorBase.BP_NPCActorBase_C"))
      (for _array_element _outactors
        (`/Engine/EditorBlueprintResources/StandardMacros.IsValid` _array_element
          (:`Is Valid`
            (`self.K2_DestroyActor` _array_element)))))
    (:`then_1`
      (bind _returnvalue (`GameplayStatics.GetActorOfClass` "/Game/ProjectContents/BP/SceneManager/BP_SceneManager_Scene02_Classroom.BP_SceneManager_Scene02_Classroom_C"))
      (`/Engine/EditorBlueprintResources/StandardMacros.IsValid` _returnvalue
        (:`Is Valid`
          (`self.K2_DestroyActor` _returnvalue)
          (bind _returnvalue_2 (`GameplayStatics.GetActorOfClass` "/Game/ProjectContents/BP/Objects/BP_PaperBall.BP_PaperBall_C"))
          (`/Engine/EditorBlueprintResources/StandardMacros.IsValid` _returnvalue_2
            (:`Is Valid`
              (`self.K2_DestroyActor` _returnvalue_2))))))
    (:`then_2`
      (`self.K2_SetActorLocation` (`GameplayStatics.GetPlayerPawn` 0) (`self.PlayerLocation`) false false))
    (:`then_3`
      (for (_array_element_2 _array_index) (`self.LevelActors`)
        (`|SpawnActorFromClass` _array_element_2 (`|GetArrayItem` (`self.ActorSpawns`) _array_index) "Undefined" "OverrideRootScale" null null))
      (`self.Get Level NPCs`))
    (:`then_4`
      (bind _returnvalue_3 (`GameplayStatics.GetActorOfClass` "/Game/ProjectContents/BP/NPC/BP_NPCActor_BigSister.BP_NPCActor_BigSister_C"))
      (`/Game/ProjectContents/BP/NPC/BP_NPCActor_BigSister.SetVisibilityFalse` _returnvalue_3)
      (`self.K2_SetActorLocation` (`self.BigSister StartLocation`)))
    (:`then_5`
      (`GameplayStatics.PlaySound2D` "/Game/ProjectContents/SFX/SFX_SchoolBell.SFX_SchoolBell" 1.0 1.0 0.0 null null)
      (cast `/Game/ProjectContents/BP/BP_GameInstance` (`GameplayStatics.GetGameInstance`)))))

(fn `MoveToNextPart`
  (`self.DisableInput` (`GameplayStatics.GetPlayerController` 0))
  (bind _result (`/Engine/EditorBlueprintResources/StandardMacros.IncrementInt` (`self.CurrentPart`))
    (:`  `
      (bind _asbp_game_instance (cast `/Game/ProjectContents/BP/BP_GameInstance` (`GameplayStatics.GetGameInstance`)))
      (bind _output_get (set `/Game/ProjectContents/BP/BP_GameInstance.ScenePart` _result _asbp_game_instance))
      (switch `int` _output_get
        (:`1`
          (`self.Part1`))
        (:`2`
          (`self.Part2`))
        (:`3`
          (`self.Part3`))
        (:`4`
          (`self.Part4`))
        (:`5`
          (`self.Part5`))
        (:`6`
          (`self.Part6`))
        (:`7`
          (`self.Part7`))
        (:`8`
          (`self.Part8`))
        (:`9`
          (`self.Part9`))
        (:`10`
          (`self.Part10`))
        (:`11`
          (`self.Part11`))))))

(fn `UserConstructionScript`)