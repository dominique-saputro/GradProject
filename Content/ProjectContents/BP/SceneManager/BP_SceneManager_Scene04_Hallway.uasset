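; Scene manager for the Scene 4 hallway that stages the Big Sister NPC's walks to and from the cafeteria.
; On BeginPlay, after a scene check, it spawns her at either hallway end based on GameInstance progress flags.
; CheckMove reads those flags to walk her across, flipping her flipbook on the return, or remove her.
; Interact cycles dialogue and, once finished, increments the scene part, whose switch has no cases.
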(event `InputAction|Interact`
  (params (Key :type "Key Structure"))
  ;[1 1 1] OnInteract
  (:`Pressed`
    (bind _asbp_game_instance (cast `/Game/ProjectContents/BP/BP_GameInstance` (`GameplayStatics.GetGameInstance`)))
    (if (`/Game/ProjectContents/BP/BP_GameInstance.isViewingScene` _asbp_game_instance)
      (if (`/Game/ProjectContents/BP/LevelActors/BP_DialogManager.isDIalogFinished` (`self.Level Dialog Manager`))
        (set `/Game/ProjectContents/BP/LevelActors/BP_DialogManager.isDIalogFinished` false (`self.Level Dialog Manager`))
        (bind _asbp_game_instance_2 (cast `/Game/ProjectContents/BP/BP_GameInstance` (`GameplayStatics.GetGameInstance`)))
        (set `/Game/ProjectContents/BP/BP_GameInstance.isViewingScene` false _asbp_game_instance_2)
        (`KismetSystemLibrary.PrintString` "DialogFinished")
        (`self.MoveToNextPart`)
        (else
          (`/Game/ProjectContents/BP/LevelActors/BP_DialogManager.Test-CycleOnKey` (`self.Level Dialog Manager`)))))))

(event `self.ReceiveBeginPlay`
  (bind _iscorrectscene (`/Game/ProjectContents/BP/BP_FunctionLib.CheckSceneIndex` (`self.CurrentScene`)))
  (if _iscorrectscene
    (`self.LevelSetup`)
    (bind _returnvalue (`GameplayStatics.GetActorOfClass` "/Game/ProjectContents/BP/LevelActors/BP_DialogManager.BP_DialogManager_C"))
    (set `self.Level Dialog Manager` _returnvalue)
    (`self.CheckMove`)))

(event `CheckMove`
  (bind _asbp_game_instance (cast `/Game/ProjectContents/BP/BP_GameInstance` (`GameplayStatics.GetGameInstance`)))
  (if (`/Game/ProjectContents/BP/BP_GameInstance.isScene4ToCafeteriaFinished` _asbp_game_instance)
    (bind _asbp_game_instance_2 (cast `/Game/ProjectContents/BP/BP_GameInstance` (`GameplayStatics.GetGameInstance`)))
    (if (`/Game/ProjectContents/BP/BP_GameInstance.isScene4CafeteriaFinished` _asbp_game_instance_2)
      (bind _asbp_game_instance_3 (cast `/Game/ProjectContents/BP/BP_GameInstance` (`GameplayStatics.GetGameInstance`)))
      (if (`/Game/ProjectContents/BP/BP_GameInstance.isScene4FromCafeteriaFinished` _asbp_game_instance_3)
        (bind _asbp_game_instance_4 (cast `/Game/ProjectContents/BP/BP_GameInstance` (`GameplayStatics.GetGameInstance`)))
        (if (`/Game/ProjectContents/BP/BP_GameInstance.isScene4ClassroomFinished` _asbp_game_instance_4)
          (bind _asbp_game_instance_5 (cast `/Game/ProjectContents/BP/BP_GameInstance` (`GameplayStatics.GetGameInstance`)))
          (if (`/Game/ProjectContents/BP/BP_GameInstance.isScene4ToCafeteriaFinished` _asbp_game_instance_5)
            (`self.K2_DestroyActor` (`self.BigSIster`))
            (else
              (`self.MoveTo Caffeteria`)))
          (else
            (`self.K2_DestroyActor` (`self.BigSIster`))))
        (else
          (`self.MoveFrom Cafeteria`)))
      (else
        (`self.K2_DestroyActor` (`self.BigSIster`))))
    (else
      (`self.MoveTo Caffeteria`))))

(event `MoveTo Caffeteria`
  (bind _bigsister (`self.BigSIster`))
  ;[1 1 1] Handle Before Cafeteria
  (`KismetSystemLibrary.Delay` 1.0)
  (bind _asbp_game_instance (cast `/Game/ProjectContents/BP/BP_GameInstance` (`GameplayStatics.GetGameInstance`)))
  (set `/Game/ProjectContents/BP/BP_GameInstance.isScene4ToCafeteriaFinished` true _asbp_game_instance)
  (`/Game/ProjectContents/BP/NPC/BP_NPCActorBase.MoveNPC Event` _bigsister (`self.Hallway Start`) (`self.Hallway End`))
  (`KismetSystemLibrary.Delay` 3.0)
  (`self.K2_DestroyActor` _bigsister))

(event `MoveFrom Cafeteria`
  (bind _bigsister (`self.BigSIster`))
  ;[1 1 1] Handle After Cafeteria
  (`KismetSystemLibrary.Delay` 1.0)
  (bind _asbp_game_instance (cast `/Game/ProjectContents/BP/BP_GameInstance` (`GameplayStatics.GetGameInstance`)))
  (set `/Game/ProjectContents/BP/BP_GameInstance.isScene4FromCafeteriaFinished` true _asbp_game_instance)
  (`/Game/ProjectContents/BP/BP_FunctionLib.Flip FlipBook` _bigsister)
  (`/Game/ProjectContents/BP/NPC/BP_NPCActorBase.MoveNPC Event` _bigsister (`self.Hallway End`) (`self.Hallway Start`))
  (`KismetSystemLibrary.Delay` 3.0)
  (`self.K2_DestroyActor` _bigsister))

(fn `LevelSetup`
  (bind _asbp_game_instance (cast `/Game/ProjectContents/BP/BP_GameInstance` (`GameplayStatics.GetGameInstance`)))
  (if (`/Game/ProjectContents/BP/BP_GameInstance.isScene4CafeteriaFinished` _asbp_game_instance)
    (bind _returnvalue (`|SpawnActorFromClass` "/Game/ProjectContents/BP/NPC/BP_NPCActor_BigSister.BP_NPCActor_BigSister_C" (`KismetMathLibrary.MakeTransform` (`self.Hallway End`) (struct) (2.1 2.1 2.1)) "Undefined" "OverrideRootScale" null null))
    (set `self.BigSIster` _returnvalue)
    (else
      (bind _returnvalue_2 (`|SpawnActorFromClass` "/Game/ProjectContents/BP/NPC/BP_NPCActor_BigSister.BP_NPCActor_BigSister_C" (`KismetMathLibrary.MakeTransform` (`self.Hallway Start`) (struct) (2.1 2.1 2.1)) "Undefined" "OverrideRootScale" null null))
      (set `self.BigSIster` _returnvalue_2))))

(fn `MoveToNextPart`
  (`self.DisableInput` (`GameplayStatics.GetPlayerController` 0))
  (bind _result (`/Engine/EditorBlueprintResources/StandardMacros.IncrementInt` (`self.CurrentPart`))
    (:`  `
      (bind _asbp_game_instance (cast `/Game/ProjectContents/BP/BP_GameInstance` (`GameplayStatics.GetGameInstance`)))
      (bind _output_get (set `/Game/ProjectContents/BP/BP_GameInstance.ScenePart` _result _asbp_game_instance))
      (switch `int` _output_get))))

(fn `UserConstructionScript`)