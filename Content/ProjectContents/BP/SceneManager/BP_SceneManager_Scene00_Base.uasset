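; Base scene manager for Scene00 that plays a scripted dialog scene, apparently still in a test state.
; On BeginPlay it flags the GameInstance as viewing a scene and passes an NPC StudentB and dialog list to the level's dialog manager.
; Interact cycles dialog; once finished, it clears the flag, disables input and increments the part index into an empty switch.
; LevelSetup can spawn actors at paired transforms, but its call is disconnected.
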(event `self.ReceiveBeginPlay`
  (bind _returnvalue (`GameplayStatics.GetActorOfClass` "/Game/ProjectContents/BP/LevelActors/BP_DialogManager.BP_DialogManager_C"))
  (set `self.Level Dialog Manager` _returnvalue)
  (`self.TestPlay`)
  (`self.EnableInput` (`GameplayStatics.GetPlayerController` 0)))

(event `TestPlay`
  (bind _asbp_game_instance (cast `/Game/ProjectContents/BP/BP_GameInstance` (`GameplayStatics.GetGameInstance`)))
  (set `/Game/ProjectContents/BP/BP_GameInstance.isViewingScene` true _asbp_game_instance)
  (bind _returnvalue (`GameplayStatics.GetActorOfClass` "/Game/ProjectContents/BP/NPC/BP_NPCActor_StudentB.BP_NPCActor_StudentB_C"))
  (`/Game/ProjectContents/BP/LevelActors/BP_DialogManager.Test-SetDialogList` (`self.Level Dialog Manager`) _returnvalue (`self.DialogText`)))

(event `TestPlay1`
  (`self.K2_DestroyActor` (stale `TestPlay` _returnvalue)))

(event `InputAction|Interact`
  (params (Key :type "Key Structure"))
  ;[1 1 1] OnInteract
  (:`Pressed`
    (if (`/Game/ProjectContents/BP/LevelActors/BP_DialogManager.isDIalogFinished` (`self.Level Dialog Manager`))
      (set `/Game/ProjectContents/BP/LevelActors/BP_DialogManager.isDIalogFinished` false (`self.Level Dialog Manager`))
      (bind _asbp_game_instance (cast `/Game/ProjectContents/BP/BP_GameInstance` (`GameplayStatics.GetGameInstance`)))
      (set `/Game/ProjectContents/BP/BP_GameInstance.isViewingScene` false _asbp_game_instance)
      (`KismetSystemLibrary.PrintString` "DialogFinished")
      (`self.MoveToNextPart`)
      (else
        (`/Game/ProjectContents/BP/LevelActors/BP_DialogManager.Test-CycleOnKey` (`self.Level Dialog Manager`))))))

(fn `LevelSetup`
  (for (_array_element _array_index) (`self.LevelActors`)
    (`|SpawnActorFromClass` _array_element (`|GetArrayItem` (`self.ActorSpawns`) _array_index) "Undefined" "OverrideRootScale" null null)))

(fn `MoveToNextPart`
  (`self.DisableInput` (`GameplayStatics.GetPlayerController` 0))
  (bind _result (`/Engine/EditorBlueprintResources/StandardMacros.IncrementInt` (`self.CurrentPart`))
    (:`  `
      (switch `int` _result))))

(fn `UserConstructionScript`)