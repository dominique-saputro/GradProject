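; Scene 4 cafeteria manager that runs the story sequence of NPC dialogue, walk-offs, cooking minigames and tear drop pickup into the classroom level.
; MoveToNextPart advances numbered Part events as BP_DialogManager finishes each conversation.
; Burger, toaster and cupboard minigames open popup widgets, with timelines panning the follow camera via a dummy actor.
; BeginPlay spawns the cast and uses GameInstance flags to restore saved progress on reload.
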(event `InputAction|Interact`
  (params (Key :type "Key Structure"))
  ;[1 1 1] OnInteract
  (:`Pressed`
    (bind _asbp_game_instance (cast `/Game/ProjectContents/BP/BP_GameInstance` (`GameplayStatics.GetGameInstance`)))
    (if (`/Game/ProjectContents/BP/BP_GameInstance.isViewingScene` _asbp_game_instance)
      (if (`/Game/ProjectContents/BP/LevelActors/BP_DialogManager.isDIalogFinished` (`self.DialogManager`))
        (set `/Game/ProjectContents/BP/LevelActors/BP_DialogManager.isDIalogFinished` false (`self.DialogManager`))
        (bind _asbp_game_instance_2 (cast `/Game/ProjectContents/BP/BP_GameInstance` (`GameplayStatics.GetGameInstance`)))
        (set `/Game/ProjectContents/BP/BP_GameInstance.isViewingScene` false _asbp_game_instance_2)
        (`KismetSystemLibrary.PrintString` "DialogFinished")
        (`self.MoveToNextPart`)
        (else
          (`/Game/ProjectContents/BP/LevelActors/BP_DialogManager.Test-CycleOnKey` (`self.DialogManager`)))))))

(event `self.ReceiveBeginPlay`
  (bind _returnvalue (`GameplayStatics.GetActorOfClass` "/Game/ProjectContents/BP/LevelActors/BP_DialogManager.BP_DialogManager_C"))
  (set `self.DialogManager` _returnvalue)
  (bind _iscorrectscene (`/Game/ProjectContents/BP/BP_FunctionLib.CheckSceneIndex` (`self.CurrentScene`)))
  (if _iscorrectscene
    (`self.LevelSetup`)
    (bind _asbp_game_instance (cast `/Game/ProjectContents/BP/BP_GameInstance` (`GameplayStatics.GetGameInstance`)))
    (if (`/Game/ProjectContents/BP/BP_GameInstance.isScene4CafeteriaFinished` _asbp_game_instance)
      (if (`/Game/ProjectContents/BP/BP_GameInstance.isScene4ClassroomFinished` _asbp_game_instance)
        (if (`/Game/ProjectContents/BP/BP_GameInstance.isScene4TearDropSpawned` _asbp_game_instance)
          (`self.Reload - TearDropSpawned`)
          (else
            (`self.Reload-ClassroomCleared`)))
        (else
          (`self.Reload-MinigameCleared`)
          (`AudioComponent.Play` (`self.BGM`) 0.0 :!label _label)))
      (else
        (bind (_currentscene _currentpart) (`/Game/ProjectContents/BP/BP_FunctionLib.CheckCurrrentPart and Scene`))
        (if (== _currentpart 10)
          (`self.Reload-MinigameSpawned`)
          (goto _label)
          (else
            (goto _label)))))))

(event `Spawn Minigames`
  (if (not (`self.isBurgerClear`))
    (bind _returnvalue (`|SpawnActorFromClass` "/Game/ProjectContents/BP/PopOutManager/BP_Minigame_Burger.BP_Minigame_Burger_C" (`KismetMathLibrary.MakeTransform` (-1500.0 10.0 500.0)) "Undefined" "OverrideRootScale" null null))
    (set `self.BurgerMinigame` _returnvalue))
  (if (not (`self.isToasterClear`))
    (bind _returnvalue_2 (`|SpawnActorFromClass` "/Game/ProjectContents/BP/PopOutManager/BP_Minigame_Toaster.BP_Minigame_Toaster_C" (`KismetMathLibrary.MakeTransform` (-2200.0 10.0 500.0)) "Undefined" "OverrideRootScale" null null))
    (set `self.ToasterMinigame` _returnvalue_2))
  (if (not (`self.isCupboardClear`))
    (bind _returnvalue_3 (`|SpawnActorFromClass` "/Game/ProjectContents/BP/PopOutManager/BP_Minigame_Cupboard.BP_Minigame_Cupboard_C" (`KismetMathLibrary.MakeTransform` (-1000.0 10.0 500.0)) "Undefined" "OverrideRootScale" null null))
    (set `self.CupboardMinigame` _returnvalue_3)))

(event `Reload-MinigameSpawned`
  (bind _bigsisteractor (`self.BigSisterActor`))
  (bind _returnvalue (`GameplayStatics.GetActorOfClass` (`|GetArrayItem` (`self.LevelActors`) 2)))
  (`self.K2_DestroyActor` _returnvalue)
  (`self.K2_DestroyActor` (`self.StudentE Actor`))
  (`self.K2_DestroyActor` (`self.StudentF Actpr`))
  (`self.K2_SetActorLocation` _bigsisteractor (- (`self.K2_GetActorLocation` _bigsisteractor) (350.0 0.0 0.0)) false false)
  (bind _asbp_game_instance (cast `/Game/ProjectContents/BP/BP_GameInstance` (`GameplayStatics.GetGameInstance`)))
  (for (_array_element _array_index) (`/Game/ProjectContents/BP/BP_GameInstance.isClearMinigame` _asbp_game_instance)
    (if _array_element
      (switch `int` _array_index
        (:`0`
          (`self.K2_DestroyActor` (`self.BurgerMinigame`))
          (set `self.isBurgerClear` true))
        (:`1`
          (`self.K2_DestroyActor` (`self.CupboardMinigame`))
          (set `self.isCupboardClear` true))
        (:`2`
          (`self.K2_DestroyActor` (`self.ToasterMinigame`))
          (set `self.isToasterClear` true)))))
  (set `self.CurrentPart` 9)
  (`self.MoveToNextPart`))

(event `Part14`
  ;[1 1 1] After ClassroomClear, Starts Part14
  (bind _asbp_game_instance (cast `/Game/ProjectContents/BP/BP_GameInstance` (`GameplayStatics.GetGameInstance`)))
  (if (and (`/Game/ProjectContents/BP/BP_GameInstance.isScene4CafeteriaFinished` _asbp_game_instance) (`/Game/ProjectContents/BP/BP_GameInstance.isScene4ClassroomFinished` _asbp_game_instance))
    (`/Game/ProjectContents/BP/BP_FunctionLib.SetupDialogManagerCycle` (`self.DialogManager`) (`self.StaffActor`) (`self.Staff5`) self)
    (`/Game/ProjectContents/BP/BP_FunctionLib.DisablePlayerInput`)
    (else
      (set `/Game/ProjectContents/BP/BP_GameInstance.isViewingScene` false _asbp_game_instance))))

(event `Reload-MinigameCleared`
  (bind _returnvalue (`GameplayStatics.GetActorOfClass` (`|GetArrayItem` (`self.LevelActors`) 2)))
  (`self.K2_DestroyActor` _returnvalue)
  (`self.K2_DestroyActor` (`self.BigSisterActor`))
  (set `self.CurrentPart` 99)
  (`self.K2_DestroyActor` (`self.StudentE Actor`))
  (`self.K2_DestroyActor` (`self.StudentF Actpr`)))

(event `Part11`
  (`/Game/ProjectContents/BP/BP_FunctionLib.SetupDialogManagerCycle` (`self.DialogManager`) (`self.BigSisterActor`) (`self.Sister2`) self))

(event `Burger Minigame STart`
  (bind _returnvalue (`GameplayStatics.GetPlayerController` 0))
  ;[1 1 1] BurgerMinigame
  (`self.Handle Change Camera`)
  (`self.HandleMoveCameraRight`)
  (`KismetSystemLibrary.Delay` 3.0)
  (bind _returnvalue_2 (`|CreateWidget` "/Game/ProjectContents/BP/Widgets/PopOut/WBP_Pop_Burger.WBP_Pop_Burger_C" _returnvalue))
  (set `PlayerController.bShowMouseCursor` true _returnvalue)
  (`UserWidget.AddToViewport` _returnvalue_2 0))

(event `CheckMinigameClear`
  (if (and (`self.isBurgerClear`) (`self.isToasterClear`) (`self.isCupboardClear`))
    (bind _asbp_game_instance (cast `/Game/ProjectContents/BP/BP_GameInstance` (`GameplayStatics.GetGameInstance`)))
    (set `/Game/ProjectContents/BP/BP_GameInstance.isScene4CafeteriaFinished` true _asbp_game_instance)
    (`self.HandleMinigameCleared`)
    (else
      (bind _asbp_game_instance_2 (cast `/Game/ProjectContents/BP/BP_GameInstance` (`GameplayStatics.GetGameInstance`)))
      (set `/Game/ProjectContents/BP/BP_GameInstance.isClearMinigame` (`|MakeArray` (`self.isBurgerClear`) (`self.isCupboardClear`) (`self.isToasterClear`)) _asbp_game_instance_2))))

(event `Part15`
  ;[1 1 1] After ClassroomClear, Starts Part14
  (`/Game/ProjectContents/BP/BP_FunctionLib.SetupDialogManagerCycle` (`self.DialogManager`) (`self.BigSisterActor`) (`self.Sister3`) self))

(event `Burger Minigame End`
  ;[1 1 1] BurgerMinigame
  (`GameplayStatics.PlaySound2D` "/Game/ProjectContents/SFX/SFX_Pickup.SFX_Pickup" 1.0 1.0 0.0 null null)
  (`AudioComponent.SetPaused` (`self.BGM`) false)
  (`self.HandleMOveCameraLeft`)
  (`KismetSystemLibrary.Delay` 3.0)
  (set `PlayerController.bShowMouseCursor` false (`GameplayStatics.GetPlayerController` 0))
  (set `self.isBurgerClear` true)
  (`self.CheckMinigameClear`))

(event `Part12`
  (bind _bigsisteractor (`self.BigSisterActor`))
  (`/Game/ProjectContents/BP/BP_FunctionLib.Flip FlipBook` _bigsisteractor)
  (bind _asbp_npcactor_base (cast `/Game/ProjectContents/BP/NPC/BP_NPCActorBase` _bigsisteractor))
  (`/Game/ProjectContents/BP/NPC/BP_NPCActorBase.MoveNPC Event` _asbp_npcactor_base (`self.K2_GetActorLocation` _bigsisteractor) (`self.LevelExit Location`))
  (`/Game/ProjectContents/BP/BP_FunctionLib.SetupDialogManagerCycle` (`self.DialogManager`) (`self.StaffActor`) (`self.Staff4`) self))

(event `Reload-ClassroomCleared`
  (bind _bigsisteractor (`self.BigSisterActor`))
  (`AudioComponent.Stop` (`self.BGM`))
  (`GameplayStatics.PlaySound2D` "/Game/ProjectContents/SFX/SFX_SchoolBell.SFX_SchoolBell" 1.0 1.0 0.0 null null)
  (set `self.CurrentPart` 13)
  (`self.K2_DestroyActor` (`self.StudentE Actor`))
  (`self.K2_DestroyActor` (`self.StudentF Actpr`))
  (`self.K2_SetActorLocation` _bigsisteractor (- (`self.K2_GetActorLocation` _bigsisteractor) (350.0 0.0 0.0)) false false))

(event `HandleMinigameCleared`
  (bind _staffactor (`self.StaffActor`))
  (bind _output_location (`KismetMathLibrary.BreakTransform` (`|GetArrayItem` (`self.ActorSpawns`))))
  (`/Game/ProjectContents/BP/BP_FunctionLib.DisablePlayerInput`)
  (`GameplayStatics.PlaySound2D` "/Game/ProjectContents/SFX/SFX_Cooking.SFX_Cooking" 1.0 1.0 0.0 null null)
  (`KismetSystemLibrary.Delay` 3.0)
  (`/Game/ProjectContents/BP/BP_FunctionLib.Flip FlipBook` _staffactor)
  (bind _asbp_npcactor_staff (cast `/Game/ProjectContents/BP/NPC/BP_NPCActor_Staff` _staffactor))
  (`/Game/ProjectContents/BP/NPC/BP_NPCActorBase.MoveNPC Event` _asbp_npcactor_staff (`self.Staff EndMove`) _output_location)
  (`self.PostMinigame-ChangeCamera`)
  (`self.PostMinigame-MoveCameraRight`))

(event `Part16`
  (bind _bigsisteractor (`self.BigSisterActor`))
  ;[1 1 1] After ClassroomClear, Starts Part14
  (`/Game/ProjectContents/BP/BP_FunctionLib.Flip FlipBook` _bigsisteractor)
  (bind _asbp_npcactor_big_sister (cast `/Game/ProjectContents/BP/NPC/BP_NPCActor_BigSister` _bigsisteractor))
  (`/Game/ProjectContents/BP/NPC/BP_NPCActorBase.MoveNPC Event` _asbp_npcactor_big_sister (`self.K2_GetActorLocation` _bigsisteractor) (`self.LevelExit Location`))
  (`KismetSystemLibrary.Delay` 0.5)
  (`|SpawnActorFromClass` "/Game/ProjectContents/BP/Objects/BP_TearDrop.BP_TearDrop_C" (`self.TearTransform`) "Undefined" "OverrideRootScale" null null)
  (`KismetSystemLibrary.Delay` 2.5)
  (`self.K2_DestroyActor` _bigsisteractor)
  (`/Game/ProjectContents/BP/BP_FunctionLib.EnablePlayerInput`)
  (bind _asbp_game_instance (cast `/Game/ProjectContents/BP/BP_GameInstance` (`GameplayStatics.GetGameInstance`)))
  (set `/Game/ProjectContents/BP/BP_GameInstance.isScene4TearDropSpawned` true _asbp_game_instance))

(event `Toaster Minigame Start`
  (bind _returnvalue (`GameplayStatics.GetPlayerController` 0))
  ;[1 1 1] ToasterMinigame
  (`self.Handle Change Camera`)
  (`self.HandleMoveCameraRight`)
  (`KismetSystemLibrary.Delay` 3.0)
  (bind _returnvalue_2 (`|CreateWidget` "/Game/ProjectContents/BP/Widgets/PopOut/WBP_Pop_Toaster.WBP_Pop_Toaster_C" _returnvalue))
  (set `PlayerController.bShowMouseCursor` true _returnvalue)
  (`UserWidget.AddToViewport` _returnvalue_2 0))

(event `Part13`
  (`self.PostMinigame-MoveCameraLeft`))

(event `Reload - TearDropSpawned`
  (`AudioComponent.Stop` (`self.BGM`))
  (set `self.CurrentPart` 17)
  (`|SpawnActorFromClass` "/Game/ProjectContents/BP/Objects/BP_TearDrop.BP_TearDrop_C" (`self.TearTransform`) "Undefined" "OverrideRootScale" null null)
  (`self.K2_DestroyActor` (`self.BigSisterActor`))
  (`self.K2_DestroyActor` (`self.StudentE Actor`))
  (`self.K2_DestroyActor` (`self.StudentF Actpr`)))

(event `PostMinigame-ChangeCamera`
  (bind _returnvalue (`self.K2_GetActorLocation` (`GameplayStatics.GetPlayerPawn` 0)))
  (bind _returnvalue_2 (`|SpawnActorFromClass` "/Game/ProjectContents/BP/Objects/BP_DummyActor.BP_DummyActor_C" (`KismetMathLibrary.MakeTransform` _returnvalue) "Undefined" "OverrideRootScale" null null))
  (set `self.DummyActor` _returnvalue_2)
  (bind _returnvalue_3 (`GameplayStatics.GetActorOfClass` "/Game/ProjectContents/BP/LevelActors/BP_FollowCamera.BP_FollowCamera_C"))
  (set `/Game/ProjectContents/BP/LevelActors/BP_FollowCamera.ActorToFollow` _returnvalue_2 _returnvalue_3)
  (`KismetSystemLibrary.PrintString` "Switched ActorToFollow")
  (bind _output_get (set `self.CameraStart` _returnvalue))
  (set `self.CameraEnd` (`KismetMathLibrary.MakeVector` -110.0 (.y _output_get) (.z _output_get)))
  (`/Game/ProjectContents/BP/BP_FunctionLib.DisablePlayerInput`))

(event `Toaster Minigame End`
  ;[1 1 1] ToasterMinigame
  (`GameplayStatics.PlaySound2D` "/Game/ProjectContents/SFX/SFX_Pickup.SFX_Pickup" 1.0 1.0 0.0 null null)
  (`AudioComponent.SetPaused` (`self.BGM`) false)
  (`self.HandleMOveCameraLeft`)
  (`KismetSystemLibrary.Delay` 3.0)
  (set `PlayerController.bShowMouseCursor` false (`GameplayStatics.GetPlayerController` 0))
  (set `self.isToasterClear` true)
  (`self.CheckMinigameClear`))

(event `PostMinigame-MoveCameraLeft`
  (bind (_direction _alpha) (`Timeline|Timeline_3` :!via `PlayFromStart`)
    (:`Update`
      (`self.K2_SetActorLocation` (`self.DummyActor`) (`KismetMathLibrary.VLerp` (`self.CameraEnd`) (`self.CameraStart`) _alpha) false false))
    (:`Finished`
      (bind _returnvalue (`GameplayStatics.GetActorOfClass` "/Game/ProjectContents/BP/LevelActors/BP_FollowCamera.BP_FollowCamera_C"))
      (set `/Game/ProjectContents/BP/LevelActors/BP_FollowCamera.ActorToFollow` (`GameplayStatics.GetPlayerPawn` 0) _returnvalue)
      (`self.K2_DestroyActor` (`self.DummyActor`))
      (`self.K2_DestroyActor` (`self.BigSisterActor`))
      (`/Game/ProjectContents/BP/BP_FunctionLib.EnablePlayerInput`))))

(event `Part0`
  (`/Game/ProjectContents/BP/BP_FunctionLib.SetupDialogManagerCycle` (`self.DialogManager`) (`self.StudentE Actor`) (`self.StudentE`) self)
  (`/Game/ProjectContents/BP/BP_FunctionLib.DisablePlayerInput`))

(event `OnTearDrop PickUp`
  ;[1 1 1] OnTearDropPickup
  (bind _asbp_game_instance (cast `/Game/ProjectContents/BP/BP_GameInstance` (`GameplayStatics.GetGameInstance`)))
  (`/Game/ProjectContents/BP/BP_GameInstance.MoveToNextScene` _asbp_game_instance)
  (bind _returnvalue (`|CreateWidget` "/Game/ProjectContents/BP/Widgets/WBP_FadeBlack.WBP_FadeBlack_C" (`GameplayStatics.GetPlayerController` 0)))
  (`UserWidget.AddToViewport` _returnvalue 0)
  (`/Game/ProjectContents/BP/Widgets/WBP_FadeBlack.FadeToBlack` _returnvalue)
  (`KismetSystemLibrary.Delay` 0.5)
  (`GameplayStatics.OpenLevel` "Game_Classroom"))

(event `Part1`
  (`/Game/ProjectContents/BP/BP_FunctionLib.SetupDialogManagerCycle` (`self.DialogManager`) (`self.StudentF Actpr`) (`self.StudentF`) self))

(event `PostMinigame-MoveCameraRight`
  (bind (_direction _alpha) (`Timeline|Timeline_2`)
    (:`Update`
      (`self.K2_SetActorLocation` (`self.DummyActor`) (`KismetMathLibrary.VLerp` (`self.CameraStart`) (`self.CameraEnd`) _alpha) false false))
    (:`Finished`
      (`/Game/ProjectContents/BP/BP_FunctionLib.SetupDialogManagerCycle` (`self.DialogManager`) (`self.StaffActor`) (`self.Staff3`) self))))

(event `Cupboard Minigame Start`
  (bind _returnvalue (`GameplayStatics.GetPlayerController` 0))
  ;[1 1 1] CupboardMinigame
  (`self.Handle Change Camera`)
  (`self.HandleMoveCameraRight`)
  (`KismetSystemLibrary.Delay` 3.0)
  (bind _returnvalue_2 (`|CreateWidget` "/Game/ProjectContents/BP/Widgets/PopOut/WBP_Pop_CupBoard.WBP_Pop_CupBoard_C" _returnvalue))
  (set `PlayerController.bShowMouseCursor` true _returnvalue)
  (`UserWidget.AddToViewport` _returnvalue_2 0))

(event `Part2`
  (`/Game/ProjectContents/BP/BP_FunctionLib.SetupDialogManagerCycle` (`self.DialogManager`) (`self.StudentE Actor`) (`self.StudentE1`) self))

(event `Cupboard Minigame End`
  ;[1 1 1] CupboardMinigame
  (`GameplayStatics.PlaySound2D` "/Game/ProjectContents/SFX/SFX_Pickup.SFX_Pickup" 1.0 1.0 0.0 null null)
  (`AudioComponent.SetPaused` (`self.BGM`) false)
  (`self.HandleMOveCameraLeft`)
  (`KismetSystemLibrary.Delay` 3.0)
  (set `PlayerController.bShowMouseCursor` false (`GameplayStatics.GetPlayerController` 0))
  (set `self.isCupboardClear` true)
  (`self.CheckMinigameClear`))

(event `Part3`
  (`/Game/ProjectContents/BP/BP_FunctionLib.SetupDialogManagerCycle` (`self.DialogManager`) (`self.StaffActor`) (`self.Staff`) self))

(event `Part4`
  (`/Game/ProjectContents/BP/BP_FunctionLib.SetupDialogManagerCycle` (`self.DialogManager`) (`self.StudentF Actpr`) (`self.StudentF1`) self))

(event `Handle Change Camera`
  (bind _returnvalue (`self.K2_GetActorLocation` (`GameplayStatics.GetPlayerPawn` 0)))
  ;[1 1 1] Handle Switch Player with Dummy Actor
  (bind _returnvalue_2 (`|SpawnActorFromClass` "/Game/ProjectContents/BP/Objects/BP_DummyActor.BP_DummyActor_C" (`KismetMathLibrary.MakeTransform` _returnvalue) "Undefined" "OverrideRootScale" null null))
  (set `self.DummyActor` _returnvalue_2)
  (bind _returnvalue_3 (`GameplayStatics.GetActorOfClass` "/Game/ProjectContents/BP/LevelActors/BP_FollowCamera.BP_FollowCamera_C"))
  (set `/Game/ProjectContents/BP/LevelActors/BP_FollowCamera.ActorToFollow` _returnvalue_2 _returnvalue_3)
  (`KismetSystemLibrary.PrintString` "Switched ActorToFollow")
  (set `self.MinigameCameraStart` _returnvalue)
  (set `self.MinigameCameraEnd` (+ _returnvalue (300.0 0.0 0.0)))
  (`self.DisableInput` (`GameplayStatics.GetPlayerPawn` 0) (`GameplayStatics.GetPlayerController` 0)))

(event `Part5`
  (`/Game/ProjectContents/BP/BP_FunctionLib.SetupDialogManagerCycle` (`self.DialogManager`) (`self.StaffActor`) (`self.Staff1`) self))

(event `Part6`
  (`/Game/ProjectContents/BP/BP_FunctionLib.SetupDialogManagerCycle` (`self.DialogManager`) (`self.StudentE Actor`) (`self.StudentE2`) self))

(event `HandleMoveCameraRight`
  ;[1 1 1] Handle Move CAmera Right
  (bind (_direction _alpha) (`Timeline|Timeline_0` :!via `PlayFromStart`)
    (:`Update`
      (`self.K2_SetActorLocation` (`self.DummyActor`) (`KismetMathLibrary.VLerp` (`self.MinigameCameraStart`) (`self.MinigameCameraEnd`) _alpha) false false))
    (:`Finished`
      (`AudioComponent.SetPaused` (`self.BGM`) true))))

(event `Part7`
  (`/Game/ProjectContents/BP/BP_FunctionLib.SetupDialogManagerCycle` (`self.DialogManager`) (`self.StudentF Actpr`) (`self.StudentF2`) self))

(event `Part8`
  (bind _studente_actor (`self.StudentE Actor`))
  (bind _studentf_actpr (`self.StudentF Actpr`))
  (bind _bigsisteractor (`self.BigSisterActor`))
  (bind _returnvalue (`self.K2_GetActorLocation` _bigsisteractor))
  (`/Game/ProjectContents/BP/BP_FunctionLib.Flip FlipBook` _studente_actor)
  (bind _asbp_npcactor_base (cast `/Game/ProjectContents/BP/NPC/BP_NPCActorBase` _studente_actor))
  (`/Game/ProjectContents/BP/NPC/BP_NPCActorBase.MoveNPC Event` _asbp_npcactor_base (`self.K2_GetActorLocation` _studente_actor) (`self.LevelExit Location`))
  (`/Game/ProjectContents/BP/BP_FunctionLib.Flip FlipBook` _studentf_actpr)
  (bind _asbp_npcactor_base_2 (cast `/Game/ProjectContents/BP/NPC/BP_NPCActorBase` _studentf_actpr))
  (`/Game/ProjectContents/BP/NPC/BP_NPCActorBase.MoveNPC Event` _asbp_npcactor_base_2 (`self.K2_GetActorLocation` _studentf_actpr) (`self.LevelExit Location`))
  (`KismetSystemLibrary.Delay` 1.0)
  (bind _asbp_npcactor_base_3 (cast `/Game/ProjectContents/BP/NPC/BP_NPCActorBase` _bigsisteractor))
  (`/Game/ProjectContents/BP/NPC/BP_NPCActorBase.MoveNPC Event` _asbp_npcactor_base_3 _returnvalue (- _returnvalue (350.0 0.0 0.0)))
  (`KismetSystemLibrary.Delay` 3.0)
  (`self.K2_DestroyActor` (`self.StudentE Actor`))
  (`self.K2_DestroyActor` (`self.StudentF Actpr`))
  (`/Game/ProjectContents/BP/BP_FunctionLib.SetupDialogManagerCycle` (`self.DialogManager`) (`self.BigSisterActor`) (`self.Sister1`) self))

(event `HandleMOveCameraLeft`
  ;[1 1 1] Handle Move Camera Left
  (bind (_direction _alpha) (`Timeline|Timeline_1` :!via `PlayFromStart`)
    (:`Update`
      (`self.K2_SetActorLocation` (`self.DummyActor`) (`KismetMathLibrary.VLerp` (`self.MinigameCameraEnd`) (`self.MinigameCameraStart`) _alpha) false false))
    (:`Finished`
      (bind _returnvalue (`GameplayStatics.GetActorOfClass` "/Game/ProjectContents/BP/LevelActors/BP_FollowCamera.BP_FollowCamera_C"))
      (set `/Game/ProjectContents/BP/LevelActors/BP_FollowCamera.ActorToFollow` (`GameplayStatics.GetPlayerPawn` 0) _returnvalue)
      (`self.EnableInput` (`GameplayStatics.GetPlayerPawn` 0) (`GameplayStatics.GetPlayerController` 0))
      (`self.K2_DestroyActor` (`self.DummyActor`)))))

(event `Part9`
  (`/Game/ProjectContents/BP/BP_FunctionLib.SetupDialogManagerCycle` (`self.DialogManager`) (`self.StaffActor`) (`self.Staff2`) self))

(event `Part10`
  (bind _staffactor (`self.StaffActor`))
  (`/Game/ProjectContents/BP/BP_FunctionLib.Flip FlipBook` _staffactor)
  (bind _asbp_npcactor_base (cast `/Game/ProjectContents/BP/NPC/BP_NPCActorBase` _staffactor))
  (`/Game/ProjectContents/BP/NPC/BP_NPCActorBase.MoveNPC Event` _asbp_npcactor_base (`self.K2_GetActorLocation` _staffactor) (`self.Staff EndMove`))
  (`KismetSystemLibrary.Delay` 3.0)
  (`self.Spawn Minigames`)
  (`self.DisableInput` (`GameplayStatics.GetPlayerController` 0))
  (`/Game/ProjectContents/BP/BP_FunctionLib.EnablePlayerInput`))

(fn `LevelSetup`
  (for (_array_element _array_index) (`self.LevelActors`)
    (bind _returnvalue (`|SpawnActorFromClass` _array_element (`|GetArrayItem` (`self.ActorSpawns`) _array_index) "Undefined" "OverrideRootScale" null null))
    (switch `int` _array_index
      (:`0`
        (set `self.StaffActor` _returnvalue))
      (:`1`
        (set `self.BigSisterActor` _returnvalue))
      (:`3`
        (set `self.StudentE Actor` _returnvalue))
      (:`4`
        (set `self.StudentF Actpr` _returnvalue))))
  (`/Game/ProjectContents/BP/BP_FunctionLib.Flip FlipBook` (`self.BigSisterActor`))
  (`self.K2_SetActorLocation` (`GameplayStatics.GetPlayerPawn` 0) (`self.PlayerSpawn`) false false)
  (`/Game/ProjectContents/BP/BP_FunctionLib.Flip FlipBook` (`self.StudentE Actor`))
  (`/Game/ProjectContents/BP/BP_FunctionLib.Flip FlipBook` (`self.StudentF Actpr`))
  (bind _returnvalue_2 (`GameplayStatics.SpawnSound2D` "/Game/ProjectContents/Music/BGM_HallwayClassroom.BGM_HallwayClassroom" 1.0 1.0 0.0 null false false))
  (set `self.BGM` _returnvalue_2))

(fn `MoveToNextPart`
  (`self.DisableInput` (`GameplayStatics.GetPlayerController` 0))
  (bind _result (`/Engine/EditorBlueprintResources/StandardMacros.IncrementInt` (`self.CurrentPart`))
    (:`  `
      (bind _asbp_game_instance (cast `/Game/ProjectContents/BP/BP_GameInstance` (`GameplayStatics.GetGameInstance`)))
      (bind _output_get (set `/Game/ProjectContents/BP/BP_GameInstance.ScenePart` _result _asbp_game_instance))
      (switch `int` _output_get
        (:`1`
          (`self.Part1`))
        (:`2`
          (`self.Part2`))
        (:`3`
          (`self.Part3`))
        (:`4`
          (`self.Part4`))
        (:`5`
          (`self.Part5`))
        (:`6`
          (`self.Part6`))
        (:`7`
          (`self.Part7`))
        (:`8`
          (`self.Part8`))
        (:`9`
          (`self.Part9`))
        (:`10`
          (`self.Part10`))
        (:`11`
          (`self.Part11`))
        (:`12`
          (`self.Part12`))
        (:`13`
          (`self.Part13`))
        (:`14`
          (`self.Part14`))
        (:`15`
          (`self.Part15`))
        (:`16`
          (`self.Part16`))))))

(fn `UserConstructionScript`)