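; Scene manager for Scene 12 (House), a scripted dialogue between Mother and BigSister ending with the sister walking away.
; On a passing scene-index check, it spawns both NPCs, hides the level-move actor and finds the dialog manager.
; The Interact key cycles dialogue, then advances numbered parts through the GameInstance's ScenePart.
; The final part timeline-lerps the sister's walk, destroys her, re-enables player input and reveals the level-move actor.
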(event `InputAction|Interact`
  (params (Key :type "Key Structure"))
  ;[1 1 1] OnInteract
  (:`Pressed`
    (bind _asbp_game_instance (cast `/Game/ProjectContents/BP/BP_GameInstance` (`GameplayStatics.GetGameInstance`)))
    (if (`/Game/ProjectContents/BP/BP_GameInstance.isViewingScene` _asbp_game_instance)
      (if (`/Game/ProjectContents/BP/LevelActors/BP_DialogManager.isDIalogFinished` (`self.Level Dialog Manager`))
        (set `/Game/ProjectContents/BP/LevelActors/BP_DialogManager.isDIalogFinished` false (`self.Level Dialog Manager`))
        (bind _asbp_game_instance_2 (cast `/Game/ProjectContents/BP/BP_GameInstance` (`GameplayStatics.GetGameInstance`)))
        (set `/Game/ProjectContents/BP/BP_GameInstance.isViewingScene` false _asbp_game_instance_2)
        (`KismetSystemLibrary.PrintString` "DialogFinished")
        (`self.MoveToNextPart`)
        (else
          (`/Game/ProjectContents/BP/LevelActors/BP_DialogManager.Test-CycleOnKey` (`self.Level Dialog Manager`)))))))

(event `self.ReceiveBeginPlay`
  (bind _iscorrectscene (`/Game/ProjectContents/BP/BP_FunctionLib.CheckSceneIndex` (`self.CurrentScene`)))
  (if _iscorrectscene
    (`self.LevelSetup`)
    (bind _returnvalue (`GameplayStatics.GetActorOfClass` "/Game/ProjectContents/BP/LevelActors/BP_DialogManager.BP_DialogManager_C"))
    (set `self.Level Dialog Manager` _returnvalue)))

(event `Part0`
  (`self.DisableInput` (`GameplayStatics.GetPlayerPawn` 0) (`GameplayStatics.GetPlayerController` 0))
  (`/Game/ProjectContents/BP/BP_FunctionLib.SetupDialogManagerCycle` (`self.Level Dialog Manager`) (`self.Mother`) (`self.Mother1`) self))

(event `Handle Start Dialog`
  (bind _mother (`self.Mother`))
  ;[1 1 1] Handle Dialog
  (`self.DisableInput` (`GameplayStatics.GetPlayerPawn` 0) (`GameplayStatics.GetPlayerController` 0))
  (bind _dialog_delay (`/Game/ProjectContents/BP/LevelActors/BP_DialogManager.Display Dialog` (`self.Level Dialog Manager`) _mother (`self.Mother1`) (`self.TextDelay`)))
  (`KismetSystemLibrary.Delay` _dialog_delay)
  (`/Game/ProjectContents/BP/BP_FunctionLib.Flip FlipBook` _mother)
  (`KismetSystemLibrary.Delay` 1.0)
  (bind _dialog_delay_2 (`/Game/ProjectContents/BP/LevelActors/BP_DialogManager.Display Dialog` (`self.Level Dialog Manager`) (`self.BigSister`) (`self.Big Sister`) (`self.TextDelay`)))
  (`KismetSystemLibrary.Delay` _dialog_delay_2)
  (`self.Handle Sister Move`))

(event `Part1`
  (`/Game/ProjectContents/BP/BP_FunctionLib.Flip FlipBook` (`self.Mother`))
  (`/Game/ProjectContents/BP/BP_FunctionLib.SetupDialogManagerCycle` (`self.Level Dialog Manager`) (`self.BigSister`) (`self.Big Sister`) self))

(event `Handle Sister Move`
  ;[1 1 1] Handle Move
  (bind _asbp_npcactor_big_sister (cast `/Game/ProjectContents/BP/NPC/BP_NPCActor_BigSister` (`self.BigSister`)))
  (`/Game/ProjectContents/BP/BP_FunctionLib.Flip FlipBook` _asbp_npcactor_big_sister)
  (`PaperFlipbookComponent.SetFlipbook` (`/Game/ProjectContents/BP/NPC/BP_NPCActorBase.PaperFlipbook` _asbp_npcactor_big_sister) "/Game/ProjectContents/Character/Joylene/FB_Joylene_BigSister_Walk.FB_Joylene_BigSister_Walk")
  (bind (_direction _alpha) (`Timeline|MoveTL` :!via `PlayFromStart`)
    (:`Update`
      (`self.K2_SetActorLocation` _asbp_npcactor_big_sister (`KismetMathLibrary.VLerp` (`self.Sister Start`) (`self.Sister End`) _alpha) false false))
    (:`Finished`
      (`PaperFlipbookComponent.SetFlipbook` (`/Game/ProjectContents/BP/NPC/BP_NPCActorBase.PaperFlipbook` _asbp_npcactor_big_sister) "/Game/ProjectContents/Character/Joylene/FB_Joylene_BigSister_Idle.FB_Joylene_BigSister_Idle")
      (`KismetSystemLibrary.Delay` 1.5)
      (`self.K2_DestroyActor` _asbp_npcactor_big_sister)
      (`self.EnableInput` (`GameplayStatics.GetPlayerPawn` 0) (`GameplayStatics.GetPlayerController` 0)))))

(event `Part2`
  (`self.Handle Sister Move`)
  (`KismetSystemLibrary.Delay` 3.0)
  (bind _returnvalue (`GameplayStatics.GetActorOfClass` "/Game/ProjectContents/BP/LevelActors/BP_MoveLevels.BP_MoveLevels_C"))
  (`self.SetActorHiddenInGame` _returnvalue false))

(fn `LevelSetup`
  (bind _bigsister (`self.BigSister`))
  (for (_array_element _array_index) (`self.LevelActors`)
    (bind _returnvalue (`|SpawnActorFromClass` _array_element (`|GetArrayItem` (`self.ActorSpawns`) _array_index) "Undefined" "OverrideRootScale" null null))
    (switch `int` _array_index
      (:`0`
        (set `self.BigSister` _returnvalue))
      (:`1`
        (set `self.Mother` _returnvalue))))
  (`/Game/ProjectContents/BP/BP_FunctionLib.Flip FlipBook` _bigsister)
  (set `self.Sister Start` (`self.K2_GetActorLocation` _bigsister))
  (bind _returnvalue_2 (`GameplayStatics.GetActorOfClass` "/Game/ProjectContents/BP/LevelActors/BP_MoveLevels.BP_MoveLevels_C"))
  (`self.SetActorHiddenInGame` _returnvalue_2 true))

(fn `MoveToNextPart`
  (`self.DisableInput` (`GameplayStatics.GetPlayerController` 0))
  (bind _result (`/Engine/EditorBlueprintResources/StandardMacros.IncrementInt` (`self.CurrentPart`))
    (:`  `
      (bind _asbp_game_instance (cast `/Game/ProjectContents/BP/BP_GameInstance` (`GameplayStatics.GetGameInstance`)))
      (bind _output_get (set `/Game/ProjectContents/BP/BP_GameInstance.ScenePart` _result _asbp_game_instance))
      (switch `int` _output_get
        (:`1`
          (`self.Part1`))
        (:`2`
          (`self.Part2`))))))

(fn `UserConstructionScript`)