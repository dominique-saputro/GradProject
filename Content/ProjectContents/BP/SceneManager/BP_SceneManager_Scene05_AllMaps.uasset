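; Scene manager for story Scene 5, an after-school sequence where the big sister NPC moves through classroom, hallways and staffroom, talking with a teacher there.
; LevelSetup spawns actors and triggers by level name and GameInstance progress flags, which persist across level loads.
; OnPlayerOverlap starts each level's dialogue or NPC walk.
; Interact cycles dialogue and advances numbered parts, while the final upstairs walk moves the game to the next scene.
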(event `self.ReceiveBeginPlay`
  (bind _iscorrectscene (`/Game/ProjectContents/BP/BP_FunctionLib.CheckSceneIndex` (`self.CurrentScene`)))
  (if _iscorrectscene
    (`self.LevelSetup`)
    (bind _returnvalue (`GameplayStatics.GetActorOfClass` "/Game/ProjectContents/BP/LevelActors/BP_DialogManager.BP_DialogManager_C"))
    (set `self.Level Dialog Manager` _returnvalue)))

(event `InputAction|Interact`
  (params (Key :type "Key Structure"))
  ;[1 1 1] OnInteract
  (:`Pressed`
    (bind _asbp_game_instance (cast `/Game/ProjectContents/BP/BP_GameInstance` (`GameplayStatics.GetGameInstance`)))
    (if (`/Game/ProjectContents/BP/BP_GameInstance.isViewingScene` _asbp_game_instance)
      (if (`/Game/ProjectContents/BP/LevelActors/BP_DialogManager.isDIalogFinished` (`self.Level Dialog Manager`))
        (set `/Game/ProjectContents/BP/LevelActors/BP_DialogManager.isDIalogFinished` false (`self.Level Dialog Manager`))
        (bind _asbp_game_instance_2 (cast `/Game/ProjectContents/BP/BP_GameInstance` (`GameplayStatics.GetGameInstance`)))
        (set `/Game/ProjectContents/BP/BP_GameInstance.isViewingScene` false _asbp_game_instance_2)
        (`KismetSystemLibrary.PrintString` "DialogFinished")
        (`self.MoveToNextPart`)
        (else
          (`/Game/ProjectContents/BP/LevelActors/BP_DialogManager.Test-CycleOnKey` (`self.Level Dialog Manager`)))))))

(event `Handle Classroom`
  ;[1 1 1] Handle Classroom
  (`/Game/ProjectContents/BP/BP_FunctionLib.DisablePlayerInput`)
  (bind _asbp_npcactor_base (cast `/Game/ProjectContents/BP/NPC/BP_NPCActorBase` (`self.BigSister`)))
  (`/Game/ProjectContents/BP/NPC/BP_NPCActorBase.MoveNPC Event` _asbp_npcactor_base (`self.ClassroomStart`) (`self.Classroom End`))
  (`KismetSystemLibrary.Delay` 3.0)
  (`self.K2_DestroyActor` _asbp_npcactor_base)
  (bind _asbp_game_instance (cast `/Game/ProjectContents/BP/BP_GameInstance` (`GameplayStatics.GetGameInstance`)))
  (set `/Game/ProjectContents/BP/BP_GameInstance.isScene5PassedClassroom` true _asbp_game_instance)
  (`self.TeleportPLayer`))

(event `TeleportPLayer`
  (bind _returnvalue (`|CreateWidget` "/Game/ProjectContents/BP/Widgets/WBP_FadeBlack.WBP_FadeBlack_C" (`GameplayStatics.GetPlayerController` 0)))
  (`UserWidget.AddToViewport` _returnvalue 0)
  (`/Game/ProjectContents/BP/Widgets/WBP_FadeBlack.FadeToBlack` _returnvalue)
  (`KismetSystemLibrary.Delay` 0.5)
  (`GameplayStatics.OpenLevel` "Game_Staffroom"))

(event `Part0`
  (`/Game/ProjectContents/BP/BP_FunctionLib.SetupDialogManagerCycle` (`self.Level Dialog Manager`) (`self.BigSister`) (`self.Big Sister0`) self))

(event `Handle Hallway1`
  ;[1 1 1] Handle Hallway 1
  (bind _asbp_npcactor_base (cast `/Game/ProjectContents/BP/NPC/BP_NPCActorBase` (`self.BigSister`)))
  (`/Game/ProjectContents/BP/NPC/BP_NPCActorBase.MoveNPC Event` _asbp_npcactor_base (`self.Hallway Start`) (`self.Hallway End`))
  (`KismetSystemLibrary.Delay` 3.0)
  (`self.K2_DestroyActor` _asbp_npcactor_base)
  (bind _asbp_game_instance (cast `/Game/ProjectContents/BP/BP_GameInstance` (`GameplayStatics.GetGameInstance`)))
  (set `/Game/ProjectContents/BP/BP_GameInstance.isScene5PassedHallway` true _asbp_game_instance))

(event `Part1`
  (`self.Handle Classroom`))

(event `Handle Upstairs Hallway1`
  ;[1 1 1] Handle Upstairs Hallway 1
  (bind _asbp_npcactor_base (cast `/Game/ProjectContents/BP/NPC/BP_NPCActorBase` (`self.BigSister`)))
  (`/Game/ProjectContents/BP/BP_FunctionLib.Flip FlipBook` _asbp_npcactor_base)
  (`/Game/ProjectContents/BP/NPC/BP_NPCActorBase.MoveNPC Event` _asbp_npcactor_base (`self.Upstairs Start`) (`self.Upstairs End`))
  (`KismetSystemLibrary.Delay` 3.0)
  (`self.K2_DestroyActor` _asbp_npcactor_base)
  (bind _asbp_game_instance (cast `/Game/ProjectContents/BP/BP_GameInstance` (`GameplayStatics.GetGameInstance`)))
  (set `/Game/ProjectContents/BP/BP_GameInstance.isScene5PassedClassroom` false _asbp_game_instance)
  (set `/Game/ProjectContents/BP/BP_GameInstance.isScene5PassedHallway` false _asbp_game_instance))

(event `Part2`
  (set `self.CurrentPart` 2)
  (`self.Handle StaffRoom`)
  (`/Game/ProjectContents/BP/BP_FunctionLib.SetupDialogManagerCycle` (`self.Level Dialog Manager`) (`self.Teacher`) (`self.Teacher1`) self)
  (`/Game/ProjectContents/BP/BP_FunctionLib.DisablePlayerInput`)
  (`KismetSystemLibrary.Delay` 3.0)
  (`/Game/ProjectContents/BP/BP_FunctionLib.EnablePlayerInput`))

(event `Part3`
  (`/Game/ProjectContents/BP/BP_FunctionLib.SetupDialogManagerCycle` (`self.Level Dialog Manager`) (`self.BigSister`) (`self.Big Sister2`) self))

(event `Handle StaffRoom`
  ;[1 1 1] Handle Staffroom Start
  (bind _asbp_npcactor_base (cast `/Game/ProjectContents/BP/NPC/BP_NPCActorBase` (`self.BigSister`)))
  (`/Game/ProjectContents/BP/BP_FunctionLib.Flip FlipBook` _asbp_npcactor_base)
  (`/Game/ProjectContents/BP/NPC/BP_NPCActorBase.MoveNPC Event` _asbp_npcactor_base (`self.Staffroom Start`) (`self.Staffroom End`))
  (bind _asbp_game_instance (cast `/Game/ProjectContents/BP/BP_GameInstance` (`GameplayStatics.GetGameInstance`)))
  (set `/Game/ProjectContents/BP/BP_GameInstance.isScene5PassedStaffroom` true _asbp_game_instance))

(event `Part4`
  (`/Game/ProjectContents/BP/BP_FunctionLib.SetupDialogManagerCycle` (`self.Level Dialog Manager`) (`self.Teacher`) (`self.Teacher2`) self))

(event `Part5`
  (`/Game/ProjectContents/BP/BP_FunctionLib.SetupDialogManagerCycle` (`self.Level Dialog Manager`) (`self.BigSister`) (`self.Big Sister3`) self))

(event `Handle Staffroom SisterMove`
  (bind _asbp_npcactor_base (cast `/Game/ProjectContents/BP/NPC/BP_NPCActorBase` (`self.BigSister`)))
  (`/Game/ProjectContents/BP/BP_FunctionLib.Flip FlipBook` _asbp_npcactor_base)
  (`/Game/ProjectContents/BP/NPC/BP_NPCActorBase.MoveNPC Event` _asbp_npcactor_base (`self.Staffroom End`) (`self.Staffroom Start`))
  (`KismetSystemLibrary.Delay` 3.0)
  (`self.K2_DestroyActor` _asbp_npcactor_base)
  (bind _returnvalue (`GameplayStatics.GetActorOfClass` "/Game/ProjectContents/BP/LevelActors/BP_MoveLevels.BP_MoveLevels_C"))
  (`self.SetActorHiddenInGame` _returnvalue false))

(event `Part6`
  (`/Game/ProjectContents/BP/BP_FunctionLib.SetupDialogManagerCycle` (`self.Level Dialog Manager`) (`self.Teacher`) (`self.Teacher3`) self))

(event `Handle Upstairs Hallway2`
  ;[1 1 1] Handle Upstairs Hallway 2
  (bind _asbp_npcactor_base (cast `/Game/ProjectContents/BP/NPC/BP_NPCActorBase` (`self.BigSister`)))
  (`/Game/ProjectContents/BP/NPC/BP_NPCActorBase.MoveNPC Event` _asbp_npcactor_base (`self.Upstairs End`) (`self.Upstairs Start`))
  (`KismetSystemLibrary.Delay` 3.0)
  (`self.K2_DestroyActor` _asbp_npcactor_base)
  (bind _asbp_game_instance (cast `/Game/ProjectContents/BP/BP_GameInstance` (`GameplayStatics.GetGameInstance`)))
  (`/Game/ProjectContents/BP/BP_GameInstance.MoveToNextScene` _asbp_game_instance)
  (`KismetSystemLibrary.PrintString` "Scene5 done"))

(event `Part7`
  (`self.Handle Staffroom SisterMove`))

(fn `LevelSetup`
  (bind _returnvalue (`GameplayStatics.GetCurrentLevelName` true))
  (switch `string` _returnvalue
    (:`Game_Classroom`
      (bind _returnvalue_2 (`|SpawnActorFromClass` "/Game/ProjectContents/BP/NPC/BP_NPCActor_BigSister.BP_NPCActor_BigSister_C" (`KismetMathLibrary.MakeTransform` (`self.ClassroomStart`) (struct) (2.0 2.0 2.0)) "Undefined" "OverrideRootScale" null null))
      (set `self.BigSister` _returnvalue_2)
      (`|SpawnActorFromClass` "/Game/ProjectContents/BP/Triggers/BP_Scene05_BIgSisterMove_Trigger.BP_Scene05_BIgSisterMove_Trigger_C" (`KismetMathLibrary.MakeTransform` (`self.ClassroomStart`)) "Undefined" "OverrideRootScale" null null)
      (`GameplayStatics.PlaySound2D` "/Game/ProjectContents/SFX/SFX_SchoolBell.SFX_SchoolBell" 1.0 1.0 0.0 null null)
      (bind _returnvalue_3 (`|CreateWidget` "/Game/ProjectContents/BP/Widgets/WBP_TextTransition.WBP_TextTransition_C" (`GameplayStatics.GetPlayerController` 0)))
      (`UserWidget.AddToViewport` _returnvalue_3 0)
      (`/Game/ProjectContents/BP/Widgets/WBP_TextTransition.Set Display Text` _returnvalue_3 "放課後"))
    (:`Game_Hallway`
      (bind _asbp_game_instance (cast `/Game/ProjectContents/BP/BP_GameInstance` (`GameplayStatics.GetGameInstance`)))
      (if (`/Game/ProjectContents/BP/BP_GameInstance.isScene5PassedClassroom` _asbp_game_instance)
        (bind _returnvalue_4 (`|SpawnActorFromClass` "/Game/ProjectContents/BP/NPC/BP_NPCActor_BigSister.BP_NPCActor_BigSister_C" (`KismetMathLibrary.MakeTransform` (`self.Hallway Start`) (struct) (2.1 2.1 2.1)) "Undefined" "OverrideRootScale" null null))
        (set `self.BigSister` _returnvalue_4)
        (`|SpawnActorFromClass` "/Game/ProjectContents/BP/Triggers/BP_Scene05_BIgSisterMove_Trigger.BP_Scene05_BIgSisterMove_Trigger_C" (`KismetMathLibrary.MakeTransform` (`self.Hallway Start`) (struct) (2.0 2.0 1.0)) "Undefined" "OverrideRootScale" null null)))
    (:`Game_Staff_Hallway`
      (bind _asbp_game_instance_2 (cast `/Game/ProjectContents/BP/BP_GameInstance` (`GameplayStatics.GetGameInstance`)))
      (if (`/Game/ProjectContents/BP/BP_GameInstance.isScene5PassedHallway` _asbp_game_instance_2)
        (bind _returnvalue_5 (`|SpawnActorFromClass` "/Game/ProjectContents/BP/NPC/BP_NPCActor_BigSister.BP_NPCActor_BigSister_C" (`KismetMathLibrary.MakeTransform` (`self.Upstairs Start`) (struct) (2.1 2.1 2.1)) "Undefined" "OverrideRootScale" null null))
        (set `self.BigSister` _returnvalue_5)
        (`|SpawnActorFromClass` "/Game/ProjectContents/BP/Triggers/BP_Scene05_BIgSisterMove_Trigger.BP_Scene05_BIgSisterMove_Trigger_C" (`KismetMathLibrary.MakeTransform` (`self.Upstairs Start`) (struct) (2.0 2.0 2.0)) "Undefined" "OverrideRootScale" null null)
        (else
          (bind _asbp_game_instance_3 (cast `/Game/ProjectContents/BP/BP_GameInstance` (`GameplayStatics.GetGameInstance`)))
          (if (`/Game/ProjectContents/BP/BP_GameInstance.isScene5PassedStaffroom` _asbp_game_instance_3)
            (bind _returnvalue_6 (`|SpawnActorFromClass` "/Game/ProjectContents/BP/NPC/BP_NPCActor_BigSister.BP_NPCActor_BigSister_C" (`KismetMathLibrary.MakeTransform` (`self.Upstairs End`) (struct) (2.1 2.1 2.1)) "Undefined" "OverrideRootScale" null null))
            (set `self.BigSister` _returnvalue_6)
            (`|SpawnActorFromClass` "/Game/ProjectContents/BP/Triggers/BP_Scene05_BIgSisterMove_Trigger.BP_Scene05_BIgSisterMove_Trigger_C" (`KismetMathLibrary.MakeTransform` (`self.Upstairs End`) (struct) (2.0 2.0 2.0)) "Undefined" "OverrideRootScale" null null)))))
    (:`Game_Staffroom`
      (for (_array_element _array_index) (`self.LevelActors`)
        (bind _returnvalue_7 (`|SpawnActorFromClass` _array_element (`|GetArrayItem` (`self.ActorSpawns`) _array_index) "Undefined" "OverrideRootScale" null null))
        (switch `int` _array_index
          (:`0`
            (set `self.BigSister` _returnvalue_7))
          (:`1`
            (set `self.Teacher` _returnvalue_7))))
      (bind _returnvalue_8 (`GameplayStatics.GetActorOfClass` "/Game/ProjectContents/BP/LevelActors/BP_MoveLevels.BP_MoveLevels_C"))
      (`self.SetActorHiddenInGame` _returnvalue_8 true)
      (`GameplayStatics.PlaySound2D` "/Game/ProjectContents/Music/Final/School_office.School_office" 1.0 1.0 0.0 null null))))

(fn `MoveToNextPart`
  (`self.DisableInput` (`GameplayStatics.GetPlayerController` 0))
  (bind _result (`/Engine/EditorBlueprintResources/StandardMacros.IncrementInt` (`self.CurrentPart`))
    (:`  `
      (bind _asbp_game_instance (cast `/Game/ProjectContents/BP/BP_GameInstance` (`GameplayStatics.GetGameInstance`)))
      (bind _output_get (set `/Game/ProjectContents/BP/BP_GameInstance.ScenePart` _result _asbp_game_instance))
      (switch `int` _output_get
        (:`1`
          (`self.Part1`))
        (:`2`
          (`self.Part2`))
        (:`3`
          (`self.Part3`))
        (:`4`
          (`self.Part4`))
        (:`5`
          (`self.Part5`))
        (:`6`
          (`self.Part6`))
        (:`7`
          (`self.Part7`))))))

(fn `OnPlayerOverlap`
  (bind _returnvalue (`GameplayStatics.GetCurrentLevelName` true))
  (switch `string` _returnvalue
    (:`Game_Classroom`
      (`self.Part0`))
    (:`Game_Hallway`
      (bind _asbp_game_instance (cast `/Game/ProjectContents/BP/BP_GameInstance` (`GameplayStatics.GetGameInstance`)))
      (if (`/Game/ProjectContents/BP/BP_GameInstance.isScene5PassedClassroom` _asbp_game_instance)
        (`self.Handle Hallway1`)))
    (:`Game_Staff_Hallway`
      (bind _asbp_game_instance_2 (cast `/Game/ProjectContents/BP/BP_GameInstance` (`GameplayStatics.GetGameInstance`)))
      (if (`/Game/ProjectContents/BP/BP_GameInstance.isScene5PassedHallway` _asbp_game_instance_2)
        (`self.Handle Upstairs Hallway1`)
        (else
          (bind _asbp_game_instance_3 (cast `/Game/ProjectContents/BP/BP_GameInstance` (`GameplayStatics.GetGameInstance`)))
          (if (`/Game/ProjectContents/BP/BP_GameInstance.isScene5PassedStaffroom` _asbp_game_instance_3)
            (`self.Handle Upstairs Hallway2`)))))
    (:`Game_Staffroom`
      (`self.Part2`))))

(fn `UserConstructionScript`)