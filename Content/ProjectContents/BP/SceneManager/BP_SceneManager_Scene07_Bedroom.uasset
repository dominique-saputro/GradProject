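; Scene manager for the Scene 07 bedroom, a scripted dialog sequence that ends by loading the park level.
; On a matching scene index it spawns the actors and positions the player and camera limit.
; Numbered Part events, advanced by MoveToNextPart, run dialog through BP_DialogManager, which the Interact key cycles.
; Parts cover a lighting timeline with faded switch to a dirty background, three students talking and leaving, then both sisters' dialog.
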(event `self.ReceiveBeginPlay`
  (bind _iscorrectscene (`/Game/ProjectContents/BP/BP_FunctionLib.CheckSceneIndex` (`self.CurrentScene`)))
  (if _iscorrectscene
    (`self.LevelSetup`)
    (bind _returnvalue (`GameplayStatics.GetActorOfClass` "/Game/ProjectContents/BP/LevelActors/BP_DialogManager.BP_DialogManager_C"))
    (set `self.Level Dialog Manager` _returnvalue)))

(event `InputAction|Interact`
  (params (Key :type "Key Structure"))
  (bind _level_dialog_manager (`self.Level Dialog Manager`))
  ;[1 1 1] OnInteract
  (:`Pressed`
    (if (`/Game/ProjectContents/BP/LevelActors/BP_DialogManager.isDIalogFinished` _level_dialog_manager)
      (set `/Game/ProjectContents/BP/LevelActors/BP_DialogManager.isDIalogFinished` false _level_dialog_manager)
      (bind _asbp_game_instance (cast `/Game/ProjectContents/BP/BP_GameInstance` (`GameplayStatics.GetGameInstance`)))
      (set `/Game/ProjectContents/BP/BP_GameInstance.isViewingScene` false _asbp_game_instance)
      (`KismetSystemLibrary.PrintString` "DialogFinished")
      (`self.MoveToNextPart`)
      (else
        (`/Game/ProjectContents/BP/LevelActors/BP_DialogManager.Test-CycleOnKey` _level_dialog_manager)))))

(event `HandleStudentMove`
  ;[1 1 1] Handle End Sene
  (for _index (range 3)
    (bind _output (`|GetArrayItem` (`self.Students`) _index))
    (bind _asbp_npcactor_base (cast `/Game/ProjectContents/BP/NPC/BP_NPCActorBase` _output))
    (`/Game/ProjectContents/BP/NPC/BP_NPCActorBase.MoveNPC Event` _asbp_npcactor_base (`self.K2_GetActorLocation` _output) (`self.StudentEnd`)))
  (`KismetSystemLibrary.Delay` 3.5)
  (for _index_2 (range 3)
    (`self.K2_DestroyActor` (`|GetArrayItem` (`self.Students`) _index_2)))
  (`KismetSystemLibrary.Delay` 1.0)
  (`self.EnableInput` (`GameplayStatics.GetPlayerPawn` 0) (`GameplayStatics.GetPlayerController` 0)))

(event `HandleChangeBackground`
  ;[1 1 1] Handle Background Change
  (bind _returnvalue (`|CreateWidget` "/Game/ProjectContents/BP/Widgets/WBP_FadeBlack.WBP_FadeBlack_C" (`GameplayStatics.GetPlayerController` 0)))
  (`UserWidget.AddToViewport` _returnvalue 0)
  (`/Game/ProjectContents/BP/Widgets/WBP_FadeBlack.FadeToBlack` _returnvalue)
  (`KismetSystemLibrary.Delay` 0.5)
  (bind _returnvalue_2 (`GameplayStatics.GetActorOfClass` "/Game/ProjectContents/BP/Objects/BP_Scene7_Background.BP_Scene7_Background_C"))
  (`PaperSpriteComponent.SetSprite` (`/Game/ProjectContents/BP/Objects/BP_Scene7_Background.Background` _returnvalue_2) (`self.DirtyBackground`))
  (`Widget.RemoveFromParent` _returnvalue)
  (bind _returnvalue_3 (`|CreateWidget` "/Game/ProjectContents/BP/Widgets/WBP_FadeBlack.WBP_FadeBlack_C" (`GameplayStatics.GetPlayerController` 0)))
  (`UserWidget.AddToViewport` _returnvalue_3 0)
  (`/Game/ProjectContents/BP/Widgets/WBP_FadeBlack.FadeFromBlack` _returnvalue_3)
  (`KismetSystemLibrary.Delay` 1.0)
  (`Widget.RemoveFromParent` _returnvalue_3))

(event `Part0`
  (`self.ChangeLighting`)
  (`KismetSystemLibrary.Delay` 6.0)
  (`self.MoveToNextPart`))

(event `StartSIsterDialog`
  ;[1 1 1] Handle SIster Dialog
  (`KismetSystemLibrary.Delay` 2.0)
  (bind _dialog_delay (`/Game/ProjectContents/BP/LevelActors/BP_DialogManager.Display Dialog` (`self.Level Dialog Manager`) (`self.BigSister`) (`self.Big Sister`) (`self.TextDelay`)))
  (`KismetSystemLibrary.Delay` _dialog_delay))

(event `Part1`
  (`/Game/ProjectContents/BP/BP_FunctionLib.SetupDialogManagerCycle` (`self.Level Dialog Manager`) (`|GetArrayItem` (`self.Students`) 2) (`self.StudentC`) self))

(event `ChangeLighting`
  (bind (_direction _alpha) (`Timeline|Timeline_0`)
    (:`Update`
      (bind _returnvalue (`GameplayStatics.GetActorOfClass` "/Script/Engine.DirectionalLight"))
      (`LightComponent.SetIntensity` (`Light.LightComponent` _returnvalue) _alpha))
    (:`Finished`
      (`self.HandleChangeBackground`))))

(event `Part2`
  (`/Game/ProjectContents/BP/BP_FunctionLib.SetupDialogManagerCycle` (`self.Level Dialog Manager`) (`|GetArrayItem` (`self.Students`) 1) (`self.StudentB`) self))

(event `Part3`
  (`/Game/ProjectContents/BP/BP_FunctionLib.SetupDialogManagerCycle` (`self.Level Dialog Manager`) (`|GetArrayItem` (`self.Students`)) (`self.StudentA`) self))

(event `HandleSceneEnd`
  (bind _asbp_game_instance (cast `/Game/ProjectContents/BP/BP_GameInstance` (`GameplayStatics.GetGameInstance`)))
  (`/Game/ProjectContents/BP/BP_GameInstance.MoveToNextScene` _asbp_game_instance)
  (bind _returnvalue (`|CreateWidget` "/Game/ProjectContents/BP/Widgets/WBP_FadeBlack.WBP_FadeBlack_C" (`GameplayStatics.GetPlayerController` 0)))
  (`UserWidget.AddToViewport` _returnvalue 0)
  (`/Game/ProjectContents/BP/Widgets/WBP_FadeBlack.FadeToBlack` _returnvalue)
  (`KismetSystemLibrary.Delay` 0.5)
  (`GameplayStatics.OpenLevel` "Game_Park"))

(event `Part4`
  (`self.HandleStudentMove`)
  (`KismetSystemLibrary.Delay` 4.0)
  (bind _returnvalue (`|SpawnActorFromClass` "/Game/ProjectContents/BP/NPC/BP_NPCActor_LIttleSister.BP_NPCActor_LIttleSister_C" (`self.LittleSisterSpawn`) "Undefined" "OverrideRootScale" null null))
  (`/Game/ProjectContents/BP/BP_FunctionLib.Flip FlipBook` _returnvalue)
  (`/Game/ProjectContents/BP/BP_FunctionLib.SetupDialogManagerCycle` (`self.Level Dialog Manager`) _returnvalue (`self.LIttleSIster`) self))

(event `Part5`
  (`/Game/ProjectContents/BP/BP_FunctionLib.SetupDialogManagerCycle` (`self.Level Dialog Manager`) (`self.BigSister`) (`self.Big Sister`) self))

(event `Part6`
  (`self.HandleSceneEnd`))

(fn `LevelSetup`
  (for (_array_element _array_index) (`self.LevelActors`)
    (bind _returnvalue (`|SpawnActorFromClass` _array_element (`|GetArrayItem` (`self.ActorSpawns`) _array_index) "Undefined" "OverrideRootScale" null null))
    (if (`self.ActorHasTag` _returnvalue "Student")
      (`KismetArrayLibrary.Array_Add` (`self.Students`) _returnvalue)
      (elif (== _array_index 3)
        (set `self.BigSister` _returnvalue))))
  (`self.K2_SetActorLocation` (`GameplayStatics.GetPlayerPawn` 0) (`self.PlayerSpawn`) false false)
  (bind _returnvalue_2 (`GameplayStatics.GetActorOfClass` "/Game/ProjectContents/BP/LevelActors/BP_FollowCamera.BP_FollowCamera_C"))
  (set `/Game/ProjectContents/BP/LevelActors/BP_FollowCamera.MaxCameraX` -480.0 _returnvalue_2))

(fn `MoveToNextPart`
  (`self.DisableInput` (`GameplayStatics.GetPlayerController` 0))
  (bind _result (`/Engine/EditorBlueprintResources/StandardMacros.IncrementInt` (`self.CurrentPart`))
    (:`  `
      (switch `int` _result
        (:`1`
          (`self.Part1`))
        (:`2`
          (`self.Part2`))
        (:`3`
          (`self.Part3`))
        (:`4`
          (`self.Part4`))
        (:`5`
          (`self.Part5`))
        (:`6`
          (`self.Part6`))))))

(fn `UserConstructionScript`)