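; Scene manager for Scene 09 (Staffroom), running a scripted Teacher and BigSister dialogue with a tel-box minigame before fading to Game_House.
; On BeginPlay it spawns the cast, season widget and music, and restores the minigame setup when reloading at part 5.
; Interact cycles BP_DialogManager lines, and finished dialogue advances numbered Part events through GameInstance.ScenePart.
; Minigame start and end pan the follow camera via a dummy actor and timelines.
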(event `self.ReceiveBeginPlay`
  (bind _iscorrectscene (`/Game/ProjectContents/BP/BP_FunctionLib.CheckSceneIndex` (`self.CurrentScene`)))
  (if _iscorrectscene
    (`self.LevelSetup`)
    (bind _returnvalue (`GameplayStatics.GetActorOfClass` "/Game/ProjectContents/BP/LevelActors/BP_DialogManager.BP_DialogManager_C"))
    (set `self.Level Dialog Manager` _returnvalue)
    (`self.CheckReload`)))

(event `InputAction|Interact`
  (params (Key :type "Key Structure"))
  ;[1 1 1] OnInteract
  (:`Pressed`
    (bind _asbp_game_instance (cast `/Game/ProjectContents/BP/BP_GameInstance` (`GameplayStatics.GetGameInstance`)))
    (if (`/Game/ProjectContents/BP/BP_GameInstance.isViewingScene` _asbp_game_instance)
      (if (`/Game/ProjectContents/BP/LevelActors/BP_DialogManager.isDIalogFinished` (`self.Level Dialog Manager`))
        (set `/Game/ProjectContents/BP/LevelActors/BP_DialogManager.isDIalogFinished` false (`self.Level Dialog Manager`))
        (bind _asbp_game_instance_2 (cast `/Game/ProjectContents/BP/BP_GameInstance` (`GameplayStatics.GetGameInstance`)))
        (set `/Game/ProjectContents/BP/BP_GameInstance.isViewingScene` false _asbp_game_instance_2)
        (`KismetSystemLibrary.PrintString` "DialogFinished")
        (`self.MoveToNextPart`)
        (else
          (`/Game/ProjectContents/BP/LevelActors/BP_DialogManager.Test-CycleOnKey` (`self.Level Dialog Manager`)))))))

(event `Part0`
  (`/Game/ProjectContents/BP/BP_FunctionLib.SetupDialogManagerCycle` (`self.Level Dialog Manager`) (`self.Teacher`) (`self.Teacher1`) self)
  (`/Game/ProjectContents/BP/BP_FunctionLib.DisablePlayerInput`))

(event `CheckReload`
  (bind _teacher (`self.Teacher`))
  (bind _asbp_game_instance (cast `/Game/ProjectContents/BP/BP_GameInstance` (`GameplayStatics.GetGameInstance`)))
  (if (== (`/Game/ProjectContents/BP/BP_GameInstance.ScenePart` _asbp_game_instance) 5)
    (`/Game/ProjectContents/BP/BP_FunctionLib.Flip FlipBook` _teacher)
    (`self.K2_SetActorLocation` _teacher (- (`self.K2_GetActorLocation` _teacher) (150.0 0.0 0.0)) false false)
    (bind _returnvalue (`|SpawnActorFromClass` "/Game/ProjectContents/BP/PopOutManager/BP_Minigame_TelBox.BP_Minigame_TelBox_C" (`KismetMathLibrary.MakeTransform` (-300.0 20.0 400.0)) "Undefined" "OverrideRootScale" null null))
    (set `self.BoxMinigame` _returnvalue)
    (bind _returnvalue_2 (`GameplayStatics.GetActorOfClass` "/Game/ProjectContents/BP/Triggers/BP_Scene09_Staffroom_Trigger.BP_Scene09_Staffroom_Trigger_C"))
    (`self.SetActorHiddenInGame` _returnvalue_2 true)))

(event `Handle End SCene`
  ;[1 1 1] Handle Scene End
  (bind _asbp_game_instance (cast `/Game/ProjectContents/BP/BP_GameInstance` (`GameplayStatics.GetGameInstance`)))
  (`/Game/ProjectContents/BP/BP_GameInstance.MoveToNextScene` _asbp_game_instance)
  (bind _returnvalue (`|CreateWidget` "/Game/ProjectContents/BP/Widgets/WBP_FadeBlack.WBP_FadeBlack_C" (`GameplayStatics.GetPlayerController` 0)))
  (`UserWidget.AddToViewport` _returnvalue 0)
  (`/Game/ProjectContents/BP/Widgets/WBP_FadeBlack.FadeToBlack` _returnvalue)
  (`KismetSystemLibrary.Delay` 0.5)
  (`GameplayStatics.OpenLevel` "Game_House"))

(event `Part1`
  (`/Game/ProjectContents/BP/BP_FunctionLib.SetupDialogManagerCycle` (`self.Level Dialog Manager`) (`self.BigSister`) (`self.Big Sister1`) self))

(event `Part2`
  (`/Game/ProjectContents/BP/BP_FunctionLib.SetupDialogManagerCycle` (`self.Level Dialog Manager`) (`self.Teacher`) (`self.Teacher2`) self))

(event `Handle Change Camera`
  (bind _returnvalue (`self.K2_GetActorLocation` (`GameplayStatics.GetPlayerPawn` 0)))
  ;[1 1 1] Handle Switch Player with Dummy Actor
  (bind _returnvalue_2 (`|SpawnActorFromClass` "/Game/ProjectContents/BP/Objects/BP_DummyActor.BP_DummyActor_C" (`KismetMathLibrary.MakeTransform` _returnvalue) "Undefined" "OverrideRootScale" null null))
  (bind _returnvalue_3 (`GameplayStatics.GetActorOfClass` "/Game/ProjectContents/BP/LevelActors/BP_FollowCamera.BP_FollowCamera_C"))
  (set `/Game/ProjectContents/BP/LevelActors/BP_FollowCamera.ActorToFollow` _returnvalue_2 _returnvalue_3)
  (`KismetSystemLibrary.PrintString` "Switched ActorToFollow")
  (set `self.CameraStart` _returnvalue)
  (set `self.CameraEnd` (+ _returnvalue (300.0 0.0 0.0)))
  (`self.DisableInput` (`GameplayStatics.GetPlayerPawn` 0) (`GameplayStatics.GetPlayerController` 0)))

(event `Part3`
  (bind _asbp_npcactor_base (cast `/Game/ProjectContents/BP/NPC/BP_NPCActorBase` (`self.Teacher`)))
  (`/Game/ProjectContents/BP/BP_FunctionLib.Flip FlipBook` _asbp_npcactor_base)
  (bind _returnvalue (`self.K2_GetActorLocation` _asbp_npcactor_base))
  (`/Game/ProjectContents/BP/NPC/BP_NPCActorBase.MoveNPC Event` _asbp_npcactor_base _returnvalue (- _returnvalue (150.0 0.0 0.0)))
  (`KismetSystemLibrary.Delay` 3.0)
  (`/Game/ProjectContents/BP/BP_FunctionLib.SetupDialogManagerCycle` (`self.Level Dialog Manager`) (`self.BigSister`) (`self.Big Sister2`) self))

(event `HandleMoveCameraRight`
  ;[1 1 1] Handle Move CAmera Right
  (bind _returnvalue (`GameplayStatics.GetActorOfClass` "/Game/ProjectContents/BP/Objects/BP_DummyActor.BP_DummyActor_C"))
  (bind (_direction _alpha) (`Timeline|Timeline_0` :!via `PlayFromStart`)
    (:`Update`
      (`self.K2_SetActorLocation` _returnvalue (`KismetMathLibrary.VLerp` (`self.CameraStart`) (`self.CameraEnd`) _alpha) false false))
    (:`Finished`
      (`AudioComponent.SetPaused` (`self.BGM`) true))))

(event `Part4`
  (bind _teacher (`self.Teacher`))
  (`/Game/ProjectContents/BP/BP_FunctionLib.Flip FlipBook` _teacher)
  (`/Game/ProjectContents/BP/BP_FunctionLib.SetupDialogManagerCycle` (`self.Level Dialog Manager`) _teacher (`self.Teacher3`) self))

(event `Part5`
  (`/Game/ProjectContents/BP/BP_FunctionLib.Flip FlipBook` (`self.Teacher`))
  (bind _returnvalue (`|SpawnActorFromClass` "/Game/ProjectContents/BP/PopOutManager/BP_Minigame_TelBox.BP_Minigame_TelBox_C" (`KismetMathLibrary.MakeTransform` (-600.0 20.0 350.0)) "Undefined" "OverrideRootScale" null null))
  (set `self.BoxMinigame` _returnvalue)
  (`/Game/ProjectContents/BP/BP_FunctionLib.EnablePlayerInput`))

(event `Part6`
  (bind _teacher (`self.Teacher`))
  (`/Game/ProjectContents/BP/BP_FunctionLib.Flip FlipBook` _teacher)
  (`/Game/ProjectContents/BP/BP_FunctionLib.SetupDialogManagerCycle` (`self.Level Dialog Manager`) _teacher (`self.Teacher5`) self))

(event `HandleMOveCameraLeft`
  ;[1 1 1] Handle Move Camera Left
  (bind _returnvalue (`GameplayStatics.GetActorOfClass` "/Game/ProjectContents/BP/Objects/BP_DummyActor.BP_DummyActor_C"))
  (bind (_direction _alpha) (`Timeline|Timeline_1` :!via `PlayFromStart`)
    (:`Update`
      (`self.K2_SetActorLocation` _returnvalue (`KismetMathLibrary.VLerp` (`self.CameraEnd`) (`self.CameraStart`) _alpha) false false))
    (:`Finished`
      (bind _returnvalue_2 (`GameplayStatics.GetActorOfClass` "/Game/ProjectContents/BP/LevelActors/BP_FollowCamera.BP_FollowCamera_C"))
      (set `/Game/ProjectContents/BP/LevelActors/BP_FollowCamera.ActorToFollow` (`GameplayStatics.GetPlayerPawn` 0) _returnvalue_2)
      (`self.EnableInput` (`GameplayStatics.GetPlayerPawn` 0) (`GameplayStatics.GetPlayerController` 0))
      (`AudioComponent.SetPaused` (`self.BGM`) false))))

(event `Part7`
  (`/Game/ProjectContents/BP/BP_FunctionLib.SetupDialogManagerCycle` (`self.Level Dialog Manager`) (`self.BigSister`) (`self.Big Sister3`) self))

(event `Part8`
  (`self.Handle End SCene`))

(event `Box Minigame Start`
  (bind _returnvalue (`GameplayStatics.GetPlayerController` 0))
  (`self.DisableInput` (`GameplayStatics.GetPlayerController` 0))
  (`self.DisableInput` (`GameplayStatics.GetPlayerPawn` 0) (`GameplayStatics.GetPlayerController` 0))
  (`self.Handle Change Camera`)
  (`self.HandleMoveCameraRight`)
  (`KismetSystemLibrary.Delay` 3.0)
  (bind _returnvalue_2 (`|CreateWidget` "/Game/ProjectContents/BP/Widgets/PopOut/WBP_Pop_Box.WBP_Pop_Box_C" _returnvalue))
  (set `PlayerController.bShowMouseCursor` true _returnvalue)
  (`UserWidget.AddToViewport` _returnvalue_2 0))

(event `Box Minigame End`
  (`GameplayStatics.PlaySound2D` "/Game/ProjectContents/SFX/SFX_Pickup.SFX_Pickup" 1.0 1.0 0.0 null null)
  (`self.HandleMOveCameraLeft`)
  (set `PlayerController.bShowMouseCursor` false (`GameplayStatics.GetPlayerController` 0))
  (`KismetSystemLibrary.Delay` 3.0)
  (`self.EnableInput` (`GameplayStatics.GetPlayerController` 0))
  (`/Game/ProjectContents/BP/BP_FunctionLib.SetupDialogManagerCycle` (`self.Level Dialog Manager`) (`self.Teacher`) (`self.Teacher4`) self))

(fn `LevelSetup`
  (for (_array_element _array_index) (`self.LevelActors`)
    (bind _returnvalue (`|SpawnActorFromClass` _array_element (`|GetArrayItem` (`self.ActorSpawns`) _array_index) "Undefined" "OverrideRootScale" null null))
    (switch `int` _array_index
      (:`0`
        (set `self.BigSister` _returnvalue))
      (:`1`
        (set `self.Teacher` _returnvalue))))
  (bind _returnvalue_2 (`|CreateWidget` "/Game/ProjectContents/BP/Widgets/WBP_SeasonChange.WBP_SeasonChange_C" (`GameplayStatics.GetPlayerController` 0)))
  (`UserWidget.AddToViewport` _returnvalue_2 0)
  (bind _returnvalue_3 (`GameplayStatics.GetActorOfClass` "/Game/ProjectContents/BP/NPC/BP_NPCActor_BigSister.BP_NPCActor_BigSister_C"))
  (`/Game/ProjectContents/BP/BP_FunctionLib.Flip FlipBook` _returnvalue_3)
  (bind _returnvalue_4 (`GameplayStatics.SpawnSound2D` "/Game/ProjectContents/Music/Final/School_office.School_office" 1.0 1.0 0.0 null false false))
  (bind _output_get (set `self.BGM` _returnvalue_4))
  (`AudioComponent.Play` _output_get 0.0))

(fn `MoveToNextPart`
  (`self.DisableInput` (`GameplayStatics.GetPlayerController` 0))
  (bind _result (`/Engine/EditorBlueprintResources/StandardMacros.IncrementInt` (`self.CurrentPart`))
    (:`  `
      (bind _asbp_game_instance (cast `/Game/ProjectContents/BP/BP_GameInstance` (`GameplayStatics.GetGameInstance`)))
      (bind _output_get (set `/Game/ProjectContents/BP/BP_GameInstance.ScenePart` _result _asbp_game_instance))
      (switch `int` _output_get
        (:`1`
          (`self.Part1`))
        (:`2`
          (`self.Part2`))
        (:`3`
          (`self.Part3`))
        (:`4`
          (`self.Part4`))
        (:`5`
          (`self.Part5`))
        (:`6`
          (`self.Part6`))
        (:`7`
          (`self.Part7`))
        (:`8`
          (`self.Part8`))))))

(fn `UserConstructionScript`)