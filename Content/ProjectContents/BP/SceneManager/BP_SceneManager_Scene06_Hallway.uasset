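; Scene manager for the Scene 06 hallway cutscene, a scripted conversation between students and the big sister that ends by fading to black and opening Game_Road.
; On a matching scene index, it spawns the cast, hides the sister and positions the player.
; Interact cycles dialog through BP_DialogManager; when finished, MoveToNextPart increments the GameInstance ScenePart and dispatches numbered Part events.
; These events queue each speaker's lines or stage timed NPC moves, flipbook flips and exits.
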(event `self.ReceiveBeginPlay`
  (bind _iscorrectscene (`/Game/ProjectContents/BP/BP_FunctionLib.CheckSceneIndex` (`self.CurrentScene`)))
  (if _iscorrectscene
    (`self.LevelSetup`)
    (bind _returnvalue (`GameplayStatics.GetActorOfClass` "/Game/ProjectContents/BP/LevelActors/BP_DialogManager.BP_DialogManager_C"))
    (set `self.Level Dialog Manager` _returnvalue)))

(event `Handle Sister Move`
  (bind _bigsister (`self.BigSister`))
  (bind _returnvalue (`self.K2_GetActorLocation` _bigsister))
  ;[1 1 1] Handle Sister Movement
  (bind _asbp_npcactor_base (cast `/Game/ProjectContents/BP/NPC/BP_NPCActorBase` _bigsister))
  (`/Game/ProjectContents/BP/BP_FunctionLib.Flip FlipBook` _asbp_npcactor_base)
  (`self.SetActorHiddenInGame` _bigsister false)
  (`/Game/ProjectContents/BP/NPC/BP_NPCActorBase.MoveNPC Event` _asbp_npcactor_base _returnvalue (- _returnvalue (600.0 0.0 0.0))))

(event `InputAction|Interact`
  (params (Key :type "Key Structure"))
  ;[1 1 1] OnInteract
  (:`Pressed`
    (bind _asbp_game_instance (cast `/Game/ProjectContents/BP/BP_GameInstance` (`GameplayStatics.GetGameInstance`)))
    (if (`/Game/ProjectContents/BP/BP_GameInstance.isViewingScene` _asbp_game_instance)
      (if (`/Game/ProjectContents/BP/LevelActors/BP_DialogManager.isDIalogFinished` (`self.Level Dialog Manager`))
        (set `/Game/ProjectContents/BP/LevelActors/BP_DialogManager.isDIalogFinished` false (`self.Level Dialog Manager`))
        (bind _asbp_game_instance_2 (cast `/Game/ProjectContents/BP/BP_GameInstance` (`GameplayStatics.GetGameInstance`)))
        (set `/Game/ProjectContents/BP/BP_GameInstance.isViewingScene` false _asbp_game_instance_2)
        (`KismetSystemLibrary.PrintString` "DialogFinished")
        (`self.MoveToNextPart`)
        (else
          (`/Game/ProjectContents/BP/LevelActors/BP_DialogManager.Test-CycleOnKey` (`self.Level Dialog Manager`)))))))

(event `Handle Student Dialog`
  ;[1 1 1] Handle Student Dialog
  (bind _dialog_delay (`/Game/ProjectContents/BP/LevelActors/BP_DialogManager.Display Dialog` (`self.Level Dialog Manager`) (`|GetArrayItem` (`self.Students`)) (`self.StudentC`) (`self.TextDelay`)))
  (`KismetSystemLibrary.Delay` _dialog_delay)
  (`self.Handle Student Move`))

(event `Part0`
  (`/Game/ProjectContents/BP/BP_FunctionLib.SetupDialogManagerCycle` (`self.Level Dialog Manager`) (`|GetArrayItem` (`self.Students`) 1) (`self.StudentB`) self))

(event `Handle Student Move`
  ;[1 1 1] Handle Student Move
  (`/Game/ProjectContents/BP/BP_FunctionLib.DisablePlayerInput`)
  (for _index (range 3)
    (bind _output (`|GetArrayItem` (`self.Students`) _index))
    (bind _asbp_npcactor_base (cast `/Game/ProjectContents/BP/NPC/BP_NPCActorBase` _output))
    (`/Game/ProjectContents/BP/NPC/BP_NPCActorBase.MoveNPC Event` _asbp_npcactor_base (`self.K2_GetActorLocation` _output) (`self.Student End`)))
  (`KismetSystemLibrary.Delay` 3.0)
  (for _index_2 (range 3)
    (`self.K2_DestroyActor` (`|GetArrayItem` (`self.Students`) _index_2))
    (`/Game/ProjectContents/BP/BP_FunctionLib.EnablePlayerInput`)))

(event `Part1`
  (`/Game/ProjectContents/BP/BP_FunctionLib.SetupDialogManagerCycle` (`self.Level Dialog Manager`) (`|GetArrayItem` (`self.Students`) 2) (`self.StudentC`) self))

(event `Handle Sister Dialog`
  (bind _bigsister (`self.BigSister`))
  ;[1 1 1] Handle Sister End
  (bind _dialog_delay (`/Game/ProjectContents/BP/LevelActors/BP_DialogManager.Display Dialog` (`self.Level Dialog Manager`) _bigsister (`self.Sister1`) (`self.TextDelay`)))
  (`KismetSystemLibrary.Delay` _dialog_delay)
  (`/Game/ProjectContents/BP/BP_FunctionLib.Flip FlipBook` _bigsister)
  (bind _asbp_npcactor_base (cast `/Game/ProjectContents/BP/NPC/BP_NPCActorBase` _bigsister))
  (`/Game/ProjectContents/BP/NPC/BP_NPCActorBase.MoveNPC Event` _asbp_npcactor_base (`self.K2_GetActorLocation` _bigsister) (`self.Student End`))
  (`KismetSystemLibrary.Delay` 2.5)
  (`self.K2_DestroyActor` _bigsister)
  (`self.Handle Scene End`))

(event `Part2`
  (`/Game/ProjectContents/BP/BP_FunctionLib.SetupDialogManagerCycle` (`self.Level Dialog Manager`) (`|GetArrayItem` (`self.Students`) 1) (`self.StudentB1`) self))

(event `Handle Scene End`
  (bind _returnvalue (`|CreateWidget` "/Game/ProjectContents/BP/Widgets/WBP_FadeBlack.WBP_FadeBlack_C" (`GameplayStatics.GetPlayerController` 0)))
  (`UserWidget.AddToViewport` _returnvalue 0)
  (`/Game/ProjectContents/BP/Widgets/WBP_FadeBlack.FadeToBlack` _returnvalue)
  (`KismetSystemLibrary.Delay` 0.5)
  (`GameplayStatics.OpenLevel` "Game_Road"))

(event `Part3`
  (`/Game/ProjectContents/BP/BP_FunctionLib.SetupDialogManagerCycle` (`self.Level Dialog Manager`) (`|GetArrayItem` (`self.Students`)) (`self.StudentA1`) self))

(event `Part4`
  (`self.Handle Sister Move`)
  (`KismetSystemLibrary.Delay` 3.0)
  (`/Game/ProjectContents/BP/BP_FunctionLib.SetupDialogManagerCycle` (`self.Level Dialog Manager`) (`|GetArrayItem` (`self.Students`)) (`self.StudentA2`) self))

(event `Part5`
  (`/Game/ProjectContents/BP/BP_FunctionLib.SetupDialogManagerCycle` (`self.Level Dialog Manager`) (`self.BigSister`) (`self.Sister1`) self))

(event `Part6`
  (`/Game/ProjectContents/BP/BP_FunctionLib.SetupDialogManagerCycle` (`self.Level Dialog Manager`) (`|GetArrayItem` (`self.Students`) 1) (`self.StudentB2`) self))

(event `Part7`
  (`/Game/ProjectContents/BP/BP_FunctionLib.SetupDialogManagerCycle` (`self.Level Dialog Manager`) (`self.BigSister`) (`self.Sister2`) self))

(event `Part8`
  (`/Game/ProjectContents/BP/BP_FunctionLib.SetupDialogManagerCycle` (`self.Level Dialog Manager`) (`|GetArrayItem` (`self.Students`)) (`self.StudentA3`) self))

(event `Part9`
  (`/Game/ProjectContents/BP/BP_FunctionLib.SetupDialogManagerCycle` (`self.Level Dialog Manager`) (`|GetArrayItem` (`self.Students`) 2) (`self.StudentC1`) self))

(event `Part10`
  (`self.Handle Student Move`)
  (`KismetSystemLibrary.Delay` 1.0)
  (`/Game/ProjectContents/BP/BP_FunctionLib.Flip FlipBook` (`self.BigSister`))
  (`KismetSystemLibrary.Delay` 2.0)
  (`/Game/ProjectContents/BP/BP_FunctionLib.SetupDialogManagerCycle` (`self.Level Dialog Manager`) (`self.BigSister`) (`self.Sister3`) self))

(event `Part11`
  (bind _bigsister (`self.BigSister`))
  (`/Game/ProjectContents/BP/BP_FunctionLib.DisablePlayerInput`)
  (bind _asbp_npcactor_base (cast `/Game/ProjectContents/BP/NPC/BP_NPCActorBase` _bigsister))
  (`/Game/ProjectContents/BP/NPC/BP_NPCActorBase.MoveNPC Event` _asbp_npcactor_base (`self.K2_GetActorLocation` _bigsister) (`self.Student End`))
  (`KismetSystemLibrary.Delay` 2.5)
  (`self.K2_DestroyActor` _bigsister)
  (`self.Handle Scene End`))

(fn `LevelSetup`
  (for (_array_element _array_index) (`self.LevelActors`)
    (bind _returnvalue (`|SpawnActorFromClass` _array_element (`|GetArrayItem` (`self.ActorSpawns`) _array_index) "Undefined" "OverrideRootScale" null null))
    (if (`self.ActorHasTag` _returnvalue "Student")
      (`KismetArrayLibrary.Array_Add` (`self.Students`) _returnvalue)
      (elif (== _array_index 3)
        (set `self.BigSister` _returnvalue))))
  (`self.SetActorHiddenInGame` (`self.BigSister`) true)
  (`self.K2_SetActorLocation` (`GameplayStatics.GetPlayerPawn` 0) (`self.PlayerSpawn`) false false))

(fn `MoveToNextPart`
  (`self.DisableInput` (`GameplayStatics.GetPlayerController` 0))
  (bind _result (`/Engine/EditorBlueprintResources/StandardMacros.IncrementInt` (`self.CurrentPart`))
    (:`  `
      (bind _asbp_game_instance (cast `/Game/ProjectContents/BP/BP_GameInstance` (`GameplayStatics.GetGameInstance`)))
      (bind _output_get (set `/Game/ProjectContents/BP/BP_GameInstance.ScenePart` _result _asbp_game_instance))
      (switch `int` _output_get
        (:`1`
          (`self.Part1`))
        (:`2`
          (`self.Part2`))
        (:`3`
          (`self.Part3`))
        (:`4`
          (`self.Part4`))
        (:`5`
          (`self.Part5`))
        (:`6`
          (`self.Part6`))
        (:`7`
          (`self.Part7`))
        (:`8`
          (`self.Part8`))
        (:`9`
          (`self.Part9`))
        (:`10`
          (`self.Part10`))
        (:`11`
          (`self.Part11`))))))

(fn `UserConstructionScript`)