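; Scene manager for Scene 10 (House): stages a dialogue between Mother and Big Sister, then their exit.
; When the scene index matches, BeginPlay spawns both NPCs and removes the level-move actor.
; Interact cycles dialogue through BP_DialogManager and advances numbered parts; the last walks both NPCs off, destroys them and spawns a tear drop.
; Picking up the tear drop advances the GameInstance scene and fades to black into Game_Staffroom.
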(event `InputAction|Interact`
  (params (Key :type "Key Structure"))
  ;[1 1 1] OnInteract
  (:`Pressed`
    (bind _asbp_game_instance (cast `/Game/ProjectContents/BP/BP_GameInstance` (`GameplayStatics.GetGameInstance`)))
    (if (`/Game/ProjectContents/BP/BP_GameInstance.isViewingScene` _asbp_game_instance)
      (if (`/Game/ProjectContents/BP/LevelActors/BP_DialogManager.isDIalogFinished` (`self.Level Dialog Manager`))
        (set `/Game/ProjectContents/BP/LevelActors/BP_DialogManager.isDIalogFinished` false (`self.Level Dialog Manager`))
        (bind _asbp_game_instance_2 (cast `/Game/ProjectContents/BP/BP_GameInstance` (`GameplayStatics.GetGameInstance`)))
        (set `/Game/ProjectContents/BP/BP_GameInstance.isViewingScene` false _asbp_game_instance_2)
        (`KismetSystemLibrary.PrintString` "DialogFinished")
        (`self.MoveToNextPart`)
        (else
          (`/Game/ProjectContents/BP/LevelActors/BP_DialogManager.Test-CycleOnKey` (`self.Level Dialog Manager`))))
      (else
        (`/Game/ProjectContents/BP/BP_FunctionLib.TriggerHint`)))))

(event `self.ReceiveBeginPlay`
  (bind _iscorrectscene (`/Game/ProjectContents/BP/BP_FunctionLib.CheckSceneIndex` (`self.CurrentScene`)))
  (if _iscorrectscene
    (`self.LevelSetup`)
    (bind _returnvalue (`GameplayStatics.GetActorOfClass` "/Game/ProjectContents/BP/LevelActors/BP_DialogManager.BP_DialogManager_C"))
    (set `self.Level Dialog Manager` _returnvalue)))

(event `Part0`
  (`self.DisableInput` (`GameplayStatics.GetPlayerPawn` 0) (`GameplayStatics.GetPlayerController` 0))
  (`/Game/ProjectContents/BP/BP_FunctionLib.SetupDialogManagerCycle` (`self.Level Dialog Manager`) (`self.Mother`) (`self.Mother1`) self))

(event `Handle Sister`
  ;[1 1 1] Handle Tear Drop
  (bind _asbp_npcactor_base (cast `/Game/ProjectContents/BP/NPC/BP_NPCActorBase` (`self.BigSIster`)))
  (`/Game/ProjectContents/BP/BP_FunctionLib.Flip FlipBook` _asbp_npcactor_base)
  (`/Game/ProjectContents/BP/NPC/BP_NPCActorBase.MoveNPC Event` _asbp_npcactor_base (`self.Sister Start`) (`self.Sister End`))
  (`KismetSystemLibrary.Delay` 3.0)
  (`self.K2_DestroyActor` _asbp_npcactor_base)
  (`self.EnableInput` (`GameplayStatics.GetPlayerPawn` 0) (`GameplayStatics.GetPlayerController` 0))
  (`|SpawnActorFromClass` "/Game/ProjectContents/BP/Objects/BP_TearDrop.BP_TearDrop_C" (`KismetMathLibrary.MakeTransform` (`self.TearDrop`) (struct) (1.5 1.5 1.5)) "Undefined" "OverrideRootScale" null null))

(event `Part1`
  (`/Game/ProjectContents/BP/BP_FunctionLib.SetupDialogManagerCycle` (`self.Level Dialog Manager`) (`self.BigSIster`) (`self.Big Sister`) self))

(event `Handle End Scene`
  (bind _returnvalue (`|CreateWidget` "/Game/ProjectContents/BP/Widgets/WBP_FadeBlack.WBP_FadeBlack_C" (`GameplayStatics.GetPlayerController` 0)))
  (`UserWidget.AddToViewport` _returnvalue 0)
  (`/Game/ProjectContents/BP/Widgets/WBP_FadeBlack.FadeToBlack` _returnvalue)
  (`KismetSystemLibrary.Delay` 0.5)
  (`GameplayStatics.OpenLevel` "Game_Staffroom"))

(event `Part2`
  (`/Game/ProjectContents/BP/BP_FunctionLib.SetupDialogManagerCycle` (`self.Level Dialog Manager`) (`self.Mother`) (`self.Mother2`) self))

(event `Part3`
  (bind _asbp_npcactor_base (cast `/Game/ProjectContents/BP/NPC/BP_NPCActorBase` (`self.Mother`)))
  (`/Game/ProjectContents/BP/BP_FunctionLib.Flip FlipBook` _asbp_npcactor_base)
  (`/Game/ProjectContents/BP/NPC/BP_NPCActorBase.MoveNPC Event` _asbp_npcactor_base (`self.Mother Start`) (`self.Mother End`))
  (`KismetSystemLibrary.Delay` 3.0)
  (`self.K2_DestroyActor` (`self.Mother`))
  (`self.Handle Sister`))

(event `Handle Start Dialog`
  ;[1 1 1] Handle Mother and Sister
  (`self.DisableInput` (`GameplayStatics.GetPlayerPawn` 0) (`GameplayStatics.GetPlayerController` 0))
  (bind _dialog_delay (`/Game/ProjectContents/BP/LevelActors/BP_DialogManager.Display Dialog` (`self.Level Dialog Manager`) (`self.Mother`) (`self.Mother1`) (`self.TextDelay`)))
  (`KismetSystemLibrary.Delay` _dialog_delay)
  (bind _dialog_delay_2 (`/Game/ProjectContents/BP/LevelActors/BP_DialogManager.Display Dialog` (`self.Level Dialog Manager`) (`self.BigSIster`) (`self.Big Sister`) (`self.TextDelay`)))
  (`KismetSystemLibrary.Delay` _dialog_delay_2)
  (bind _dialog_delay_3 (`/Game/ProjectContents/BP/LevelActors/BP_DialogManager.Display Dialog` (`self.Level Dialog Manager`) (`self.Mother`) (`self.Mother2`) (`self.TextDelay`)))
  (`KismetSystemLibrary.Delay` _dialog_delay_3)
  (bind _asbp_npcactor_base (cast `/Game/ProjectContents/BP/NPC/BP_NPCActorBase` (`self.Mother`)))
  (`/Game/ProjectContents/BP/BP_FunctionLib.Flip FlipBook` _asbp_npcactor_base)
  (`/Game/ProjectContents/BP/NPC/BP_NPCActorBase.MoveNPC Event` _asbp_npcactor_base (`self.Mother Start`) (`self.Mother End`))
  (`KismetSystemLibrary.Delay` 3.0)
  (`self.Handle Sister`)
  (`self.K2_DestroyActor` _asbp_npcactor_base))

(fn `LevelSetup`
  (bind _bigsister (`self.BigSIster`))
  (for (_array_element _array_index) (`self.LevelActors`)
    (bind _returnvalue (`|SpawnActorFromClass` _array_element (`|GetArrayItem` (`self.ActorSpawns`) _array_index) "Undefined" "OverrideRootScale" null null))
    (switch `int` _array_index
      (:`0`
        (set `self.BigSIster` _returnvalue))
      (:`1`
        (set `self.Mother` _returnvalue))))
  (`/Game/ProjectContents/BP/BP_FunctionLib.Flip FlipBook` _bigsister)
  (set `self.Sister Start` (`self.K2_GetActorLocation` _bigsister))
  (set `self.Mother Start` (`self.K2_GetActorLocation` (`self.Mother`)))
  (bind _returnvalue_2 (`GameplayStatics.GetActorOfClass` "/Game/ProjectContents/BP/LevelActors/BP_MoveLevels.BP_MoveLevels_C"))
  (`self.K2_DestroyActor` _returnvalue_2))

(fn `MoveToNextPart`
  (`self.DisableInput` (`GameplayStatics.GetPlayerController` 0))
  (bind _result (`/Engine/EditorBlueprintResources/StandardMacros.IncrementInt` (`self.CurrentPart`))
    (:`  `
      (bind _asbp_game_instance (cast `/Game/ProjectContents/BP/BP_GameInstance` (`GameplayStatics.GetGameInstance`)))
      (bind _output_get (set `/Game/ProjectContents/BP/BP_GameInstance.ScenePart` _result _asbp_game_instance))
      (switch `int` _output_get
        (:`1`
          (`self.Part1`))
        (:`2`
          (`self.Part2`))
        (:`3`
          (`self.Part3`))))))

(fn `OnTearDropPickUp`
  (bind _asbp_game_instance (cast `/Game/ProjectContents/BP/BP_GameInstance` (`GameplayStatics.GetGameInstance`)))
  (`/Game/ProjectContents/BP/BP_GameInstance.MoveToNextScene` _asbp_game_instance)
  (set `self.MoveLevel ToolTip` "Go to bedroom")
  (bind _returnvalue (`GameplayStatics.GetActorOfClass` "/Game/ProjectContents/BP/LevelActors/BP_MoveLevels.BP_MoveLevels_C"))
  (`self.EnableInput` _returnvalue (`GameplayStatics.GetPlayerController` 0))
  (`TextRenderComponent.K2_SetText` (`/Game/ProjectContents/BP/LevelActors/BP_MoveLevels.ToolTip` _returnvalue) (`self.MoveLevel ToolTip`))
  (`self.Handle End Scene`))

(fn `UserConstructionScript`)