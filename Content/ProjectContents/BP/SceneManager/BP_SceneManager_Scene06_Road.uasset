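; Scene manager for the after-school road scene, running a scripted walk-and-talk between three students and the big sister.
; On BeginPlay it spawns the cast, fades in and locks level-move input, then a timeline slides NPCs along X.
; A looping timer reuses the Interact logic to auto-advance student dialogue through numbered parts.
; When walking ends, students despawn, auto-scroll pauses for the sister's dialogue, then she exits and the next scene loads.
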(event `self.ReceiveBeginPlay`
  (bind _iscorrectscene (`/Game/ProjectContents/BP/BP_FunctionLib.CheckSceneIndex` (`self.CurrentScene`)))
  (if _iscorrectscene
    (`self.Level Setup`)
    (bind _returnvalue (`GameplayStatics.GetActorOfClass` "/Game/ProjectContents/BP/LevelActors/BP_DialogManager.BP_DialogManager_C"))
    (set `self.Level Dialog Manager` _returnvalue)
    (bind _returnvalue_2 (`|CreateWidget` "/Game/ProjectContents/BP/Widgets/WBP_FadeBlack.WBP_FadeBlack_C" (`GameplayStatics.GetPlayerController` 0)))
    (`UserWidget.AddToViewport` _returnvalue_2 0)
    (`/Game/ProjectContents/BP/Widgets/WBP_FadeBlack.FadeFromBlack` _returnvalue_2)
    (`KismetSystemLibrary.Delay` 1.0)
    (`Widget.RemoveFromParent` _returnvalue_2)
    (bind _returnvalue_3 (`GameplayStatics.GetActorOfClass` "/Game/ProjectContents/BP/LevelActors/BP_MoveLevels.BP_MoveLevels_C"))
    (`self.DisableInput` _returnvalue_3 (`GameplayStatics.GetPlayerController` 0))
    (`KismetSystemLibrary.Delay` 3.0)
    (`self.Handle Movement`)
    (`GameplayStatics.PlaySound2D` "/Game/ProjectContents/Music/Final/AfterSchool.AfterSchool" 1.0 1.0 0.0 null null)))

(event `Handle Movement`
  ;[1 1 1] Handle NPC Movement
  (for _index (range 4)
    (`KismetArrayLibrary.Array_Insert` (`self.Movement Delta`) (- (`|GetArrayItem` (`self.Movement End`) _index) (`|GetArrayItem` (`self.Movement Start`) _index)) _index)
    (bind _returnvalue (`GameplayStatics.GetActorOfClass` (`|GetArrayItem` (`self.LevelActors`) _index)))
    (`KismetArrayLibrary.Array_Insert` (`self.MovingActors`) _returnvalue _index)
    (`self.Change NPC Walking`))
  (`self.Part0`)
  (bind (_direction _alpha) (`Timeline|StudentMovement`)
    (:`Update`
      (for _index_2 (range 4)
        (bind (_output_x _output_y _output_z) (`KismetMathLibrary.BreakVector` (`|GetArrayItem` (`self.Movement Start`) _index_2)))
        (bind _output_x_2 (`KismetMathLibrary.BreakVector` (`|GetArrayItem` (`self.Movement Delta`) _index_2)))
        (`self.K2_SetActorLocation` (`|GetArrayItem` (`self.MovingActors`) _index_2) (`KismetMathLibrary.MakeVector` (+ _output_x (* _output_x_2 _alpha)) _output_y _output_z) false false)))
    (:`Finished`
      (`self.Change NPC Idle`)
      (`self.Handle Move Out`))))

(event `InputAction|Interact`
  (params (Key :type "Key Structure"))
  ;[1 1 1] OnInteract
  (:`Pressed`
    (bind _asbp_game_instance (cast `/Game/ProjectContents/BP/BP_GameInstance` (`GameplayStatics.GetGameInstance`) :!label _label))
    (if (`/Game/ProjectContents/BP/BP_GameInstance.isViewingScene` _asbp_game_instance)
      (if (`/Game/ProjectContents/BP/LevelActors/BP_DialogManager.isDIalogFinished` (`self.Level Dialog Manager`))
        (set `/Game/ProjectContents/BP/LevelActors/BP_DialogManager.isDIalogFinished` false (`self.Level Dialog Manager`))
        (bind _asbp_game_instance_2 (cast `/Game/ProjectContents/BP/BP_GameInstance` (`GameplayStatics.GetGameInstance`)))
        (set `/Game/ProjectContents/BP/BP_GameInstance.isViewingScene` false _asbp_game_instance_2)
        (`KismetSystemLibrary.PrintString` "DialogFinished")
        (`self.Move to Next Part`)
        (else
          (`/Game/ProjectContents/BP/LevelActors/BP_DialogManager.Test-CycleOnKey` (`self.Level Dialog Manager`)))))))

(event `StartAutoScroll`
  (bind _returnvalue (`KismetSystemLibrary.K2_SetTimerDelegate` (delegate `CallTriggerEvent`) (`self.Text Delay`) true))
  (set `self.AutoScrollTimer` _returnvalue))

(event `CallTriggerEvent`
  (goto _label))

(event `Part0`
  (`/Game/ProjectContents/BP/BP_FunctionLib.SetupDialogManagerCycle` (`self.Level Dialog Manager`) (`|GetArrayItem` (`self.StudentsArray`) 1) (`self.StudentB`) self)
  (`self.StartAutoScroll`))

(event `Handle Move Out`
  (`KismetSystemLibrary.Delay` 0.5)
  (for _index (range 3)
    (bind _output (`|GetArrayItem` (`self.MovingActors`) _index))
    (`/Engine/EditorBlueprintResources/StandardMacros.IsValid` _output
      (:`Is Valid`
        (`self.K2_DestroyActor` _output))))
  (`self.Part7`)
  (set `self.CurrentPart` 7))

(event `Part1`
  (`/Game/ProjectContents/BP/BP_FunctionLib.SetupDialogManagerCycle` (`self.Level Dialog Manager`) (`|GetArrayItem` (`self.StudentsArray`)) (`self.StudentA`) self))

(event `Part2`
  (`/Game/ProjectContents/BP/BP_FunctionLib.SetupDialogManagerCycle` (`self.Level Dialog Manager`) (`|GetArrayItem` (`self.StudentsArray`) 2) (`self.StudentC`) self))

(event `Handle Scene End`
  (bind _returnvalue (`GameplayStatics.GetActorOfClass` "/Game/ProjectContents/BP/LevelActors/BP_MoveLevels.BP_MoveLevels_C"))
  (`self.EnableInput` _returnvalue (`GameplayStatics.GetPlayerController` 0))
  (bind _asbp_game_instance (cast `/Game/ProjectContents/BP/BP_GameInstance` (`GameplayStatics.GetGameInstance`)))
  (`/Game/ProjectContents/BP/BP_GameInstance.MoveToNextScene` _asbp_game_instance))

(event `Part3`
  (`/Game/ProjectContents/BP/BP_FunctionLib.SetupDialogManagerCycle` (`self.Level Dialog Manager`) (`|GetArrayItem` (`self.StudentsArray`)) (`self.StudentA1`) self))

(event `Part4`
  (`/Game/ProjectContents/BP/BP_FunctionLib.SetupDialogManagerCycle` (`self.Level Dialog Manager`) (`|GetArrayItem` (`self.StudentsArray`) 1) (`self.StudentB1`) self))

(event `Part5`
  (`/Game/ProjectContents/BP/BP_FunctionLib.SetupDialogManagerCycle` (`self.Level Dialog Manager`) (`|GetArrayItem` (`self.StudentsArray`) 2) (`self.StudentC1`) self))

(event `Part6`
  (`/Game/ProjectContents/BP/BP_FunctionLib.SetupDialogManagerCycle` (`self.Level Dialog Manager`) (`|GetArrayItem` (`self.StudentsArray`)) (`self.StudentA2`) self))

(event `Part7`
  (`KismetSystemLibrary.K2_PauseTimerHandle` (`self.AutoScrollTimer`))
  (set `/Game/ProjectContents/BP/LevelActors/BP_DialogManager.CurrentTextIndex` 0 (`self.Level Dialog Manager`))
  (bind _returnvalue (`GameplayStatics.GetActorOfClass` "/Game/ProjectContents/BP/NPC/BP_NPCActor_BigSister.BP_NPCActor_BigSister_C"))
  (bind _output_get (set `self.BigSisterActor` _returnvalue))
  (`/Game/ProjectContents/BP/BP_FunctionLib.SetupDialogManagerCycle` (`self.Level Dialog Manager`) _output_get (`self.BigSister`) self))

(event `Part8`
  (bind _bigsisteractor (`self.BigSisterActor`))
  (bind _returnvalue (`self.K2_GetActorLocation` _bigsisteractor))
  (`/Game/ProjectContents/BP/NPC/BP_NPCActorBase.MoveNPC Event` _bigsisteractor _returnvalue (+ _returnvalue (800.0 0.0 0.0)))
  (`KismetSystemLibrary.Delay` 3.0)
  (`self.K2_DestroyActor` _bigsisteractor)
  (`self.Handle Scene End`))

(fn `Change NPC Idle`
  (for (_array_element _array_index) (`self.MovingActors`)
    (switch `int` _array_index
      (:`0`
        (bind _asbp_npcactor_student_a (cast `/Game/ProjectContents/BP/NPC/BP_NPCActor_StudentA` _array_element))
        (`/Game/ProjectContents/BP/NPC/BP_NPCActorBase.SetFlipbookIdle` _asbp_npcactor_student_a))
      (:`1`
        (bind _asbp_npcactor_student_b (cast `/Game/ProjectContents/BP/NPC/BP_NPCActor_StudentB` _array_element))
        (`/Game/ProjectContents/BP/NPC/BP_NPCActorBase.SetFlipbookIdle` _asbp_npcactor_student_b))
      (:`2`
        (bind _asbp_npcactor_student_c (cast `/Game/ProjectContents/BP/NPC/BP_NPCActor_StudentC` _array_element))
        (`/Game/ProjectContents/BP/NPC/BP_NPCActorBase.SetFlipbookIdle` _asbp_npcactor_student_c))
      (:`3`
        (bind _asbp_npcactor_big_sister (cast `/Game/ProjectContents/BP/NPC/BP_NPCActor_BigSister` _array_element))
        (`/Game/ProjectContents/BP/NPC/BP_NPCActorBase.SetFlipbookIdle` _asbp_npcactor_big_sister)))))

(fn `Change NPC Walking`
  (for (_array_element _array_index) (`self.MovingActors`)
    (switch `int` _array_index
      (:`0`
        (bind _asbp_npcactor_student_a (cast `/Game/ProjectContents/BP/NPC/BP_NPCActor_StudentA` _array_element))
        (`/Game/ProjectContents/BP/NPC/BP_NPCActorBase.SetFlipbookWalk` _asbp_npcactor_student_a))
      (:`1`
        (bind _asbp_npcactor_student_b (cast `/Game/ProjectContents/BP/NPC/BP_NPCActor_StudentB` _array_element))
        (`/Game/ProjectContents/BP/NPC/BP_NPCActorBase.SetFlipbookWalk` _asbp_npcactor_student_b))
      (:`2`
        (bind _asbp_npcactor_student_c (cast `/Game/ProjectContents/BP/NPC/BP_NPCActor_StudentC` _array_element))
        (`/Game/ProjectContents/BP/NPC/BP_NPCActorBase.SetFlipbookWalk` _asbp_npcactor_student_c))
      (:`3`
        (bind _asbp_npcactor_big_sister (cast `/Game/ProjectContents/BP/NPC/BP_NPCActor_BigSister` _array_element))
        (`/Game/ProjectContents/BP/NPC/BP_NPCActorBase.SetFlipbookWalk` _asbp_npcactor_big_sister)))))

(fn `Level Setup`
  (`|ExecutionSequence`
    (:`then_0`
      (for (_array_element _array_index) (`self.LevelActors`)
        (bind _returnvalue (`|SpawnActorFromClass` _array_element (`|GetArrayItem` (`self.ActorSpawns`) _array_index) "Undefined" "OverrideRootScale" null null))
        (if (!= _array_index 4)
          (`KismetArrayLibrary.Array_Add` (`self.StudentsArray`) _returnvalue))))
    (:`then_1`
      (`self.K2_SetActorLocation` (`GameplayStatics.GetPlayerPawn` 0) (`self.PlayerSpawn`) false false)
      (bind _returnvalue_2 (`GameplayStatics.GetActorOfClass` "/Game/ProjectContents/BP/LevelActors/BP_FollowCamera.BP_FollowCamera_C"))
      (bind _output_get (set `self.FollowCameraActor` _returnvalue_2))
      (set `/Game/ProjectContents/BP/LevelActors/BP_FollowCamera.CameraXOffset` 170.0 _output_get))))

(fn `Move to Next Part`
  (`self.DisableInput` (`GameplayStatics.GetPlayerController` 0))
  (bind _result (`/Engine/EditorBlueprintResources/StandardMacros.IncrementInt` (`self.CurrentPart`))
    (:`  `
      (bind _asbp_game_instance (cast `/Game/ProjectContents/BP/BP_GameInstance` (`GameplayStatics.GetGameInstance`)))
      (bind _output_get (set `/Game/ProjectContents/BP/BP_GameInstance.ScenePart` _result _asbp_game_instance))
      (switch `int` _output_get
        (:`0`
          (`self.Part0`))
        (:`1`
          (`self.Part1`))
        (:`2`
          (`self.Part2`))
        (:`3`
          (`self.Part3`))
        (:`4`
          (`self.Part4`))
        (:`5`
          (`self.Part5`))
        (:`6`
          (`self.Part6`))
        (:`7`
          (`self.Part7`))
        (:`8`
          (`self.Part8`))))))

(fn `UserConstructionScript`)