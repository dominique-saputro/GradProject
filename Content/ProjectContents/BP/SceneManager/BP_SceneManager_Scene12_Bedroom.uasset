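; Scene manager for the Scene 12 bedroom cutscene, which runs a BigSister dialog and then transitions to the classroom level.
; When the scene index matches, it spawns the level actors and positions the player and follow camera.
; Interact cycles dialog, and once finished, Part1 hands the camera to a spawned dummy actor that a Timeline slides to pan the view.
; It then advances the GameInstance scene, fades to black and opens Game_Classroom.
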(event `self.ReceiveBeginPlay`
  (bind _iscorrectscene (`/Game/ProjectContents/BP/BP_FunctionLib.CheckSceneIndex` (`self.CurrentScene`)))
  (if _iscorrectscene
    (`self.LevelSetup`)
    (bind _returnvalue (`GameplayStatics.GetActorOfClass` "/Game/ProjectContents/BP/LevelActors/BP_DialogManager.BP_DialogManager_C"))
    (set `self.Level Dialog Manager` _returnvalue)))

(event `InputAction|Interact`
  (params (Key :type "Key Structure"))
  (bind _level_dialog_manager (`self.Level Dialog Manager`))
  ;[1 1 1] OnInteract
  (:`Pressed`
    (if (`/Game/ProjectContents/BP/LevelActors/BP_DialogManager.isDIalogFinished` _level_dialog_manager)
      (set `/Game/ProjectContents/BP/LevelActors/BP_DialogManager.isDIalogFinished` false _level_dialog_manager)
      (bind _asbp_game_instance (cast `/Game/ProjectContents/BP/BP_GameInstance` (`GameplayStatics.GetGameInstance`)))
      (set `/Game/ProjectContents/BP/BP_GameInstance.isViewingScene` false _asbp_game_instance)
      (`KismetSystemLibrary.PrintString` "DialogFinished")
      (`self.MoveToNextPart`)
      (else
        (`/Game/ProjectContents/BP/LevelActors/BP_DialogManager.Test-CycleOnKey` _level_dialog_manager)))))

(event `Handle Start Dialog`
  (bind _followcamera (`self.FollowCamera`))
  (bind _dialog_delay (`/Game/ProjectContents/BP/LevelActors/BP_DialogManager.Display Dialog` (`self.Level Dialog Manager`) (`self.BigSister`) (`self.Big Sister`) (`self.TextDelay`)))
  (`KismetSystemLibrary.Delay` _dialog_delay)
  (set `/Game/ProjectContents/BP/LevelActors/BP_FollowCamera.MaxCameraX` (* (`/Game/ProjectContents/BP/LevelActors/BP_FollowCamera.MinCameraX` _followcamera) -1.0) _followcamera)
  (`self.HandleDummyActor`))

(event `HandleDummyActor`
  (bind _returnvalue (`self.K2_GetActorLocation` (`GameplayStatics.GetPlayerPawn` 0)))
  ;[1 1 1] Handle Switch Player with Dummy Actor
  (bind _returnvalue_2 (`|SpawnActorFromClass` "/Game/ProjectContents/BP/Objects/BP_DummyActor.BP_DummyActor_C" (`KismetMathLibrary.MakeTransform` _returnvalue) "Undefined" "OverrideRootScale" null null))
  (set `/Game/ProjectContents/BP/LevelActors/BP_FollowCamera.ActorToFollow` _returnvalue_2 (`self.FollowCamera`))
  (`KismetSystemLibrary.PrintString` "Switched ActorToFollow")
  (set `self.Start` _returnvalue)
  (set `self.End` (- _returnvalue (-1500.0 0.0 0.0)))
  (`self.HandleMoveCameraRight`))

(event `Part0`
  (`/Game/ProjectContents/BP/BP_FunctionLib.SetupDialogManagerCycle` (`self.Level Dialog Manager`) (`self.BigSister`) (`self.Big Sister`) self))

(event `Part1`
  (bind _followcamera (`self.FollowCamera`))
  (set `/Game/ProjectContents/BP/LevelActors/BP_FollowCamera.MaxCameraX` (* (`/Game/ProjectContents/BP/LevelActors/BP_FollowCamera.MinCameraX` _followcamera) -1.0) _followcamera)
  (`self.HandleDummyActor`))

(event `HandleMoveCameraRight`
  ;[1 1 1] Handle Move CAmera Right
  (bind _returnvalue (`GameplayStatics.GetActorOfClass` "/Game/ProjectContents/BP/Objects/BP_DummyActor.BP_DummyActor_C"))
  (bind (_direction _alpha) (`Timeline|Timeline_0` :!via `PlayFromStart`)
    (:`Update`
      (`self.K2_SetActorLocation` _returnvalue (`KismetMathLibrary.VLerp` (`self.Start`) (`self.End`) _alpha) false false))
    (:`Finished`
      (`KismetSystemLibrary.Delay` 3.0)
      (`self.Handle End Scene`))))

(event `HandleMOveCameraLeft`
  ;[1 1 1] Handle Move Camera Left
  (bind _returnvalue (`GameplayStatics.GetActorOfClass` "/Game/ProjectContents/BP/Objects/BP_DummyActor.BP_DummyActor_C"))
  (bind (_direction _alpha) (`Timeline|Timeline_1` :!via `PlayFromStart`)
    (:`Update`
      (`self.K2_SetActorLocation` _returnvalue (`KismetMathLibrary.VLerp` (`self.End`) (`self.Start`) _alpha) false false))
    (:`Finished`
      (`KismetSystemLibrary.Delay` 2.0))))

(event `Handle End Scene`
  (bind _asbp_game_instance (cast `/Game/ProjectContents/BP/BP_GameInstance` (`GameplayStatics.GetGameInstance`)))
  (`/Game/ProjectContents/BP/BP_GameInstance.MoveToNextScene` _asbp_game_instance)
  (bind _returnvalue (`|CreateWidget` "/Game/ProjectContents/BP/Widgets/WBP_FadeBlack.WBP_FadeBlack_C" (`GameplayStatics.GetPlayerController` 0)))
  (`UserWidget.AddToViewport` _returnvalue 0)
  (`/Game/ProjectContents/BP/Widgets/WBP_FadeBlack.FadeToBlack` _returnvalue)
  (`KismetSystemLibrary.Delay` 0.5)
  (`GameplayStatics.OpenLevel` "Game_Classroom"))

(fn `LevelSetup`
  (for (_array_element _array_index) (`self.LevelActors`)
    (bind _returnvalue (`|SpawnActorFromClass` _array_element (`|GetArrayItem` (`self.ActorSpawns`) _array_index) "Undefined" "OverrideRootScale" null null))
    (if (== _array_index 0)
      (set `self.BigSister` _returnvalue)))
  (`self.K2_SetActorLocation` (`GameplayStatics.GetPlayerPawn` 0) (`self.PlayerSpawn`) false false)
  (`/Game/ProjectContents/BP/BP_FunctionLib.Flip FlipBook` (`self.BigSister`))
  (bind _returnvalue_2 (`GameplayStatics.GetActorOfClass` "/Game/ProjectContents/BP/LevelActors/BP_FollowCamera.BP_FollowCamera_C"))
  (bind _output_get (set `self.FollowCamera` _returnvalue_2))
  (set `/Game/ProjectContents/BP/LevelActors/BP_FollowCamera.MaxCameraX` (`/Game/ProjectContents/BP/LevelActors/BP_FollowCamera.MinCameraX` _output_get) _output_get))

(fn `MoveToNextPart`
  (`self.DisableInput` (`GameplayStatics.GetPlayerController` 0))
  (bind _result (`/Engine/EditorBlueprintResources/StandardMacros.IncrementInt` (`self.CurrentPart`))
    (:`  `
      (switch `int` _result
        (:`1`
          (`self.Part1`))))))

(fn `UserConstructionScript`)