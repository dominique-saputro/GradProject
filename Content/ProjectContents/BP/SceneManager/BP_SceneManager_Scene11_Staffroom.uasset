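; Scene manager for the staffroom scene (Scene 11), a scripted conversation between Teacher, Mother and BigSister.
; When the scene index check passes, it spawns the NPCs, plays office audio and shows a season-change widget.
; Interact cycles dialogue and advances numbered parts, each handing one speaker's lines to the dialog manager.
; The last part advances the game instance's scene, fades to black and opens Game_House.
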(event `self.ReceiveBeginPlay`
  (bind _iscorrectscene (`/Game/ProjectContents/BP/BP_FunctionLib.CheckSceneIndex` (`self.CurrentScene`)))
  (if _iscorrectscene
    (`self.LevelSetup`)
    (bind _returnvalue (`GameplayStatics.GetActorOfClass` "/Game/ProjectContents/BP/LevelActors/BP_DialogManager.BP_DialogManager_C"))
    (set `self.Level Dialog Manager` _returnvalue)
    (`self.Handle Start Widget`)))

(event `InputAction|Interact`
  (params (Key :type "Key Structure"))
  ;[1 1 1] OnInteract
  (:`Pressed`
    (bind _asbp_game_instance (cast `/Game/ProjectContents/BP/BP_GameInstance` (`GameplayStatics.GetGameInstance`)))
    (if (`/Game/ProjectContents/BP/BP_GameInstance.isViewingScene` _asbp_game_instance)
      (if (`/Game/ProjectContents/BP/LevelActors/BP_DialogManager.isDIalogFinished` (`self.Level Dialog Manager`))
        (set `/Game/ProjectContents/BP/LevelActors/BP_DialogManager.isDIalogFinished` false (`self.Level Dialog Manager`))
        (bind _asbp_game_instance_2 (cast `/Game/ProjectContents/BP/BP_GameInstance` (`GameplayStatics.GetGameInstance`)))
        (set `/Game/ProjectContents/BP/BP_GameInstance.isViewingScene` false _asbp_game_instance_2)
        (`KismetSystemLibrary.PrintString` "DialogFinished")
        (`self.MoveToNextPart`)
        (else
          (`/Game/ProjectContents/BP/LevelActors/BP_DialogManager.Test-CycleOnKey` (`self.Level Dialog Manager`)))))))

(event `Handle Start Widget`
  ;[1 1 1] Handle Starting Widget
  (bind _returnvalue (`|CreateWidget` "/Game/ProjectContents/BP/Widgets/WBP_SeasonChange.WBP_SeasonChange_C" (`GameplayStatics.GetPlayerController` 0)))
  (`UserWidget.AddToViewport` _returnvalue 0))

(event `Part0`
  (`/Game/ProjectContents/BP/BP_FunctionLib.SetupDialogManagerCycle` (`self.Level Dialog Manager`) (`self.Teacher`) (`self.Teacher1`) self))

(event `Handle Start Dialog`
  ;[1 1 1] Handle Dialog
  (bind _dialog_delay (`/Game/ProjectContents/BP/LevelActors/BP_DialogManager.Display Dialog` (`self.Level Dialog Manager`) (`self.Teacher`) (`self.Teacher1`) (`self.TextDelay`)))
  (`KismetSystemLibrary.Delay` _dialog_delay)
  (bind _dialog_delay_2 (`/Game/ProjectContents/BP/LevelActors/BP_DialogManager.Display Dialog` (`self.Level Dialog Manager`) (`self.Mother`) (`self.Mother1`) (`self.TextDelay`)))
  (`KismetSystemLibrary.Delay` _dialog_delay_2)
  (bind _dialog_delay_3 (`/Game/ProjectContents/BP/LevelActors/BP_DialogManager.Display Dialog` (`self.Level Dialog Manager`) (`self.Teacher`) (`self.Teacher2`) (`self.TextDelay`)))
  (`KismetSystemLibrary.Delay` _dialog_delay_3)
  (bind _dialog_delay_4 (`/Game/ProjectContents/BP/LevelActors/BP_DialogManager.Display Dialog` (`self.Level Dialog Manager`) (`self.Mother`) (`self.Mother2`) (`self.TextDelay`)))
  (`KismetSystemLibrary.Delay` _dialog_delay_4))

(event `Part1`
  (`/Game/ProjectContents/BP/BP_FunctionLib.SetupDialogManagerCycle` (`self.Level Dialog Manager`) (`self.Mother`) (`self.Mother1`) self))

(event `Part2`
  (`/Game/ProjectContents/BP/BP_FunctionLib.SetupDialogManagerCycle` (`self.Level Dialog Manager`) (`self.Teacher`) (`self.Teacher2`) self))

(event `Handle Move Sister and Mother`
  ;[1 1 1] Handle Move
  (`/Game/ProjectContents/BP/NPC/BP_NPCActorBase.MoveNPC Event` (`self.Mother`) (`self.Mother Start`) (`self.Mother End`))
  (`KismetSystemLibrary.Delay` 0.5)
  (`/Game/ProjectContents/BP/NPC/BP_NPCActorBase.MoveNPC Event` (`self.BigSister`) (`self.Sister Start`) (`self.Sister End`))
  (`KismetSystemLibrary.Delay` 3.0)
  (`self.K2_DestroyActor` (`self.BigSister`))
  (`self.K2_DestroyActor` (`self.Mother`))
  (`self.Handle EndScene`))

(event `Part3`
  (`/Game/ProjectContents/BP/BP_FunctionLib.SetupDialogManagerCycle` (`self.Level Dialog Manager`) (`self.Mother`) (`self.Mother2`) self))

(event `Handle EndScene`
  ;[1 1 1] Handle End Scene
  (bind _asbp_game_instance (cast `/Game/ProjectContents/BP/BP_GameInstance` (`GameplayStatics.GetGameInstance`)))
  (`/Game/ProjectContents/BP/BP_GameInstance.MoveToNextScene` _asbp_game_instance)
  (bind _returnvalue (`|CreateWidget` "/Game/ProjectContents/BP/Widgets/WBP_FadeBlack.WBP_FadeBlack_C" (`GameplayStatics.GetPlayerController` 0)))
  (`UserWidget.AddToViewport` _returnvalue 0)
  (`/Game/ProjectContents/BP/Widgets/WBP_FadeBlack.FadeToBlack` _returnvalue)
  (`KismetSystemLibrary.Delay` 0.5)
  (`GameplayStatics.OpenLevel` "Game_House"))

(event `Part4`
  (`/Game/ProjectContents/BP/BP_FunctionLib.SetupDialogManagerCycle` (`self.Level Dialog Manager`) (`self.BigSister`) (`self.BigSister1`) self))

(event `Part5`
  (`self.Handle EndScene`))

(fn `LevelSetup`
  (bind _output_location (`KismetMathLibrary.BreakTransform` (`|GetArrayItem` (`self.ActorSpawns`) 2)))
  (bind _output_location_2 (`KismetMathLibrary.BreakTransform` (`|GetArrayItem` (`self.ActorSpawns`) 1)))
  (for (_array_element _array_index) (`self.LevelActors`)
    (bind _returnvalue (`|SpawnActorFromClass` _array_element (`|GetArrayItem` (`self.ActorSpawns`) _array_index) "Undefined" "OverrideRootScale" null null))
    (switch `int` _array_index
      (:`0`
        (bind _asbp_npcactor_teacher (cast `/Game/ProjectContents/BP/NPC/BP_NPCActor_Teacher` _returnvalue))
        (set `self.Teacher` _asbp_npcactor_teacher))
      (:`1`
        (bind _asbp_npcactor_big_sister (cast `/Game/ProjectContents/BP/NPC/BP_NPCActor_BigSister` _returnvalue))
        (set `self.BigSister` _asbp_npcactor_big_sister))
      (:`2`
        (bind _asbp_npcactor_mother (cast `/Game/ProjectContents/BP/NPC/BP_NPCActor_Mother` _returnvalue))
        (set `self.Mother` _asbp_npcactor_mother))))
  (`/Game/ProjectContents/BP/BP_FunctionLib.Flip FlipBook` (`self.Mother`))
  (`/Game/ProjectContents/BP/BP_FunctionLib.Flip FlipBook` (`self.BigSister`))
  (set `self.Sister Start` _output_location_2)
  (set `self.Mother Start` _output_location)
  (bind _returnvalue_2 (`|CreateWidget` "/Game/ProjectContents/BP/Widgets/WBP_SeasonChange.WBP_SeasonChange_C" (`GameplayStatics.GetPlayerController` 0)))
  (`UserWidget.AddToViewport` _returnvalue_2 0)
  (`GameplayStatics.PlaySound2D` "/Game/ProjectContents/Music/Final/School_office.School_office" 1.0 1.0 0.0 null null))

(fn `MoveToNextPart`
  (`self.DisableInput` (`GameplayStatics.GetPlayerController` 0))
  (bind _result (`/Engine/EditorBlueprintResources/StandardMacros.IncrementInt` (`self.CurrentPart`))
    (:`  `
      (bind _asbp_game_instance (cast `/Game/ProjectContents/BP/BP_GameInstance` (`GameplayStatics.GetGameInstance`)))
      (bind _output_get (set `/Game/ProjectContents/BP/BP_GameInstance.ScenePart` _result _asbp_game_instance))
      (switch `int` _output_get
        (:`1`
          (`self.Part1`))
        (:`2`
          (`self.Part2`))
        (:`3`
          (`self.Part3`))
        (:`4`
          (`self.Part4`))
        (:`5`
          (`self.Part5`))))))

(fn `UserConstructionScript`)