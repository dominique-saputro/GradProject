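; Scene manager for the Park (Scene 08), a scripted story sequence between two sisters that ends by loading the staffroom level.
; BeginPlay checks the scene index, spawns the sisters and plays a delay-timed ball game before the first dialogue.
; Interact cycles dialogue through BP_DialogManager, then advances numbered Part events via MoveToNextPart, or shows a hint.
; Parts stage NPC moves, a dummy-actor camera pan and a blacked-out climbing moment with sound.
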(event `InputAction|Interact`
  (params (Key :type "Key Structure"))
  ;[1 1 1] OnInteract
  (:`Pressed`
    (bind _asbp_game_instance (cast `/Game/ProjectContents/BP/BP_GameInstance` (`GameplayStatics.GetGameInstance`)))
    (if (`/Game/ProjectContents/BP/BP_GameInstance.isViewingScene` _asbp_game_instance)
      (if (`/Game/ProjectContents/BP/LevelActors/BP_DialogManager.isDIalogFinished` (`self.Level Dialog Manager`))
        (set `/Game/ProjectContents/BP/LevelActors/BP_DialogManager.isDIalogFinished` false (`self.Level Dialog Manager`))
        (bind _asbp_game_instance_2 (cast `/Game/ProjectContents/BP/BP_GameInstance` (`GameplayStatics.GetGameInstance`)))
        (set `/Game/ProjectContents/BP/BP_GameInstance.isViewingScene` false _asbp_game_instance_2)
        (`KismetSystemLibrary.PrintString` "DialogFinished")
        (`self.MoveToNextPart`)
        (else
          (`/Game/ProjectContents/BP/LevelActors/BP_DialogManager.Test-CycleOnKey` (`self.Level Dialog Manager`))))
      (else
        (`/Game/ProjectContents/BP/BP_FunctionLib.TriggerHint`)))))

(event `self.ReceiveBeginPlay`
  (bind _iscorrectscene (`/Game/ProjectContents/BP/BP_FunctionLib.CheckSceneIndex` (`self.CurrentScene`)))
  (if _iscorrectscene
    (`self.LevelSetup`)
    (bind _returnvalue (`GameplayStatics.GetActorOfClass` "/Game/ProjectContents/BP/LevelActors/BP_DialogManager.BP_DialogManager_C"))
    (set `self.Level Dialog Manager` _returnvalue)
    (`self.HandlePlayBall`)))

(event `HandlePlayBall`
  ;[1 1 1] Handle Play Ball
  (`/Game/ProjectContents/BP/BP_FunctionLib.Flip FlipBook` (`self.BigSister`))
  (`KismetSystemLibrary.Delay` 1.0)
  (`self.MoveBall Left` (-500.0 0.0 0.0))
  (`KismetSystemLibrary.Delay` 2.0)
  (`self.MoveBall Right` (500.0 0.0 0.0))
  (`KismetSystemLibrary.Delay` 2.0)
  (`self.MoveBall Left` (-500.0 0.0 0.0))
  (`KismetSystemLibrary.Delay` 2.0)
  (`self.MoveBall Right` (1500.0 0.0 0.0))
  (`self.Part0`))

(event `Part0`
  (`KismetSystemLibrary.Delay` 1.0)
  (bind _asbp_npcactor_base (cast `/Game/ProjectContents/BP/NPC/BP_NPCActorBase` (`self.BigSister`)))
  (`/Game/ProjectContents/BP/BP_FunctionLib.Flip FlipBook` _asbp_npcactor_base)
  (`/Game/ProjectContents/BP/BP_FunctionLib.SetupDialogManagerCycle` (`self.Level Dialog Manager`) (`self.BigSister`) (`self.Big Sister0`) self))

(event `MoveBall Right`
  (params (MoveLrngth :type "Vector Structure" :default (500.0 0.0 0.0)))
  ;[1 1 1] Handle MoveBall
  (bind _returnvalue (`GameplayStatics.GetActorOfClass` "/Game/ProjectContents/BP/Objects/BP_Ball.BP_Ball_C"))
  (set `/Game/ProjectContents/BP/Objects/BP_Ball.GoalPoint` (+ (`/Game/ProjectContents/BP/Objects/BP_Ball.StartPoint` _returnvalue) MoveLrngth) _returnvalue)
  (set `/Game/ProjectContents/BP/Objects/BP_Ball.RotationMultipier` -400.0 _returnvalue)
  (`/Game/ProjectContents/BP/Objects/BP_Ball.MoveBall` _returnvalue))

(event `MoveBall Left`
  (params (MoveLength :type "Vector Structure"))
  ;[1 1 1] Handle MoveBall
  (bind _returnvalue (`GameplayStatics.GetActorOfClass` "/Game/ProjectContents/BP/Objects/BP_Ball.BP_Ball_C"))
  (set `/Game/ProjectContents/BP/Objects/BP_Ball.GoalPoint` (+ (`/Game/ProjectContents/BP/Objects/BP_Ball.StartPoint` _returnvalue) MoveLength) _returnvalue)
  (set `/Game/ProjectContents/BP/Objects/BP_Ball.RotationMultipier` 400.0 _returnvalue)
  (`/Game/ProjectContents/BP/Objects/BP_Ball.MoveBall` _returnvalue))

(event `Part1`
  (bind _bigsister (`self.BigSister`))
  (bind _returnvalue (`self.K2_GetActorLocation` _bigsister))
  (`/Game/ProjectContents/BP/BP_FunctionLib.SetupDialogManagerCycle` (`self.Level Dialog Manager`) (`self.LittleSister`) (`self.LittleSIster0`) self)
  (bind _asbp_npcactor_base (cast `/Game/ProjectContents/BP/NPC/BP_NPCActorBase` _bigsister))
  (`/Game/ProjectContents/BP/NPC/BP_NPCActorBase.MoveNPC Event` _asbp_npcactor_base _returnvalue (+ _returnvalue (800.0 0.0 0.0)))
  (bind _asbp_game_instance (cast `/Game/ProjectContents/BP/BP_GameInstance` (`GameplayStatics.GetGameInstance`)))
  (set `/Game/ProjectContents/BP/BP_GameInstance.IsScene8PlayBallFinished` true _asbp_game_instance))

(event `Handle BigSIsterMove`
  ;[1 1 1] Handle Big Sister Move
  (`KismetSystemLibrary.Delay` 1.0)
  (bind _asbp_npcactor_base (cast `/Game/ProjectContents/BP/NPC/BP_NPCActorBase` (`self.BigSister`)))
  (`/Game/ProjectContents/BP/BP_FunctionLib.Flip FlipBook` _asbp_npcactor_base)
  (`KismetSystemLibrary.Delay` 1.0)
  (bind _returnvalue (`self.K2_GetActorLocation` _asbp_npcactor_base))
  (`/Game/ProjectContents/BP/NPC/BP_NPCActorBase.MoveNPC Event` _asbp_npcactor_base _returnvalue (+ _returnvalue (550.0 0.0 0.0)))
  (bind _asbp_game_instance (cast `/Game/ProjectContents/BP/BP_GameInstance` (`GameplayStatics.GetGameInstance`)))
  (set `/Game/ProjectContents/BP/BP_GameInstance.IsScene8PlayBallFinished` true _asbp_game_instance))

(event `Part2`
  (bind _bigsister (`self.BigSister`))
  (bind _returnvalue (`self.K2_GetActorLocation` _bigsister))
  (`self.DisableInput` (`GameplayStatics.GetPlayerPawn` 0) (`GameplayStatics.GetPlayerController` 0))
  (`self.Handle Change Camera Follow`)
  (`KismetSystemLibrary.Delay` 6.0)
  (`self.EnableInput` (`GameplayStatics.GetPlayerPawn` 0) (`GameplayStatics.GetPlayerController` 0))
  (`self.SetActorEnableCollision` _bigsister false)
  (`/Game/ProjectContents/BP/BP_FunctionLib.Flip FlipBook` _bigsister)
  (bind _asbp_npcactor_base (cast `/Game/ProjectContents/BP/NPC/BP_NPCActorBase` _bigsister))
  (`/Game/ProjectContents/BP/NPC/BP_NPCActorBase.MoveNPC Event` _asbp_npcactor_base _returnvalue (+ _returnvalue (-1200.0 0.0 0.0)))
  (`KismetSystemLibrary.Delay` 3.0)
  (`/Game/ProjectContents/BP/BP_FunctionLib.SetupDialogManagerCycle` (`self.Level Dialog Manager`) (`self.BigSister`) (`self.Big Sister`) self))

(event `Handle Change Camera Follow`
  ;[1 1 1] Handle Camera Move
  (bind _returnvalue (`GameplayStatics.GetActorOfClass` "/Game/ProjectContents/BP/LevelActors/BP_FollowCamera.BP_FollowCamera_C"))
  (bind _returnvalue_2 (`|SpawnActorFromClass` "/Game/ProjectContents/BP/Objects/BP_DummyActor.BP_DummyActor_C" (`KismetMathLibrary.MakeTransform` (`self.K2_GetActorLocation` (`GameplayStatics.GetPlayerPawn` 0))) "Undefined" "OverrideRootScale" null null))
  (set `/Game/ProjectContents/BP/LevelActors/BP_FollowCamera.ActorToFollow` _returnvalue_2 _returnvalue)
  (set `self.Start` (`self.K2_GetActorLocation` _returnvalue_2))
  (bind (_returnvalue_x _returnvalue_y _returnvalue_z) (`KismetMathLibrary.BreakVector` (`self.K2_GetActorLocation` _returnvalue_2)))
  (set `self.End` (`KismetMathLibrary.MakeVector` 550.0 _returnvalue_y _returnvalue_z))
  (bind (_direction _alpha) (`Timeline|MoveDummyActor` :!via `PlayFromStart`)
    (:`Update`
      (`self.K2_SetActorLocation` _returnvalue_2 (`KismetMathLibrary.VLerp` (`self.Start`) (`self.End`) _alpha) false false)
      (if (== _alpha 1.0)
        (`self.K2_SetActorLocation` (`self.LittleSister`) (-950.0 30.0 675.0) false false)))
    (:`Finished`
      (bind _returnvalue_3 (`GameplayStatics.GetActorOfClass` "/Game/ProjectContents/BP/LevelActors/BP_FollowCamera.BP_FollowCamera_C"))
      (set `/Game/ProjectContents/BP/LevelActors/BP_FollowCamera.ActorToFollow` (`GameplayStatics.GetPlayerPawn` 0) _returnvalue_3)
      (`self.K2_DestroyActor` _returnvalue_2))))

(event `Part3`
  (`/Game/ProjectContents/BP/BP_FunctionLib.SetupDialogManagerCycle` (`self.Level Dialog Manager`) (`self.LittleSister`) (`self.LittleSIster1`) self))

(event `Part4`
  (`/Game/ProjectContents/BP/BP_FunctionLib.SetupDialogManagerCycle` (`self.Level Dialog Manager`) (`self.BigSister`) (`self.Big Sister1`) self))

(event `Part5`
  (`self.HandleClimbing`)
  (`KismetSystemLibrary.Delay` 1.5)
  (`/Game/ProjectContents/BP/BP_FunctionLib.SetupDialogManagerCycle` (`self.Level Dialog Manager`) (`self.LittleSister`) (`self.Little Sister2`) self)
  (`self.EnableInput` (`GameplayStatics.GetPlayerPawn` 0) (`GameplayStatics.GetPlayerController` 0)))

(event `Handle Dialog 1`
  (bind _bigsister (`self.BigSister`))
  (bind _returnvalue (`self.K2_GetActorLocation` _bigsister))
  ;[1 1 1] Handle Dialog 1
  (`self.EnableInput` (`GameplayStatics.GetPlayerPawn` 0) (`GameplayStatics.GetPlayerController` 0))
  (`|ExecutionSequence`
    (:`then_0`
      (`/Game/ProjectContents/BP/BP_FunctionLib.Flip FlipBook` _bigsister)
      (`/Game/ProjectContents/BP/LevelActors/BP_DialogManager.DisplayTextAlways` (`self.Level Dialog Manager`) _bigsister "!!!")
      (`KismetSystemLibrary.Delay` 2.0)
      (bind _asbp_npcactor_base (cast `/Game/ProjectContents/BP/NPC/BP_NPCActorBase` _bigsister))
      (`/Game/ProjectContents/BP/NPC/BP_NPCActorBase.MoveNPC Event` _asbp_npcactor_base _returnvalue (+ _returnvalue (-550.0 0.0 0.0))))
    (:`then_1`
      (`KismetSystemLibrary.Delay` 3.0)
      (bind _dialog_delay (`/Game/ProjectContents/BP/LevelActors/BP_DialogManager.Display Dialog` (`self.Level Dialog Manager`) (`self.LittleSister`) (`self.LittleSIster1`) (`self.TextDelay`)))
      (`KismetSystemLibrary.Delay` _dialog_delay)
      (bind _dialog_delay_2 (`/Game/ProjectContents/BP/LevelActors/BP_DialogManager.Display Dialog` (`self.Level Dialog Manager`) (`self.BigSister`) (`self.Big Sister1`) (`self.TextDelay`)))
      (`KismetSystemLibrary.Delay` _dialog_delay_2)
      (`self.HandleClimbing`))))

(event `Part6`
  (`/Game/ProjectContents/BP/BP_FunctionLib.SetupDialogManagerCycle` (`self.Level Dialog Manager`) (`self.BigSister`) (`self.Big Sister2`) self))

(event `Part7`
  (`/Game/ProjectContents/BP/BP_FunctionLib.SetupDialogManagerCycle` (`self.Level Dialog Manager`) (`self.LittleSister`) (`self.Little SIster3`) self))

(event `HandleClimbing`
  ;[1 1 1] Handle Climbing
  (`|ExecutionSequence`
    (:`then_0`
      (bind _returnvalue (`|CreateWidget` "/Game/ProjectContents/BP/Widgets/WBP_FadeBlack.WBP_FadeBlack_C" (`GameplayStatics.GetPlayerController` 0)))
      (`UserWidget.AddToViewport` _returnvalue 0)
      (`/Game/ProjectContents/BP/Widgets/WBP_FadeBlack.FadeToBlack` _returnvalue)
      (`KismetSystemLibrary.Delay` 0.5)
      (bind _returnvalue_2 (`|CreateWidget` "/Game/ProjectContents/BP/Widgets/WBP_Black.WBP_Black_C" (`GameplayStatics.GetPlayerController` 0)))
      (`UserWidget.AddToViewport` _returnvalue_2 0)
      (`Widget.RemoveFromParent` _returnvalue))
    (:`then_1`
      (`GameplayStatics.PlaySound2D` "/Game/ProjectContents/SFX/SFX_ClimbingFalling.SFX_ClimbingFalling" 1.0 1.0 0.0 null null))
    (:`then_2`
      (`KismetSystemLibrary.Delay` 6.0)
      (bind _returnvalue_3 (`|CreateWidget` "/Game/ProjectContents/BP/Widgets/WBP_FadeBlack.WBP_FadeBlack_C" (`GameplayStatics.GetPlayerController` 0)))
      (`UserWidget.AddToViewport` _returnvalue_3 0)
      (`/Game/ProjectContents/BP/Widgets/WBP_FadeBlack.FadeFromBlack` _returnvalue_3)
      (`Widget.RemoveFromParent` _returnvalue_2))))

(event `Part8`
  (`/Game/ProjectContents/BP/BP_FunctionLib.SetupDialogManagerCycle` (`self.Level Dialog Manager`) (`self.BigSister`) (`self.Big SIster3`) self))

(event `Part9`
  (`/Game/ProjectContents/BP/BP_FunctionLib.SetupDialogManagerCycle` (`self.Level Dialog Manager`) (`self.LittleSister`) (`self.Little Sister4`) self))

(event `Part10`
  (`self.Handle End Scene`))

(event `Handle Dialog 2`
  ;[1 1 1] Handle Dialog 2
  (`self.EnableInput` (`GameplayStatics.GetPlayerPawn` 0) (`GameplayStatics.GetPlayerController` 0))
  (`KismetSystemLibrary.Delay` 1.5)
  (bind _dialog_delay (`/Game/ProjectContents/BP/LevelActors/BP_DialogManager.Display Dialog` (`self.Level Dialog Manager`) (`self.LittleSister`) (`self.Little Sister2`) (`self.TextDelay`)))
  (`KismetSystemLibrary.Delay` _dialog_delay)
  (bind _dialog_delay_2 (`/Game/ProjectContents/BP/LevelActors/BP_DialogManager.Display Dialog` (`self.Level Dialog Manager`) (`self.BigSister`) (`self.Big Sister2`) (`self.TextDelay`)))
  (`KismetSystemLibrary.Delay` _dialog_delay_2)
  (bind _dialog_delay_3 (`/Game/ProjectContents/BP/LevelActors/BP_DialogManager.Display Dialog` (`self.Level Dialog Manager`) (`self.LittleSister`) (`self.Little SIster3`) (`self.TextDelay`)))
  (`KismetSystemLibrary.Delay` _dialog_delay_3)
  (bind _dialog_delay_4 (`/Game/ProjectContents/BP/LevelActors/BP_DialogManager.Display Dialog` (`self.Level Dialog Manager`) (`self.BigSister`) (`self.Big SIster3`) (`self.TextDelay`)))
  (`KismetSystemLibrary.Delay` _dialog_delay_4)
  (bind _dialog_delay_5 (`/Game/ProjectContents/BP/LevelActors/BP_DialogManager.Display Dialog` (`self.Level Dialog Manager`) (`self.LittleSister`) (`self.Little Sister4`) (`self.TextDelay`)))
  (`KismetSystemLibrary.Delay` _dialog_delay_5)
  (`self.Handle End Scene`))

(event `Handle End Scene`
  (bind _asbp_game_instance (cast `/Game/ProjectContents/BP/BP_GameInstance` (`GameplayStatics.GetGameInstance`)))
  (`/Game/ProjectContents/BP/BP_GameInstance.MoveToNextScene` _asbp_game_instance)
  (bind _returnvalue (`|CreateWidget` "/Game/ProjectContents/BP/Widgets/WBP_FadeBlack.WBP_FadeBlack_C" (`GameplayStatics.GetPlayerController` 0)))
  (`UserWidget.AddToViewport` _returnvalue 0)
  (`/Game/ProjectContents/BP/Widgets/WBP_FadeBlack.FadeToBlack` _returnvalue)
  (`KismetSystemLibrary.Delay` 0.5)
  (`GameplayStatics.OpenLevel` "Game_Staffroom"))

(fn `LevelSetup`
  (for (_array_element _array_index) (`self.LevelActors`)
    (bind _returnvalue (`|SpawnActorFromClass` _array_element (`|GetArrayItem` (`self.ActorSpawns`) _array_index) "Undefined" "OverrideRootScale" null null))
    (switch `int` _array_index
      (:`0`
        (set `self.BigSister` _returnvalue))
      (:`1`
        (set `self.LittleSister` _returnvalue))))
  (`GameplayStatics.PlaySound2D` "/Game/ProjectContents/Music/BGM_Park.BGM_Park" 1.0 1.0 0.0 null null))

(fn `MoveToNextPart`
  (`self.DisableInput` (`GameplayStatics.GetPlayerController` 0))
  (bind _result (`/Engine/EditorBlueprintResources/StandardMacros.IncrementInt` (`self.CurrentPart`))
    (:`  `
      (bind _asbp_game_instance (cast `/Game/ProjectContents/BP/BP_GameInstance` (`GameplayStatics.GetGameInstance`)))
      (bind _output_get (set `/Game/ProjectContents/BP/BP_GameInstance.ScenePart` _result _asbp_game_instance))
      (switch `int` _output_get
        (:`1`
          (`self.Part1`))
        (:`2`
          (`self.Part2`))
        (:`3`
          (`self.Part3`))
        (:`4`
          (`self.Part4`))
        (:`5`
          (`self.Part5`))
        (:`6`
          (`self.Part6`))
        (:`7`
          (`self.Part7`))
        (:`8`
          (`self.Part8`))
        (:`9`
          (`self.Part9`))
        (:`10`
          (`self.Part10`))))))

(fn `UserConstructionScript`)