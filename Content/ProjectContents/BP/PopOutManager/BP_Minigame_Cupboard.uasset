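; BP_Minigame_Cupboard is a one-shot interaction trigger that starts the cupboard minigame in the Scene04 Cafeteria.
; Player pawn overlap enables input and restyles the NSTrigger particle effect as larger and blue, while leaving disables input and restores it to smaller and white.
; Pressing Interact calls CupboardMinigameStart on the cafeteria scene manager, found by class lookup, then destroys the trigger.
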(event `InputAction|Interact`
  (params (Key :type "Key Structure"))
  (:`Pressed`
    (bind _returnvalue (`GameplayStatics.GetActorOfClass` "/Game/ProjectContents/BP/SceneManager/BP_SceneManager_Scene04_Cafeteria.BP_SceneManager_Scene04_Cafeteria_C"))
    (`/Game/ProjectContents/BP/SceneManager/BP_SceneManager_Scene04_Cafeteria.Cupboard Minigame Start` _returnvalue)
    (`self.K2_DestroyActor`)))

(event `self.ReceiveActorBeginOverlap`
  (params (OtherActor :type "Actor Object Reference"))
  (bind _ns_trigger (`self.NS_Trigger`))
  ;[1 1 1] Toggle Tooltip on Overlap
  (cast `/Game/ProjectContents/BP/Player/BP_PawnPlayerBase` OtherActor)
  (`self.EnableInput` (`GameplayStatics.GetPlayerController` 0))
  (`NiagaraComponent.SetVariableLinearColor` _ns_trigger "Color" (make `LinearColor` 0.0 0.0 1.0 1.0))
  (`NiagaraComponent.SetVariableFloat` _ns_trigger "Size" 30.0)
  (`NiagaraComponent.ReinitializeSystem` _ns_trigger))

(event `self.ReceiveActorEndOverlap`
  (params (OtherActor :type "Actor Object Reference"))
  (bind _ns_trigger (`self.NS_Trigger`))
  ;[1 1 1] Toggle Tooltip on Overlap
  (cast `/Game/ProjectContents/BP/Player/BP_PawnPlayerBase` OtherActor)
  (`self.DisableInput` (`GameplayStatics.GetPlayerController` 0))
  (`NiagaraComponent.SetVariableLinearColor` _ns_trigger "Color" (make `LinearColor` 1.0 1.0 1.0 1.0))
  (`NiagaraComponent.SetVariableFloat` _ns_trigger "Size" 15.0)
  (`NiagaraComponent.ReinitializeSystem` _ns_trigger))

(fn `UserConstructionScript`)