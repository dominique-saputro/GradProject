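; BP_Minigame_Drinks is an interactable trigger that launches the drink minigame in the cafeteria scene.
; When the player pawn overlaps it, it shows a text prompt and enables input; leaving disables input, but the node that would hide the prompt is unconnected.
; Pressing Interact calls DrinkMinigameStart on the Scene04 cafeteria scene manager, then destroys the trigger.
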(event `self.ReceiveActorBeginOverlap`
  (params (OtherActor :type "Actor Object Reference"))
  ;[1 1 1] Toggle Tooltip on Overlap
  (cast `/Game/ProjectContents/BP/Player/BP_PawnPlayerBase` OtherActor)
  (`SceneComponent.SetVisibility` (`self.TextRender`) true false)
  (`self.EnableInput` (`GameplayStatics.GetPlayerController` 0)))

(event `InputAction|Interact`
  (params (Key :type "Key Structure"))
  (:`Pressed`
    (bind _returnvalue (`GameplayStatics.GetActorOfClass` "/Game/ProjectContents/BP/SceneManager/BP_SceneManager_Scene04_Cafeteria.BP_SceneManager_Scene04_Cafeteria_C"))
    (`/Game/ProjectContents/BP/SceneManager/BP_SceneManager_Scene04_Cafeteria.Drink Minigame Start` _returnvalue)
    (`self.K2_DestroyActor`)))

(event `self.ReceiveActorEndOverlap`
  (params (OtherActor :type "Actor Object Reference"))
  ;[1 1 1] Toggle Tooltip on Overlap
  (cast `/Game/ProjectContents/BP/Player/BP_PawnPlayerBase` OtherActor)
  (`self.DisableInput` (`GameplayStatics.GetPlayerController` 0)))

(fn `UserConstructionScript`)