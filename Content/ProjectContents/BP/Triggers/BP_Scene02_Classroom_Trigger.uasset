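; One-shot overlap trigger for the Scene 02 classroom that starts a camera change.
; When a player pawn enters while the game instance's ScenePart is 1, it disables that player's input, calls HandleChangeCamera on the classroom scene manager, then destroys itself.
; On BeginPlay it hides its TextRender label and disables input on itself.
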(event `self.ReceiveBeginPlay`
  (`SceneComponent.SetVisibility` (`self.TextRender`) false false)
  (`self.DisableInput` (`GameplayStatics.GetPlayerController` 0)))

(event `self.ReceiveActorBeginOverlap`
  (params (OtherActor :type "Actor Object Reference"))
  (cast `/Game/ProjectContents/BP/Player/BP_PawnPlayerBase` OtherActor)
  (bind _asbp_game_instance (cast `/Game/ProjectContents/BP/BP_GameInstance` (`GameplayStatics.GetGameInstance`)))
  (if (== (`/Game/ProjectContents/BP/BP_GameInstance.ScenePart` _asbp_game_instance) 1)
    (`self.DisableInput` (`GameplayStatics.GetPlayerPawn` 0) (`GameplayStatics.GetPlayerController` 0))
    (bind _returnvalue (`GameplayStatics.GetActorOfClass` "/Game/ProjectContents/BP/SceneManager/BP_SceneManager_Scene02_Classroom.BP_SceneManager_Scene02_Classroom_C"))
    (`/Game/ProjectContents/BP/SceneManager/BP_SceneManager_Scene02_Classroom.Handle Change Camera` _returnvalue)
    (`self.K2_DestroyActor`)))

(fn `UserConstructionScript`)