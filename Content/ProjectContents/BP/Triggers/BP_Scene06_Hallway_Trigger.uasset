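; A one-shot interact trigger that starts the Scene06 Hallway sequence.
; Overlap by a BP_PawnPlayerBase enables input and restyles the NSTrigger Niagara effect as larger and blue; leaving disables input and restores a small white look.
; Pressing Interact plays a selection sound, calls Part0 on the BP_SceneManager_Scene06_Hallway found in the level, then destroys the trigger.
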(event `InputAction|Interact`
  (params (Key :type "Key Structure"))
  (:`Pressed`
    (`GameplayStatics.PlaySound2D` "/Engine/VREditor/Sounds/UI/Selection_Changes.Selection_Changes" 1.0 1.0 0.0 null null)
    (bind _returnvalue (`GameplayStatics.GetActorOfClass` "/Game/ProjectContents/BP/SceneManager/BP_SceneManager_Scene06_Hallway.BP_SceneManager_Scene06_Hallway_C"))
    (`/Game/ProjectContents/BP/SceneManager/BP_SceneManager_Scene06_Hallway.Part0` _returnvalue)
    (`self.K2_DestroyActor`)))

(event `self.ReceiveBeginPlay`
  (`self.DisableInput` (`GameplayStatics.GetPlayerController` 0)))

(event `self.ReceiveActorBeginOverlap`
  (params (OtherActor :type "Actor Object Reference"))
  (bind _ns_trigger (`self.NS_Trigger`))
  (cast `/Game/ProjectContents/BP/Player/BP_PawnPlayerBase` OtherActor)
  (`self.EnableInput` (`GameplayStatics.GetPlayerController` 0))
  (`NiagaraComponent.SetVariableLinearColor` _ns_trigger "Color" (make `LinearColor` 0.0 0.0 1.0 1.0))
  (`NiagaraComponent.SetVariableFloat` _ns_trigger "Size" 50.0)
  (`NiagaraComponent.ReinitializeSystem` _ns_trigger))

(event `self.ReceiveActorEndOverlap`
  (params (OtherActor :type "Actor Object Reference"))
  (bind _ns_trigger (`self.NS_Trigger`))
  (cast `/Game/ProjectContents/BP/Player/BP_PawnPlayerBase` OtherActor)
  (`self.DisableInput` (`GameplayStatics.GetPlayerController` 0))
  (`NiagaraComponent.SetVariableLinearColor` _ns_trigger "Color" (make `LinearColor` 1.0 1.0 1.0 1.0))
  (`NiagaraComponent.SetVariableFloat` _ns_trigger "Size" 15.0)
  (`NiagaraComponent.ReinitializeSystem` _ns_trigger))

(fn `UserConstructionScript`)