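; Scene 4 classroom interaction trigger that starts the classroom sequence through its scene manager.
; On BeginPlay it destroys itself if the GameInstance marks either the classroom or the cafeteria part as finished.
; Player overlap toggles a text tooltip and actor input.
; Interact, only when the cafeteria flag is set at that moment, calls Part0 on BP_SceneManager_Scene04_Classroom and destroys the trigger.
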(event `self.ReceiveBeginPlay`
  (bind _asbp_game_instance (cast `/Game/ProjectContents/BP/BP_GameInstance` (`GameplayStatics.GetGameInstance`)))
  (if (`/Game/ProjectContents/BP/BP_GameInstance.isScene4ClassroomFinished` _asbp_game_instance)
    (`self.K2_DestroyActor`)
    (else
      (bind _asbp_game_instance_2 (cast `/Game/ProjectContents/BP/BP_GameInstance` (`GameplayStatics.GetGameInstance`)))
      (if (`/Game/ProjectContents/BP/BP_GameInstance.isScene4CafeteriaFinished` _asbp_game_instance_2)
        (`self.K2_DestroyActor`)))))

(event `self.ReceiveActorBeginOverlap`
  (params (OtherActor :type "Actor Object Reference"))
  ;[1 1 1] Toggle Tooltip on Overlap
  (cast `/Game/ProjectContents/BP/Player/BP_PlayerOpenRoom` OtherActor
    (:`then`
      _)
    (:`CastFailed`
      (cast `/Game/ProjectContents/BP/Player/BP_PawnPlayerBase` OtherActor)))
  (`SceneComponent.SetVisibility` (`self.TextRender`) true false)
  (`self.EnableInput` (`GameplayStatics.GetPlayerController` 0)))

(event `InputAction|Interact` :consume false
  (params (Key :type "Key Structure"))
  ;[1 1 1] Start Dialog on Interact
  (:`Pressed`
    (bind _asbp_game_instance (cast `/Game/ProjectContents/BP/BP_GameInstance` (`GameplayStatics.GetGameInstance`)))
    (if (`/Game/ProjectContents/BP/BP_GameInstance.isScene4CafeteriaFinished` _asbp_game_instance)
      (bind _returnvalue (`GameplayStatics.GetActorOfClass` "/Game/ProjectContents/BP/SceneManager/BP_SceneManager_Scene04_Classroom.BP_SceneManager_Scene04_Classroom_C"))
      (`/Game/ProjectContents/BP/SceneManager/BP_SceneManager_Scene04_Classroom.Part0` _returnvalue)
      (`self.K2_DestroyActor`))))

(event `self.ReceiveActorEndOverlap`
  (params (OtherActor :type "Actor Object Reference"))
  ;[1 1 1] Toggle Tooltip on Overlap
  (cast `/Game/ProjectContents/BP/Player/BP_PlayerOpenRoom` OtherActor
    (:`then`
      _)
    (:`CastFailed`
      (cast `/Game/ProjectContents/BP/Player/BP_PawnPlayerBase` OtherActor)))
  (`SceneComponent.SetVisibility` (`self.TextRender`) false false)
  (`self.DisableInput` (`GameplayStatics.GetPlayerController` 0)))

(fn `UserConstructionScript`)