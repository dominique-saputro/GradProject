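; Interaction trigger for the Scene 04 cafeteria that starts or advances its dialog when the player presses Interact inside it.
; Player overlap toggles the actor's input and restyles the Niagara marker by color and size to show it is active.
; On Interact, a GameInstance flag decides whether the cafeteria scene manager runs Part0 or MoveToNextPart, then the trigger destroys itself.
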(event `InputAction|Interact`
  (params (Key :type "Key Structure"))
  ;[1 1 1] Start Dialog on Interact
  (:`Pressed`
    (bind _asbp_game_instance (cast `/Game/ProjectContents/BP/BP_GameInstance` (`GameplayStatics.GetGameInstance`)))
    (if (`/Game/ProjectContents/BP/BP_GameInstance.isScene4CafeteriaFinished` _asbp_game_instance)
      (bind _returnvalue (`GameplayStatics.GetActorOfClass` "/Game/ProjectContents/BP/SceneManager/BP_SceneManager_Scene04_Cafeteria.BP_SceneManager_Scene04_Cafeteria_C"))
      (`/Game/ProjectContents/BP/SceneManager/BP_SceneManager_Scene04_Cafeteria.MoveToNextPart` _returnvalue)
      (`self.K2_DestroyActor`)
      (else
        (bind _returnvalue_2 (`GameplayStatics.GetActorOfClass` "/Game/ProjectContents/BP/SceneManager/BP_SceneManager_Scene04_Cafeteria.BP_SceneManager_Scene04_Cafeteria_C"))
        (`/Game/ProjectContents/BP/SceneManager/BP_SceneManager_Scene04_Cafeteria.Part0` _returnvalue_2)
        (`self.K2_DestroyActor`)))))

(event `self.ReceiveBeginPlay`
  (`self.DisableInput` (`GameplayStatics.GetPlayerController` 0)))

(event `self.ReceiveActorBeginOverlap`
  (params (OtherActor :type "Actor Object Reference"))
  (bind _ns_trigger (`self.NS_Trigger`))
  (cast `/Game/ProjectContents/BP/Player/BP_PawnPlayerBase` OtherActor)
  (`self.EnableInput` (`GameplayStatics.GetPlayerController` 0))
  (`NiagaraComponent.SetVariableLinearColor` _ns_trigger "Color" (make `LinearColor` 0.0 0.0 1.0 1.0))
  (`NiagaraComponent.SetVariableFloat` _ns_trigger "Size" 50.0)
  (`NiagaraComponent.ReinitializeSystem` _ns_trigger))

(event `self.ReceiveActorEndOverlap`
  (params (OtherActor :type "Actor Object Reference"))
  (bind _ns_trigger (`self.NS_Trigger`))
  (cast `/Game/ProjectContents/BP/Player/BP_PawnPlayerBase` OtherActor)
  (`self.DisableInput` (`GameplayStatics.GetPlayerController` 0))
  (`NiagaraComponent.SetVariableLinearColor` _ns_trigger "Color" (make `LinearColor` 1.0 1.0 1.0 1.0))
  (`NiagaraComponent.SetVariableFloat` _ns_trigger "Size" 15.0)
  (`NiagaraComponent.ReinitializeSystem` _ns_trigger))

(fn `UserConstructionScript`)