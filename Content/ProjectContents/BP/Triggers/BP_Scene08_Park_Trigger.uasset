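; BP_Scene08_Park_Trigger is an overlap trigger for the park area of Scene 8.
; On begin play it hides its TextRender label and disables its own input.
; When a player pawn overlaps it and the game instance reports the Scene 8 play-ball event finished, it disables the player pawn's input and looks up the park scene manager.
; The manager reference goes unused, and a DestroyActor node is left unconnected.
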(event `self.ReceiveBeginPlay`
  (`SceneComponent.SetVisibility` (`self.TextRender`) false false)
  (`self.DisableInput` (`GameplayStatics.GetPlayerController` 0)))

(event `self.ReceiveActorBeginOverlap`
  (params (OtherActor :type "Actor Object Reference"))
  (cast `/Game/ProjectContents/BP/Player/BP_PawnPlayerBase` OtherActor)
  (bind _asbp_game_instance (cast `/Game/ProjectContents/BP/BP_GameInstance` (`GameplayStatics.GetGameInstance`)))
  (if (`/Game/ProjectContents/BP/BP_GameInstance.IsScene8PlayBallFinished` _asbp_game_instance)
    (`self.DisableInput` (`GameplayStatics.GetPlayerPawn` 0) (`GameplayStatics.GetPlayerController` 0))
    (`GameplayStatics.GetActorOfClass` "/Game/ProjectContents/BP/SceneManager/BP_SceneManager_Scene08_Park.BP_SceneManager_Scene08_Park_C")))

(fn `UserConstructionScript`)