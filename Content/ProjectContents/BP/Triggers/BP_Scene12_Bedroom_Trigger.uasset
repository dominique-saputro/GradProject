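; BP_Scene12_Bedroom_Trigger is a trigger actor that starts the sister dialog in the Scene 12 bedroom.
; On BeginPlay it hides its text render and disables its own input.
; When a BP_PawnPlayerBase overlaps it, it disables input on the player pawn, calls Part0 on the BP_SceneManager_Scene12_Bedroom found in the level, then destroys itself, so it fires only once.
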(event `self.ReceiveBeginPlay`
  (`SceneComponent.SetVisibility` (`self.TextRender`) false false)
  (`self.DisableInput` (`GameplayStatics.GetPlayerController` 0)))

(event `self.ReceiveActorBeginOverlap`
  (params (OtherActor :type "Actor Object Reference"))
  ;[1 1 1] Handle Sister DIalog
  (cast `/Game/ProjectContents/BP/Player/BP_PawnPlayerBase` OtherActor)
  (`self.DisableInput` (`GameplayStatics.GetPlayerPawn` 0) (`GameplayStatics.GetPlayerController` 0))
  (bind _returnvalue (`GameplayStatics.GetActorOfClass` "/Game/ProjectContents/BP/SceneManager/BP_SceneManager_Scene12_Bedroom.BP_SceneManager_Scene12_Bedroom_C"))
  (`/Game/ProjectContents/BP/SceneManager/BP_SceneManager_Scene12_Bedroom.Part0` _returnvalue)
  (`self.K2_DestroyActor`))

(fn `UserConstructionScript`)