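; Big sister NPC actor, drawn as a Paper2D flipbook with a shadow and a text render, that can be hidden and shown.
; SetVisibilityFalse hides all three components, while SetVisibilityTrue turns the flipbook to a fixed 180-degree relative rotation and reveals only it and the shadow, leaving the text hidden.
; The event graph holds only disabled stubs, and construction defers to the parent class.
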(fn `SetVisibilityFalse`
  (`SceneComponent.SetVisibility` (`self.PaperFlipbook`) false false)
  (`SceneComponent.SetVisibility` (`self.Shadow`) false false)
  (`SceneComponent.SetVisibility` (`self.TextRender`) false false))

(fn `SetVisibilityTrue`
  (bind _paperflipbook (`self.PaperFlipbook`))
  (`SceneComponent.K2_SetRelativeRotation` _paperflipbook (struct :`Yaw` 180.0) false false)
  (`SceneComponent.SetVisibility` _paperflipbook true false)
  (`SceneComponent.SetVisibility` (`self.Shadow`) true false))

(fn `UserConstructionScript`
  (`parent.UserConstructionScript`))