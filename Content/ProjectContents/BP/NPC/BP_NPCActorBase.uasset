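; Base NPC actor that shows cycling dialog lines in a text render when the player interacts nearby.
; Box overlap with either player class toggles input and proximity, hiding the text on exit.
; Interact calls OnInteractPressed unless the game instance is viewing a scene; its CurrentScene switch has only a default branch, which advances dialog.
; Events also swap idle, walk and sit flipbooks, and a timeline lerps the NPC between two positions.
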(event `MoveNPC Event`
  (params (StartPosition :type "Vector Structure") (EndPosition :type "Vector Structure"))
  ;[1 1 1] Move NPC Event
  (bind (_direction _alpha) (`Timeline|MoveNPC` :!via `PlayFromStart`)
    (:`Update`
      (`self.K2_SetActorLocation` (`KismetMathLibrary.VLerp` StartPosition EndPosition _alpha))
      (`PaperFlipbookComponent.SetFlipbook` (`self.PaperFlipbook`) (`self.WalkFlipbook`)))
    (:`Finished`
      (`PaperFlipbookComponent.SetFlipbook` (`self.PaperFlipbook`) (`self.Idle Flipbook`)))))

(event `self.ReceiveBeginPlay`
  ;[1 1 1] Set Actor Starting Location
  (`self.DisableInput` (`GameplayStatics.GetPlayerController` 0)))

(event `self.Box.OnComponentBeginOverlap`
  (params (OverlappedComponent :type "PrimitiveComponent Object Reference") (OtherActor :type "Actor Object Reference") (OtherComp :type "PrimitiveComponent Object Reference") (OtherBodyIndex :type Integer) (bFromSweep :type Boolean) (SweepResult :type "HitResult Structure (by ref)"))
  ;[1 1 1] Toggle Visibility
  (cast `/Game/ProjectContents/BP/Player/BP_PawnPlayerBase` OtherActor
    (:`then`
      _)
    (:`CastFailed`
      (cast `/Game/ProjectContents/BP/Player/BP_PlayerOpenRoom` OtherActor)))
  (set `self.isPlayerNear` true)
  (`self.EnableInput` (`GameplayStatics.GetPlayerController` 0)))

(event `self.Box.OnComponentEndOverlap`
  (params (OverlappedComponent :type "PrimitiveComponent Object Reference") (OtherActor :type "Actor Object Reference") (OtherComp :type "PrimitiveComponent Object Reference") (OtherBodyIndex :type Integer))
  ;[1 1 1] Toggle Visibility
  (cast `/Game/ProjectContents/BP/Player/BP_PawnPlayerBase` OtherActor
    (:`then`
      _)
    (:`CastFailed`
      (cast `/Game/ProjectContents/BP/Player/BP_PlayerOpenRoom` OtherActor)))
  (set `self.isPlayerNear` false)
  (`self.DisableInput` (`GameplayStatics.GetPlayerController` 0))
  (`SceneComponent.SetVisibility` (`self.TextRender`) false false))

(event `SetFlipbookSit`
  (`PaperFlipbookComponent.SetFlipbook` (`self.PaperFlipbook`) (`self.SitFlipbook`))
  (`SceneComponent.SetVisibility` (`self.Shadow`) false false))

(event `InputAction|Interact` :consume false
  (params (Key :type "Key Structure"))
  ;[1 1 1] On Interact Pressed
  (:`Pressed`
    (if (`self.isPlayerNear`)
      (bind _asbp_game_instance (cast `/Game/ProjectContents/BP/BP_GameInstance` (`GameplayStatics.GetGameInstance`)))
      (if (not (`/Game/ProjectContents/BP/BP_GameInstance.isViewingScene` _asbp_game_instance))
        (`self.OnInteractPressed`)))))

(event `SetFlipbookIdle`
  (`PaperFlipbookComponent.SetFlipbook` (`self.PaperFlipbook`) (`self.Idle Flipbook`))
  (`SceneComponent.SetVisibility` (`self.Shadow`) true false))

(event `SetFlipbookWalk`
  (`PaperFlipbookComponent.SetFlipbook` (`self.PaperFlipbook`) (`self.WalkFlipbook`))
  (`SceneComponent.SetVisibility` (`self.Shadow`) true false))

(fn `ChangeDialogOnInteract`
  (if (== (`self.CurrentDialogIndex`) (- (`KismetArrayLibrary.Array_Length` (`self.DialogList`)) 1))
    (bind _output_get (set `self.CurrentDialogIndex` 0))
    (`TextRenderComponent.K2_SetText` (`self.TextRender`) (`KismetTextLibrary.Conv_StringToText` (`|GetArrayItem` (`self.DialogList`) _output_get)))
    (else
      (bind _result (`/Engine/EditorBlueprintResources/StandardMacros.IncrementInt` (`self.CurrentDialogIndex`))
        (:`  `
          (`TextRenderComponent.K2_SetText` (`self.TextRender`) (`KismetTextLibrary.Conv_StringToText` (`|GetArrayItem` (`self.DialogList`) _result))))))))

(fn `OnInteractPressed`
  (bind _asbp_game_instance (cast `/Game/ProjectContents/BP/BP_GameInstance` (`GameplayStatics.GetGameInstance`)))
  (switch `int` (`/Game/ProjectContents/BP/BP_GameInstance.CurrentScene` _asbp_game_instance)
    (:`Default`
      (`self.ChangeDialogOnInteract`)
      (`SceneComponent.SetVisibility` (`self.TextRender`) true false))))

(fn `UserConstructionScript`
  (locals (NewLocalVar_0 :type "TextRenderComponent Object Reference"))
  (`TextRenderComponent.K2_SetText` (`self.TextRender`) (`KismetTextLibrary.Conv_StringToText` (`|GetArrayItem` (`self.DIalogList`)))))