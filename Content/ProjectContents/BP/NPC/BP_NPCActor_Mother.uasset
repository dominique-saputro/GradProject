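; BP_NPCActor_Mother is the Blueprint for the Mother NPC, a Paper2D flipbook character with a shadow and a text render component.
; Scene 2 teacher functions start a talk by rotating the flipbook half a turn and showing the passed-in text, then end it by restoring the rotation and hiding the text.
; A separate function hides both the flipbook and its shadow.
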(fn `Scene2_TeacherEnd`
  (`SceneComponent.K2_SetRelativeRotation` :`self` (`self.PaperFlipbook`))
  (`SceneComponent.SetVisibility` (`self.TextRender`) false false))

(fn `Scene2_TeacherStart`
  (params (`Display Text` :type Text))
  (bind _textrender (`self.TextRender`))
  (`SceneComponent.K2_SetRelativeRotation` (`self.PaperFlipbook`) (struct :`Yaw` 180.0) false false)
  (`TextRenderComponent.K2_SetText` _textrender `Display Text`)
  (`SceneComponent.SetVisibility` _textrender true false))

(fn `SetVisibilityFalse_0`
  (`SceneComponent.SetVisibility` (`self.PaperFlipbook`) false false)
  (`SceneComponent.SetVisibility` (`self.Shadow`) false false))

(fn `UserConstructionScript`
  (`parent.UserConstructionScript`))