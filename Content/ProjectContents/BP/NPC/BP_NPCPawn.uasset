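; NPC pawn with a flipbook sprite that walks to a goal position and shows dialog text.
; On begin play it starts a simple AI move with a walking flipbook, then switches to idle after a fixed delay, regardless of arrival.
; Overlaps toggle text visibility and a player-near flag, which is checked only when movement starts.
; NPCInteractions cycles the text through a dialog list, wrapping around; nothing here calls it.
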(event `self.ReceiveBeginPlay`
  (`self.MoveNPC`)
  (`KismetSystemLibrary.Delay` 2.2)
  (`PaperFlipbookComponent.SetFlipbook` (`self.Sprite`) (`self.IdleFlipbook`)))

(event `self.ReceiveActorBeginOverlap`
  (params (OtherActor :type "Actor Object Reference"))
  ;[1 1 1] Toggle Visibility
  (`SceneComponent.SetVisibility` (`self.TextRender`) true false)
  (set `self.isPlayerNear` true))

(event `self.Box.OnComponentEndOverlap`
  (params (OverlappedComponent :type "PrimitiveComponent Object Reference") (OtherActor :type "Actor Object Reference") (OtherComp :type "PrimitiveComponent Object Reference") (OtherBodyIndex :type Integer))
  ;[1 1 1] Toggle Visibility
  (`SceneComponent.SetVisibility` (`self.TextRender`) false false)
  (set `self.isPlayerNear` false))

(fn `MoveNPC`
  (if (`self.isPlayerNear`)
    (`KismetSystemLibrary.PrintString` "StopMoving")
    (else
      (`AIBlueprintHelperLibrary.SimpleMoveToLocation` (`self.GetController`) (`self.GoalPosition`))
      (`PaperFlipbookComponent.SetFlipbook` (`self.Sprite`) (`self.WalkingFlipbook`)))))

(fn `NPC Interactions`
  (if (== (`self.CurrentDialogIndex`) (- (`KismetArrayLibrary.Array_Length` (`self.DialogList`)) 1))
    (bind _output_get (set `self.CurrentDialogIndex` 0))
    (`TextRenderComponent.K2_SetText` (`self.TextRender`) (`KismetTextLibrary.Conv_StringToText` (`|GetArrayItem` (`self.DialogList`) _output_get)))
    (else
      (bind _result (`/Engine/EditorBlueprintResources/StandardMacros.IncrementInt` (`self.CurrentDialogIndex`))
        (:`  `
          (`TextRenderComponent.K2_SetText` (`self.TextRender`) (`KismetTextLibrary.Conv_StringToText` (`|GetArrayItem` (`self.DialogList`) _result))))))))

(fn `UserConstructionScript`)