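; BP_PaperBall is a one-shot scripted paper ball throw that triggers part of the classroom scene.
; The first overlap of its Box reveals the hidden sprite, starts the throw, and two seconds later calls Part3 on BP_SceneManager_Scene02_Classroom.
; Two chained timelines lerp the actor from StartPoint to TeacherHead, then down to GoalPoint.
; Sprite and shadow are hidden on construction, and the shadow is hidden again after the drop.
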(event `self.Box.OnComponentBeginOverlap`
  (params (OverlappedComponent :type "PrimitiveComponent Object Reference") (OtherActor :type "Actor Object Reference") (OtherComp :type "PrimitiveComponent Object Reference") (OtherBodyIndex :type Integer) (bFromSweep :type Boolean) (SweepResult :type "HitResult Structure (by ref)"))
  ;[1 1 1] Start Classroom Scene on Overlap
  (if (not (`self.isPaperBallThrown`))
    (bind _returnvalue (`GameplayStatics.GetActorOfClass` "/Game/ProjectContents/BP/SceneManager/BP_SceneManager_Scene02_Classroom.BP_SceneManager_Scene02_Classroom_C"))
    (set `self.isPaperBallThrown` true)
    (`self.Throwing PaperBall`)
    (`KismetSystemLibrary.Delay` 2.0)
    (`/Game/ProjectContents/BP/SceneManager/BP_SceneManager_Scene02_Classroom.Part3` _returnvalue)))

(event `Throwing PaperBall`
  ;[1 1 1] Throwing Movement
  (`SceneComponent.SetVisibility` (`self.PaperSprite`) true false)
  (bind (_direction _alpha) (`Timeline|PaperBallPath`)
    (:`Update`
      (bind _returnvalue (`KismetMathLibrary.VLerp` (`self.StartPoint`) (`self.TeacherHead`) _alpha))
      (`self.K2_SetActorLocation` _returnvalue))
    (:`Finished`
      (bind (_direction_2 _alpha_2) (`Timeline|PaperBallDrop`)
        (:`Update`
          (`self.K2_SetActorLocation` (`KismetMathLibrary.VLerp` _returnvalue (`self.GoalPoint`) _alpha_2)))
        (:`Finished`
          (`SceneComponent.SetVisibility` (`self.Shadow`) false false))))))

(fn `UserConstructionScript`
  (`SceneComponent.SetVisibility` (`self.PaperSprite`) false false)
  (`SceneComponent.SetVisibility` (`self.Shadow`) false false))