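; BP_Ball is a ball actor that travels to a goal point while appearing to roll.
; MoveBall plays the MoveTime timeline, lerping the actor from StartPoint to GoalPoint without sweep and pitching the Sphere component by alpha times a rotation multiplier.
; StartPoint is captured at BeginPlay and again when each move finishes, so successive moves continue from the last position.
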(event `self.ReceiveBeginPlay`
  (set `self.StartPoint` (`self.K2_GetActorLocation`)))

(event `MoveBall`
  (bind (_direction _alpha) (`Timeline|MoveTime` :!via `PlayFromStart`)
    (:`Update`
      (`self.K2_SetActorLocation` (`KismetMathLibrary.VLerp` (`self.StartPoint`) (`self.GoalPoint`) _alpha))
      (`SceneComponent.K2_SetRelativeRotation` (`self.Sphere`) (`KismetMathLibrary.MakeRotator` 0.0 (* _alpha (`self.RotationMultipier`))) false false))
    (:`Finished`
      (set `self.StartPoint` (`self.K2_GetActorLocation`)))))

(fn `UserConstructionScript`)