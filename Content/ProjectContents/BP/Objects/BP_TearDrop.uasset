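; BP_TearDrop is a tear drop pickup that the player collects with the Interact input.
; Begin and end overlap with either BP_PawnPlayerBase or BP_PlayerOpenRoom enable and disable the actor's input, so Interact only responds while the player is nearby.
; Pressing Interact plays a pickup sound, adds the WBP_ObtainTearDrop widget to the viewport and destroys the actor.
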(event `InputAction|Interact`
  (params (Key :type "Key Structure"))
  (:`Pressed`
    (`GameplayStatics.PlaySound2D` "/Engine/VREditor/Sounds/UI/Object_PickUp.Object_PickUp" 1.0 1.0 0.0 null null)
    (bind _returnvalue (`|CreateWidget` "/Game/ProjectContents/BP/Widgets/WBP_ObtainTearDrop.WBP_ObtainTearDrop_C" (`GameplayStatics.GetPlayerController` 0)))
    (`UserWidget.AddToViewport` _returnvalue 0)
    (`self.K2_DestroyActor`)))

(event `self.ReceiveActorBeginOverlap`
  (params (OtherActor :type "Actor Object Reference"))
  ;[1 1 1] Toggle Input on Overlap
  (cast `/Game/ProjectContents/BP/Player/BP_PawnPlayerBase` OtherActor
    (:`then`
      _)
    (:`CastFailed`
      (cast `/Game/ProjectContents/BP/Player/BP_PlayerOpenRoom` OtherActor)))
  (`self.EnableInput` (`GameplayStatics.GetPlayerController` 0)))

(event `self.ReceiveActorEndOverlap`
  (params (OtherActor :type "Actor Object Reference"))
  ;[1 1 1] Toggle Input on Overlap
  (cast `/Game/ProjectContents/BP/Player/BP_PawnPlayerBase` OtherActor
    (:`then`
      _)
    (:`CastFailed`
      (cast `/Game/ProjectContents/BP/Player/BP_PlayerOpenRoom` OtherActor)))
  (`self.DisableInput` (`GameplayStatics.GetPlayerController` 0)))

(fn `UserConstructionScript`)