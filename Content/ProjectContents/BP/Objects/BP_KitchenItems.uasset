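; BP_KitchenItems is a pickup the player takes for the Scene 4 minigame.
; Box overlap with the player pawn shows a text prompt and enables input, and leaving reverses both.
; Pressing Interact adds the item name to the inventory on the minigame manager found at BeginPlay, then destroys the actor.
; An UpdateSprite event applies the selected sprite and builds the "Take" prompt from the item name.
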(event `InputAction|Interact`
  (params (Key :type "Key Structure"))
  (:`Pressed`
    (`KismetArrayLibrary.Array_Add` (`/Game/ProjectContents/BP/LevelActors/BP_Scene4_MinigameManager.Inventory` (`self.MinigameManager`)) (`self.ItemName`))
    (`self.K2_DestroyActor`)))

(event `self.ReceiveBeginPlay`
  (bind _returnvalue (`GameplayStatics.GetActorOfClass` "/Game/ProjectContents/BP/LevelActors/BP_Scene4_MinigameManager.BP_Scene4_MinigameManager_C"))
  (set `self.MinigameManager` _returnvalue)
  (`SceneComponent.SetVisibility` (`self.TextRender`) false false))

(event `UpdateSprite`
  (`PaperSpriteComponent.SetSprite` (`self.PaperSprite`) (`self.SelectedSprite`))
  (`TextRenderComponent.K2_SetText` (`self.TextRender`) (`KismetTextLibrary.Conv_StringToText` (`KismetStringLibrary.Concat_StrStr` (`KismetStringLibrary.Concat_StrStr` "Take " (`self.ItemName`)) "?"))))

(event `self.Box.OnComponentBeginOverlap`
  (params (OverlappedComponent :type "PrimitiveComponent Object Reference") (OtherActor :type "Actor Object Reference") (OtherComp :type "PrimitiveComponent Object Reference") (OtherBodyIndex :type Integer) (bFromSweep :type Boolean) (SweepResult :type "HitResult Structure (by ref)"))
  (cast `/Game/ProjectContents/BP/Player/BP_PawnPlayerBase` OtherActor)
  (`self.EnableInput` (`GameplayStatics.GetPlayerController` 0))
  (`SceneComponent.SetVisibility` (`self.TextRender`) true false))

(event `self.Box.OnComponentEndOverlap`
  (params (OverlappedComponent :type "PrimitiveComponent Object Reference") (OtherActor :type "Actor Object Reference") (OtherComp :type "PrimitiveComponent Object Reference") (OtherBodyIndex :type Integer))
  (cast `/Game/ProjectContents/BP/Player/BP_PawnPlayerBase` OtherActor)
  (`self.DisableInput` (`GameplayStatics.GetPlayerController` 0))
  (`SceneComponent.SetVisibility` (`self.TextRender`) false false))

(fn `UserConstructionScript`)